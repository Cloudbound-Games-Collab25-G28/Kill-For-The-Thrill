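; Enemy Blueprint that wanders the level and dies on taking any damage.
; From BeginPlay, RandomRoam uses AIMoveTo to reach a random reachable point around its current location, then waits briefly and calls itself again.
; The loop continues only on a successful move, as no failure path is wired.
; Any damage, regardless of amount, destroys the actor and then broadcasts the OnEnemyDeath dispatcher.
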(event Custom|RandomRoam
  (AI|AIMoveTo self (.RandomLocation (AI|Navigation|GetRandomReachablePointinRadius (Transformation|GetActorLocation) 2e+03 0 0)) 0 1e+01 false
    (:OnSuccess
      (Utilities|FlowControl|Delay (Math|Random|RandomFloatinRange 1.0 2.0))
      (CallFunction|RandomRoam))))

(event EventBeginPlay
  (CallFunction|RandomRoam))

(event Game|Damage|EventAnyDamage
  (params (Damage :type Float%20%28single-precision%29) (DamageType :type Damage%20Type%20Object%20Reference) (InstigatedBy :type Controller%20Object%20Reference) (DamageCauser :type Actor%20Object%20Reference))
  (Actor|DestroyActor)
  (Default|CallOnEnemyDeath))

(fn ConstructionScript)