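; Melee weapon Blueprint that extends its parent's combo system with area damage for three regular attacks and a charged attack.
; Each combo step runs a sphere trace at the Arrow with increasing radius and damage, while charged hits scale both by charge amount above a minimum threshold.
; The shared DamageObjectInRange ignores the player and damages every returned hit, with debug drawing and printing enabled.
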(event EventBeginPlay)

(event Collision|EventActorBeginOverlap
  (params (OtherActor :type Actor%20Object%20Reference)))

(event EventTick
  (params (DeltaSeconds :type Float%20%28single-precision%29)))

(fn ConstructionScript
  (|CallParentFunction))

(fn RegularComboSwapper
  (|CallParentFunction))

(fn RegularCombo1
  (bind _arrow (Variables|Default|GetArrow))
  (bind _returnvalue (Transformation|GetWorldLocation _arrow))
  (CallFunction|DamageObjectinRange _returnvalue _returnvalue (Variables|Default|GetSphere%20trace%20radius) (+ (Variables|Default|GetBase%20Damage%20Amount) 5.0)))

(fn RegularCombo2
  (bind _arrow (Variables|Default|GetArrow))
  (bind _returnvalue (Transformation|GetWorldLocation _arrow))
  (CallFunction|DamageObjectinRange _returnvalue _returnvalue (+ (Variables|Default|GetSphere%20trace%20radius) 5e+01) (+ (Variables|Default|GetBase%20Damage%20Amount) 1e+01)))

(fn RegularCombo3
  (bind _arrow (Variables|Default|GetArrow))
  (bind _returnvalue (Transformation|GetWorldLocation _arrow))
  (CallFunction|DamageObjectinRange _returnvalue _returnvalue (+ (Variables|Default|GetSphere%20trace%20radius) 1e+02) (+ (Variables|Default|GetBase%20Damage%20Amount) 25.0)))

(fn DamageObjectinRange
  (params (Start :type Vector) (End :type Vector) (Radius :type Float%20%28single-precision%29) (BaseDamage :type Float%20%28single-precision%29))
  (bind _outhits (Collision|MultiSphereTraceForObjects Start End Radius (Variables|Default|Getobject%20types) false (Utilities|Array|MakeArray (Variables|Default|GetPlayer%20Reference)) "ForDuration" true "(R=0.060860,G=0.000000,B=1.000000,A=1.000000)"))
  (for _array_element _outhits
    (Game|Damage|ApplyDamage (.HitActor (Collision|BreakHitResult _array_element)) (Math|Conversions|ToFloat(Integer) (Math|Float|Round BaseDamage)) 0 0 "/Script/Engine.DamageType")
    (Development|PrintString (Utilities|String|Append "Damage dealt to" (Utilities|GetDisplayName (.HitActor (Collision|BreakHitResult _array_element)))))))

(fn ChargedAttackScaling
  (params (Charged%20Amount :type Float%20%28double-precision%29))
  (bind _arrow (Variables|Default|GetArrow))
  (bind _returnvalue (Transformation|GetWorldLocation _arrow))
  (if (> Charged%20Amount 0.25)
    (CallFunction|DamageObjectinRange _returnvalue _returnvalue (* (+ (Variables|Default|GetSphere%20trace%20radius) 1.5e+02) (+ Charged%20Amount 1.0)) (* (+ (Variables|Default|GetBase%20Damage%20Amount) 2e+01) (* Charged%20Amount 2.0)))))