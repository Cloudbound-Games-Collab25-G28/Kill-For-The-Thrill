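; BP_BaseProjectile is a base weapon projectile Blueprint that deals damage around an impact point.
; Its Hit event runs a small zero-length multi-sphere object trace at the supplied location, ignoring the instigator, owner and itself.
; Each returned hit receives rounded base damage with the configured damage type, with no de-duplication of actors.
; Debug trace drawing and a print of each damaged actor are left on.
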(event Collision|EventHit
  (params (MyComp :type Primitive%20Component%20Object%20Reference) (Other :type Actor%20Object%20Reference) (OtherComp :type Primitive%20Component%20Object%20Reference) (bSelfMoved :type Boolean) (HitLocation :type Vector :default "0, 0, 0") (HitNormal :type Vector :default "0, 0, 0") (NormalImpulse :type Vector :default "0, 0, 0") (Hit :type Hit%20Result%20Structure%20%28by%20ref%29))
  (bind _outhits (Collision|MultiSphereTraceForObjects HitLocation HitLocation 1e+01 (Variables|Default|GetObject%20types) false (Utilities|Array|MakeArray (Variables|Actor|GetInstigator) self (Components|GetOwner)) "ForDuration" true "(R=0.060860,G=0.000000,B=1.000000,A=1.000000)" "(R=0.000000,G=1.000000,B=0.000000,A=1.000000)" 1.0))
  (for _array_element _outhits
    (Game|Damage|ApplyDamage (.HitActor (Collision|BreakHitResult _array_element)) (Math|Conversions|ToFloat(Integer) (Math|Float|Round (Variables|Default|GetBase%20Damage%20Amount))) 0 0 "/Script/Engine.DamageType")
    (Development|PrintString (Utilities|String|Append "Damage dealt to" (Utilities|GetDisplayName (.HitActor (Collision|BreakHitResult _array_element)))))))

(fn ConstructionScript)