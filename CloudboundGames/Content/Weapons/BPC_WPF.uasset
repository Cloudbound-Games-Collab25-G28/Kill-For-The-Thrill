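; BPC_WPF is a Blueprint component that gives a character a weapon and handles its attack input.
; CreateWeapon spawns BP_WeaponExample, snaps it to the character's "Weapon socket" and stores the reference.
; Releasing or canceling IA_E_Held chooses by hold time between a normal attack with swing sound and a charged attack with clamped strength.
; ChargedAttackFunction offers the charged path as a direct call, while SendReferenceForce and GetCurrentReference are empty.
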(event Custom|Create%20Weapon
  (params (Char%20Ref :type BP%20Weapon%20Character%20Object%20Reference))
  ;[1 1 1] Can be swapped through whatever
  (bind _returnvalue (Game|SpawnActorfromClass "/Game/Weapons/BP_WeaponExample.BP_WeaponExample_C" (Math|Transform|MakeTransform "1000.000000,1810.000000,100.000000" "0, 0, 0" "1.000000,1.000000,1.000000") "AlwaysSpawn" "MultiplyWithRoot" Char%20Ref 0))
  (Transformation|AttachActorToActor _returnvalue Char%20Ref "Weapon socket" "SnapToTarget" "SnapToTarget" "SnapToTarget" true)
  (Variables|Default|SetCurrent%20Weapon%20Reference _returnvalue))

(event Input|EnhancedActionEvents|EnhancedInputActionIA_E_Held
  (params (ActionValue :type Boolean) (ElapsedSeconds :type Float%20%28double-precision%29) (TriggeredSeconds :type Float%20%28double-precision%29) (InputAction :type Input%20Action%20Object%20Reference :default "/Game/Weapons/WepInputs/IA_E_Held.IA_E_Held"))
  (:Canceled
    ;[1 1 1] Checks if basically theres a charge or not
    (if (>= ElapsedSeconds 0.25) :!label _label
      (Default|ChargedAttackWeapon (Variables|Default|GetCurrent%20Weapon%20Reference) (Math|Float|Clamp(Float) (* ElapsedSeconds 1.0)))
      (else
        (Audio|PlaySoundatLocation "/Game/Audio/combat/Sword_Swing/MS_SwordSwing.MS_SwordSwing" (Transformation|GetActorLocation (Components|GetOwner)) "0, 0, 0" 1.0 1.0 0.0 0 0 0 0)
        (Default|AttackwiththeWeapon (Variables|Default|GetCurrent%20Weapon%20Reference)))))
  (:Completed
    (goto _label)))

(fn ChargedAttackFunction
  (params (Input%20Float :type Float%20%28double-precision%29))
  ;[1 1 1] Alternative action for using the BP parent function version
  (if (>= Input%20Float 0.25)
    (Default|ChargedAttackWeapon (Variables|Default|GetCurrent%20Weapon%20Reference) (Math|Float|Clamp(Float) (* Input%20Float 1.0)))))

(fn SendReferenceForce
  (return 0))

(fn GetCurrentReference
  (return 0))