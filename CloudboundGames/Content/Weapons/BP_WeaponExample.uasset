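; Example weapon Blueprint with a regular combo attack and a charged attack, serving as a template for child weapons.
; Attacking starts a short timer and advances a three-step combo with growing sphere-trace radius, and a separate event resets the combo index.
; Charged attacks scale the radius by charge tier and cancel below the minimum.
; Both debug-draw traces at handleSocket and apply damage to hits, though only regular attacks pass BaseDamage.
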(event Custom|Attack%20with%20the%20weapon
  (Utilities|Time|SetTimerbyEvent (EventDispatchers|CreateEvent :!event Custom|Reset%20Combo%20Action%20to%200) 0.75 false true)
  (CallFunction|RegularAttack))

(event Custom|Reset%20Combo%20Action%20to%200
  (Variables|Default|SetLocal%20Index%20Attack%20Combo 0))

(fn ConstructionScript)

(fn ChargedAttackWeapon
  (params (Charged%20Amount :type Float%20%28double-precision%29))
  (bind _defaultsceneroot (Variables|Default|GetDefaultSceneRoot))
  (bind _returnvalue (Transformation|GetSocketLocation _defaultsceneroot "handleSocket"))
  ;[1 1 1] Differs on weapon/child bp/bpc, if this does nothing leave it as empty
  ;[1 1 1] Example of how you'd use the charge amount to differ the values, this is just in the example.
  ; Child bp's of this should have everything but the print strings.
  (if (>= Charged%20Amount 0.75)
    (Development|PrintString "Full Charge")
    ;[1 1 1] Can be made into function
    (Variables|Default|SetRadius 1.8e+02)
    (bind _outhits (Collision|MultiSphereTraceByChannel _returnvalue _returnvalue (Variables|Default|GetRadius) "TraceTypeQuery1" false 0 "ForDuration" true "(R=1.000000,G=0.000000,B=0.985139,A=1.000000)" "(R=0.000000,G=1.000000,B=0.000000,A=1.000000)" 2.0 :!label _label))
    (for _array_element _outhits
      ;;[1 1 1] Implement using interface/dispatcher
      (Game|Damage|ApplyDamage (.HitActor (Collision|BreakHitResult _array_element)) 0.0 0 0 "/Script/Engine.DamageType"))
    (elif (>= Charged%20Amount 0.5)
      (Development|PrintString "Medium Charge")
      (Variables|Default|SetRadius 135.0)
      (goto _label)
      (elif (>= Charged%20Amount 0.25)
        (Development|PrintString "Short Charge")
        (Variables|Default|SetRadius 9e+01)
        (goto _label)
        (else
          ;[1 1 1] Replaced with function in char as of for now
          (Development|PrintString "Not Charged, Cancelled"))))))

(fn RegularAttack
  (bind _staticmesh (Variables|Default|GetStaticMesh))
  (bind _returnvalue (Transformation|GetSocketLocation _staticmesh "handleSocket"))
  (bind _returnvalue_2 (+ _returnvalue ""))
  (switch int (Variables|Default|GetLocal%20Index%20Attack%20Combo)
    (:0
      (Variables|Default|SetLocal%20Index%20Attack%20Combo 1)
      (Development|PrintString "Combo 1 " true true "(R=0.997782,G=0.000000,B=1.000000,A=1.000000)")
      ;[1 1 1] Just for now since its janky
      (Variables|Default|SetRadius 1.5e+02))
    (:1
      (Variables|Default|SetLocal%20Index%20Attack%20Combo 2)
      (Development|PrintString "Combo 2 " true true "(R=0.997782,G=0.000000,B=1.000000,A=1.000000)")
      (Variables|Default|SetRadius 225.0))
    (:2
      (Variables|Default|SetLocal%20Index%20Attack%20Combo 0)
      (Development|PrintString "Combo 3" true true "(R=0.997782,G=0.000000,B=1.000000,A=1.000000)")
      (Variables|Default|SetRadius 3e+02)))
  ;;[1 1 1] Can be put into function
  (bind _outhits (Collision|MultiSphereTraceByChannel _returnvalue_2 _returnvalue_2 (Variables|Default|GetRadius) "TraceTypeQuery1" false 0 "ForDuration" true "(R=0.000000,G=0.095898,B=1.000000,A=1.000000)" "(R=0.000000,G=1.000000,B=0.000000,A=1.000000)" 2.0))
  (for _array_element _outhits
    (Game|Damage|ApplyDamage (.HitActor (Collision|BreakHitResult _array_element)) (Variables|Default|GetBase%20Damage) (Game|GetInstigatorController (Components|GetOwner)) 0 "/Script/Engine.DamageType")))

(fn GetCurrentReference
  (return 0))