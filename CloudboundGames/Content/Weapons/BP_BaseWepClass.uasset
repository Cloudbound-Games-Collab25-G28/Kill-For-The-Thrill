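; Base weapon Blueprint that provides a three-step regular attack combo and a charged attack entry point for child weapons.
; Each attack sets a timer and advances a looping combo index, standing in for animation notifies, to call one of three empty combo functions meant for child overrides.
; Charged attacks pass their charge amount to a tier check that currently only prints the charge level.
; Montage playback is unwired placeholder code.
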(event Custom|Attack%20with%20the%20weapon
  (Utilities|Time|SetTimerbyEvent (EventDispatchers|CreateEvent :!event Custom|Reset%20Combo%20Action%20to%200) 0.75 false true)
  (CallFunction|RegularComboSwapper))

(event Custom|Reset%20Combo%20Action%20to%200
  (Variables|Default|SetLocal%20Index%20Attack%20Combo 0))

(fn ConstructionScript)

(fn ChargedAttackFunction
  (params (Charged%20Amount :type Float%20%28double-precision%29))
  (CallFunction|ChargedAttackScaling Charged%20Amount))

(fn RegularComboSwapper
  ;[1 1 1] This is just due to not having notifiers from anims currently
  (switch int (Variables|Default|GetLocal%20Index%20Attack%20Combo)
    (:0
      (Variables|Default|SetLocal%20Index%20Attack%20Combo 1)
      (CallFunction|RegularCombo1))
    (:1
      (Variables|Default|SetLocal%20Index%20Attack%20Combo 2)
      (CallFunction|RegularCombo2))
    (:2
      (Variables|Default|SetLocal%20Index%20Attack%20Combo 0)
      (CallFunction|RegularCombo3))))

(fn RegularCombo1
  ;[1 1 1] Change in child bp
)

(fn RegularCombo2
  ;[1 1 1] Change in child bp
)

(fn RegularCombo3
  ;[1 1 1] Change in child bp
)

(fn ChargedAttackScaling
  (params (Charged%20Amount :type Float%20%28double-precision%29))
  (if (>= Charged%20Amount 0.75)
    (Development|PrintString "Full Charge")
    (elif (>= Charged%20Amount 0.5)
      (Development|PrintString "Medium Charge")
      (elif (>= Charged%20Amount 0.25)
        (Development|PrintString "Short Charge")))))

(fn GetCurrentReference
  (return 0))