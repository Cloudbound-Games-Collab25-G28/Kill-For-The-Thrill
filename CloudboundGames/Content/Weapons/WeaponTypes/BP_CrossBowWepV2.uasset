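; Crossbow weapon Blueprint that overrides its parent weapon's regular and charged attacks to fire projectiles from DirectionArrow.
; Regular attacks cycle through a three-step combo without calling the parent swapper, and every step spawns the same short-lived piercing projectile with boosted base damage.
; Charged attacks spawn a test AoE projectile whose damage and lifetime scale linearly with charge amount.
; Both projectile types take the player as Instigator.
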(event EventBeginPlay)

(event Collision|EventActorBeginOverlap
  (params (OtherActor :type Actor%20Object%20Reference)))

(event EventTick
  (params (DeltaSeconds :type Float%20%28single-precision%29)))

(fn ConstructionScript
  (|CallParentFunction))

(fn RegularComboSwapper
  ;[1 1 1] This is the parent function (can be changed if using only one combo)
  (switch int (Variables|Default|GetLocal%20Index%20Attack%20Combo)
    (:0
      (Variables|Default|SetLocal%20Index%20Attack%20Combo 1)
      (CallFunction|RegularCombo1))
    (:1
      (Variables|Default|SetLocal%20Index%20Attack%20Combo 2)
      (CallFunction|RegularCombo2))
    (:2
      (Variables|Default|SetLocal%20Index%20Attack%20Combo 0)
      (CallFunction|RegularCombo3))))

(fn RegularCombo1
  (CallFunction|FireProjectileBasic))

(fn RegularCombo2
  (CallFunction|FireProjectileBasic))

(fn RegularCombo3
  (CallFunction|FireProjectileBasic))

(fn FireProjectileBasic
  (Game|SpawnActorfromClass "/Game/Weapons/WeaponTypes/Projectiles/BP_PierceProjectile.BP_PierceProjectile_C" (Transformation|GetWorldTransform (Variables|Default|GetDirection%20Arrow)) "AlwaysSpawn" "MultiplyWithRoot" 0 (+ (Variables|Default|GetBase%20Damage%20Amount) 1e+01) 0.1 (Variables|Default|GetPlayer%20Reference)))

(fn ChargedAttackScaling
  (params (Charged%20Amount :type Float%20%28double-precision%29))
  (Game|SpawnActorfromClass "/Game/Weapons/WeaponTypes/Projectiles/BP_AoeProjectileTest.BP_AoeProjectileTest_C" (Transformation|GetWorldTransform (Variables|Default|GetDirection%20Arrow)) "AlwaysSpawn" "MultiplyWithRoot" 0 (+ (+ (Variables|Default|GetBase%20Damage%20Amount) 15.0) (* (* Charged%20Amount 1e+01) 2.0)) (+ (/ Charged%20Amount 1e+01) 0.1) (Variables|Default|GetPlayer%20Reference)))