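; Melee weapon child Blueprint that overrides combo and charge attack steps, leaving regular and charged attack handling to its parent class.
; Each of the three combo hits and three charge tiers sets its own sphere radius and calls DamageObjsInRange at the Arrow's location, ignoring the player.
; That helper runs a debug-drawn multi-sphere object trace and applies damage, returning inside the loop after the first hit.
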(event EventBeginPlay)

(event Collision|EventActorBeginOverlap
  (params (OtherActor :type Actor%20Object%20Reference)))

(event EventTick
  (params (DeltaSeconds :type Float%20%28single-precision%29)))

(fn ConstructionScript
  (|CallParentFunction))

(fn RegularAttack
  (|CallParentFunction))

(fn ChargedAttackWeapon
  (params (Charged%20Amount :type Float%20%28double-precision%29))
  (|CallParentFunction Charged%20Amount))

(fn FullChargeAttack
  (bind _arrow (Variables|Default|GetArrow))
  (bind _returnvalue (Transformation|GetWorldLocation _arrow))
  (Variables|Default|SetSphere%20trace%20radius 7.5e+02)
  (CallFunction|DamageObj'sinRange (Variables|Default|GetSphere%20trace%20radius) (Variables|Default|Getobject%20types) (Utilities|Array|MakeArray (Variables|Default|GetPlayer%20Reference)) _returnvalue _returnvalue))

(fn MediumChargeAttack
  (bind _arrow (Variables|Default|GetArrow))
  (bind _returnvalue (Transformation|GetWorldLocation _arrow))
  (Variables|Default|SetSphere%20trace%20radius 5e+02)
  (CallFunction|DamageObj'sinRange (Variables|Default|GetSphere%20trace%20radius) (Variables|Default|Getobject%20types) (Utilities|Array|MakeArray (Variables|Default|GetPlayer%20Reference)) _returnvalue _returnvalue))

(fn LightChargeAttack
  (bind _arrow (Variables|Default|GetArrow))
  (bind _returnvalue (Transformation|GetWorldLocation _arrow))
  (Variables|Default|SetSphere%20trace%20radius 2.5e+02)
  (CallFunction|DamageObj'sinRange (Variables|Default|GetSphere%20trace%20radius) (Variables|Default|Getobject%20types) (Utilities|Array|MakeArray (Variables|Default|GetPlayer%20Reference)) _returnvalue _returnvalue))

(fn RegularCombo1
  (bind _arrow (Variables|Default|GetArrow))
  (bind _returnvalue (Transformation|GetWorldLocation _arrow))
  (Variables|Default|SetSphere%20trace%20radius 1.5e+02)
  (CallFunction|DamageObj'sinRange (Variables|Default|GetSphere%20trace%20radius) (Variables|Default|Getobject%20types) (Utilities|Array|MakeArray (Variables|Default|GetPlayer%20Reference)) _returnvalue _returnvalue))

(fn RegularCombo2
  (bind _arrow (Variables|Default|GetArrow))
  (bind _returnvalue (Transformation|GetWorldLocation _arrow))
  (Variables|Default|SetSphere%20trace%20radius 2.5e+02)
  (CallFunction|DamageObj'sinRange (Variables|Default|GetSphere%20trace%20radius) (Variables|Default|Getobject%20types) (Utilities|Array|MakeArray (Variables|Default|GetPlayer%20Reference)) _returnvalue _returnvalue))

(fn RegularCombo3
  (bind _arrow (Variables|Default|GetArrow))
  (bind _returnvalue (Transformation|GetWorldLocation _arrow))
  (Variables|Default|SetSphere%20trace%20radius 4.5e+02)
  (CallFunction|DamageObj'sinRange (Variables|Default|GetSphere%20trace%20radius) (Variables|Default|Getobject%20types) (Utilities|Array|MakeArray (Variables|Default|GetPlayer%20Reference)) _returnvalue _returnvalue))

(fn DamageObj'sinRange
  (params (Radius :type Float%20%28single-precision%29) (ObjectTypes :type Array%20of%20EObjectTypeQuery%20Enums :default "ObjectTypeQuery1") (ActorsToIgnore :type Array%20of%20Actor%20Object%20References) (End :type Vector :default "0, 0, 0") (Start :type Vector :default "0, 0, 0"))
  (bind _outhits (Collision|MultiSphereTraceForObjects Start End Radius ObjectTypes false ActorsToIgnore "ForDuration" true "(R=0.060860,G=0.000000,B=1.000000,A=1.000000)"))
  (for _array_element _outhits
    (Game|Damage|ApplyDamage (.HitActor (Collision|BreakHitResult _array_element)) (Variables|Default|GetBase%20Damage%20Amount) 0 0 "/Script/Engine.DamageType")
    (return)))