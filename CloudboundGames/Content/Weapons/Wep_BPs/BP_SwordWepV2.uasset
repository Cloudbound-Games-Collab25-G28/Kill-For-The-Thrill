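; Sword weapon Blueprint that extends a parent weapon with a three-hit combo and a charged area attack.
; Each combo step box-traces at its own box component with rising damage, then runs after-attack logic and a short timer.
; Charges above a threshold sphere-trace with charge-scaled radius and damage, then reset player movement speed.
; Both traces ignore the player, draw debug shapes and pass damage through the player's upgrade component before applying it.
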(event Custom|Small%20timer%20after%20attacking
  (Utilities|Time|SetTimerbyEvent (EventDispatchers|CreateEvent :!event Custom|Reset%20the%20players%20movement) 0.4 false true))

(event Custom|Reset%20the%20players%20movement
  (CallFunction|ResetPlayerMovementSpeed))

(fn ConstructionScript
  (|CallParentFunction))

(fn RegularComboSwapper
  (|CallParentFunction))

(fn RegularCombo1
  (bind _attack_1_combo (Variables|Default|GetAttack%201%20Combo))
  (bind _returnvalue (Transformation|GetWorldLocation _attack_1_combo))
  (CallFunction|DamageObjectinRangeBoxes _returnvalue _returnvalue (+ (Variables|Default|GetBase%20Damage%20Amount) 1e+01) (.yaw (Transformation|GetWorldRotation _attack_1_combo)) (Variables|/Script/Engine.BoxComponent|GetBoxExtent _attack_1_combo)))

(fn RegularCombo2
  (bind _attack_2_combo (Variables|Default|GetAttack%202%20Combo))
  (bind _returnvalue (Transformation|GetWorldLocation _attack_2_combo))
  (CallFunction|DamageObjectinRangeBoxes _returnvalue _returnvalue (+ (Variables|Default|GetBase%20Damage%20Amount) 2e+01) (.yaw (Transformation|GetWorldRotation _attack_2_combo)) (Variables|/Script/Engine.BoxComponent|GetBoxExtent _attack_2_combo)))

(fn RegularCombo3
  (bind _attack_3_combo (Variables|Default|GetAttack%203%20Combo))
  (bind _returnvalue (Transformation|GetWorldLocation _attack_3_combo))
  (CallFunction|DamageObjectinRangeBoxes _returnvalue _returnvalue (+ (Variables|Default|GetBase%20Damage%20Amount) 35.0) (.yaw (Transformation|GetWorldRotation _attack_3_combo)) (Variables|/Script/Engine.BoxComponent|GetBoxExtent _attack_3_combo)))

(fn DamageObjectinRangeSphere
  (params (Start :type Vector) (End :type Vector) (Radius :type Float%20%28single-precision%29) (BaseDamage :type Float%20%28single-precision%29))
  (bind _outhits (Collision|MultiSphereTraceForObjects Start End Radius (Variables|Default|Getobject%20types) false (Utilities|Array|MakeArray (Variables|Default|GetPlayer%20Reference)) "ForDuration" true "(R=1.000000,G=0.000000,B=0.034709,A=1.000000)" "(R=0.000000,G=1.000000,B=0.000000,A=1.000000)" 0.2))
  (for _array_element _outhits
    (bind _finaldamage (Default|ModifyDamage (Variables|/Game/Weapons/BP_WeaponCharacter.BP_WeaponCharacter_C|GetBPC_Upgrades (Variables|Default|GetPlayer%20Reference)) BaseDamage))
    (Game|Damage|ApplyDamage (.HitActor (Collision|BreakHitResult _array_element)) _finaldamage 0 0 "/Script/Engine.DamageType")
    (Development|PrintString (Utilities|String|Append "Damage dealt to" (Utilities|GetDisplayName (.HitActor (Collision|BreakHitResult _array_element)))))))

(fn ChargedAttackScaling
  (params (Charged%20Amount :type Float%20%28double-precision%29))
  (bind _arrow (Variables|Default|GetArrow))
  (bind _returnvalue (Transformation|GetWorldLocation _arrow))
  (if (> Charged%20Amount 0.25)
    (CallFunction|DamageObjectinRangeSphere _returnvalue _returnvalue (* (+ (Variables|Default|GetSphere%20trace%20radius) 1.5e+02) (+ Charged%20Amount 1.0)) (* (+ (Variables|Default|GetBase%20Damage%20Amount) 2e+01) (* Charged%20Amount 2.0)))
    (CallFunction|ResetPlayerMovementSpeed)))

(fn DamageObjectinRangeBoxes
  (params (Start :type Vector) (End :type Vector) (BaseDamage :type Float%20%28single-precision%29) (Orientation%20Z%20%28Yaw%29 :type Float%20%28single-precision%29) (HalfSize :type Vector))
  (bind _outhits (Class|KismetSystemLibrary|BoxTraceMultiforObjects Start End HalfSize (Math|Rotator|MakeRotator 0.0 0.0 Orientation%20Z%20%28Yaw%29) (Variables|Default|Getobject%20types) false (Utilities|Array|MakeArray (Variables|Default|GetPlayer%20Reference)) "ForDuration" true "(R=1.000000,G=0.000000,B=0.121054,A=1.000000)" "(R=0.000000,G=1.000000,B=0.000000,A=1.000000)" 0.2))
  (for _array_element _outhits
    (bind _finaldamage (Default|ModifyDamage (Variables|/Game/Weapons/BP_WeaponCharacter.BP_WeaponCharacter_C|GetBPC_Upgrades (Variables|Default|GetPlayer%20Reference)) BaseDamage))
    (Game|Damage|ApplyDamage (.HitActor (Collision|BreakHitResult _array_element)) _finaldamage 0 0 "/Script/Engine.DamageType")
    (Development|PrintString (Utilities|String|Append "Damage dealt to" (Utilities|GetDisplayName (.HitActor (Collision|BreakHitResult _array_element)))))
    (CallFunction|AfterAttack)
    (CallFunction|SmallTimerAfterAttacking))
  (CallFunction|AfterAttack)
  (CallFunction|SmallTimerAfterAttacking))