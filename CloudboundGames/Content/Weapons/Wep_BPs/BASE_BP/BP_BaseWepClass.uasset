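; Base weapon Blueprint providing regular combo, charged and special attack logic, with attack functions meant for child Blueprints to fill in.
; Regular attacks pass a timer-reset DoOnce spam limit, then cycle an index through three empty combo hooks while slowing the player.
; Charged attacks only print a charge tier, and the special attack slows then immediately resets player movement.
; Timers stand in for animation notifies, and montage playback is unconnected.
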(event Custom|Attack%20with%20the%20weapon
  ;[1 1 1] Should be replaced in child bp's by their anim timer
  (Utilities|FlowControl|DoOnce false
    (:Completed
      (Utilities|Time|SetTimerbyEvent (delegate Custom|Spam%20limit%20reset) 0.3 false true)
      (CallFunction|RegularComboSwapper))))

(event Custom|Reset%20Combo%20Action%20to%200
  ;[1 1 1] Should be replaced in child bp's by their anim timer
  (Variables|Default|SetLocal%20Index%20Attack%20Combo 0)
  (Utilities|FlowControl|DoOnce false) ; enters at Reset
)

(event Custom|Special%20Attack%20on%20Weapon
  ;[1 1 1] Should be replaced in child bp's by their anim timer
  (CallFunction|SpecialAttackFunction))

(event Custom|After%20Attack
  ;[1 1 1] Should be replaced in child bp's by their anim timer
  (Utilities|Time|SetTimerbyEvent (EventDispatchers|CreateEvent :!event Custom|Reset%20Combo%20Action%20to%200) 0.6 false true))

(event Custom|Spam%20limit%20reset
  ;[1 1 1] Should be replaced in child bp's by their anim timer
  (Utilities|FlowControl|DoOnce false) ; enters at Reset
)

(fn ConstructionScript)

(fn ChargedAttackWeaponFunction
  (params (Charged%20Amount :type Float%20%28double-precision%29))
  (CallFunction|ChargedAttackScaling Charged%20Amount))

(fn RegularComboSwapper
  ;[1 1 1] This is just due to not having notifiers from anims currently
  (switch int (Variables|Default|GetLocal%20Index%20Attack%20Combo)
    (:0
      (Variables|Default|SetLocal%20Index%20Attack%20Combo 1)
      (CallFunction|RegularCombo1)
      (CallFunction|ForciblySlowthePlayerDown (Variables|Default|GetPlayer%20Max%20walk%20Speed)))
    (:1
      (Variables|Default|SetLocal%20Index%20Attack%20Combo 2)
      (CallFunction|RegularCombo2)
      (CallFunction|ForciblySlowthePlayerDown (Variables|Default|GetPlayer%20Max%20walk%20Speed)))
    (:2
      (Variables|Default|SetLocal%20Index%20Attack%20Combo 0)
      (CallFunction|RegularCombo3)
      (CallFunction|ForciblySlowthePlayerDown (Variables|Default|GetPlayer%20Max%20walk%20Speed)))))

(fn RegularCombo1
  ;[1 1 1] Change in child bp
)

(fn RegularCombo2
  ;[1 1 1] Change in child bp
)

(fn RegularCombo3
  ;[1 1 1] Change in child bp
)

(fn ChargedAttackScaling
  (params (Charged%20Amount :type Float%20%28double-precision%29))
  (if (>= Charged%20Amount 0.75)
    (Development|PrintString "Full Charge")
    (elif (>= Charged%20Amount 0.5)
      (Development|PrintString "Medium Charge")
      (elif (>= Charged%20Amount 0.25)
        (Development|PrintString "Short Charge")))))

(fn SpecialAttackFunction
  ;[1 1 1] Do in child bp's
  (Default|SlowPlayerDownWhileAttacking (Variables|Default|GetPlayer%20Reference) (Variables|Default|GetPlayer%20Max%20walk%20Speed))
  (CallFunction|ResetPlayerMovementSpeed))

(fn ResetPlayerMovementSpeed
  (Default|ResetPlayerMovement (Variables|Default|GetPlayer%20Reference)))

(fn ForciblySlowthePlayerDown
  (params (Slowed%20Amount :type Float%20%28double-precision%29))
  (Default|SlowPlayerDownWhileAttacking (Variables|Default|GetPlayer%20Reference) Slowed%20Amount))

(fn GetCurrentReference
  (return 0))