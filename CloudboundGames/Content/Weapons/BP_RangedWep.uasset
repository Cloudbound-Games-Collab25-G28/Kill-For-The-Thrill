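; Ranged weapon Blueprint that extends a parent weapon class to fire projectiles as its regular attack.
; The combo swapper replaces the parent's logic, cycling a local index through three attack steps.
; Only the first step fires, spawning BP_BaseProjectile at the Arrow component's world transform; the other two are empty stubs.
; Charged attacks pass straight to the parent, and charge scaling is an empty stub.
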(event EventBeginPlay)

(event Collision|EventActorBeginOverlap
  (params (OtherActor :type Actor%20Object%20Reference)))

(event EventTick
  (params (DeltaSeconds :type Float%20%28single-precision%29)))

(fn ConstructionScript
  (|CallParentFunction))

(fn RegularComboSwapper
  ;[1 1 1] This is the parent function (can be changed if using only one combo)
  (switch int (Variables|Default|GetLocal%20Index%20Attack%20Combo)
    (:0
      (Variables|Default|SetLocal%20Index%20Attack%20Combo 1)
      (CallFunction|RegularCombo1))
    (:1
      (Variables|Default|SetLocal%20Index%20Attack%20Combo 2)
      (CallFunction|RegularCombo2))
    (:2
      (Variables|Default|SetLocal%20Index%20Attack%20Combo 0)
      (CallFunction|RegularCombo3))))

(fn ChargedAttackFunction
  (params (Charged%20Amount :type Float%20%28double-precision%29))
  (|CallParentFunction Charged%20Amount))

(fn RegularCombo1
  (CallFunction|FireBaseAttack))

(fn RegularCombo2)

(fn RegularCombo3)

(fn FireBaseAttack
  (Game|SpawnActorfromClass "/Game/Weapons/BP_BaseProjectile.BP_BaseProjectile_C" (Transformation|GetWorldTransform (Variables|Default|GetArrow)) "AlwaysSpawn" "MultiplyWithRoot" 0 0))

(fn ChargedAttackScaling
  (params (Charged%20Amount :type Float%20%28double-precision%29)))