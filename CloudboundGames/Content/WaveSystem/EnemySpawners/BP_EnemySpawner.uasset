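; BP_EnemySpawner is a wave-system spawner that holds a queue of enemy classes and spawns them at its own transform.
; Queued enemies spawn immediately if no enemy overlaps its collision sphere, while a looping timer also attempts spawns without that check.
; It binds to each spawned enemy's death event, has a handler that reports eliminations to the wave game mode, and can destroy all tracked enemies.
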(event Custom|OnEnemyEliminated
  (Default|OnEnemyEliminated (CallFunction|GetWaveGameMode)))

(event Custom|TrySpawnEnemy
  (CallFunction|SpawnEnemy))

(event Custom|ClearAllEnemies
  (for _array_element (Variables|Default|GetSpawnedEnemies)
    (Utilities|IsValid _array_element
      (:Is%20Valid
        (Actor|DestroyActor _array_element)))))

(event EventBeginPlay
  (Utilities|Time|SetTimerbyEvent (delegate Custom|TrySpawnEnemy) 5.0 true))

(fn ConstructionScript)

(fn SpawnEnemy
  (if (Utilities|Array|IsValidIndex (Variables|Default|GetEnemyQueue))
    (bind _returnvalue (Game|SpawnActorfromClass (Utilities|Array|Get(acopy) (Variables|Default|GetEnemyQueue)) (Transformation|GetActorTransform) "AdjustIfPossibleButAlwaysSpawn" "MultiplyWithRoot" 0 0))
    (Utilities|IsValid _returnvalue
      (:Is%20Valid
        (EventDispatchers|BindEventtoOnEnemyDeath _returnvalue (EventDispatchers|CreateEvent :!event Custom|OnEnemyEliminated))
        (Utilities|Array|RemoveIndex (Variables|Default|GetEnemyQueue))
        (Utilities|Array|Add (Variables|Default|GetSpawnedEnemies) _returnvalue)
        (return true)))
    (else
      (return false))))

(fn AddEnemytoQueue
  (params (EnemyClass :type BP%20Enemy%20Base%20Class%20Reference%20%28by%20ref%29))
  (Utilities|Array|Add (Variables|Default|GetEnemyQueue) EnemyClass)
  (if (not (Utilities|Array|IsValidIndex (Collision|GetOverlappingActors (Variables|Default|GetSphereCollision) "/Game/Enemy/BP_Enemy_Base.BP_Enemy_Base_C" :!class /Script/Engine.PrimitiveComponent)))
    (CallFunction|SpawnEnemy)))