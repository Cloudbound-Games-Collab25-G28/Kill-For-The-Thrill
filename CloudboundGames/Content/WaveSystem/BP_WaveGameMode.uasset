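; Wave game mode that alternates timed interludes with enemy waves and shows a win widget after the last.
; Each wave loads its enemy pool from the data table row matching its number, then queues random picks at random spawners, capped by an enemy limit.
; Kills drive refills or end the wave, as can a countdown whose starting time grows per wave.
; Event dispatchers broadcast wave, kill and timer changes.
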(event Custom|StartTimer
  ;[1 1 1] WaveTimer
  (if (== (Variables|Time|GetSeconds) 0)
    (if (== (Variables|Time|GetMinutes) 0)
      (Utilities|FlowControl|DoOnce false
        (:Completed
          (if (not (Variables|Default|GetOnBreak))
            (CallFunction|Interlude))))
      (else
        (Variables|Time|SetSeconds 59)
        (Variables|Time|SetMinutes (- (Variables|Time|GetMinutes) 1))
        (Default|CallOnTimerUpdate (Variables|Time|GetMinutes) (Variables|Time|GetSeconds) :!label _label)))
    (else
      (Variables|Time|SetSeconds (- (Variables|Time|GetSeconds) 1))
      (goto _label))))

(event Custom|BeginNextWave
  (Variables|Default|SetOnBreak false)
  (CallFunction|StartWave))

(event Custom|Interlude
  (bind _wavenumber (Variables|Default|GetWaveNumber))
  (Variables|Default|SetOnBreak true)
  (CallFunction|EndWave)
  (Math|Integer|IncrementInt _wavenumber
    (:%20%20
      (if (<= _wavenumber (Variables|Default|GetTotalWaves))
        (bind _returnvalue (Utilities|Time|SetTimerbyEvent (delegate Custom|BeginNextWave) (Variables|Default|GetInterludeDuration)))
        (Variables|Default|SetInterludeTimer _returnvalue)
        (else
          (CallFunction|GameWon))))))

(event Custom|ResetTimer
  ;[1 1 1] WaveTimer
  (Utilities|FlowControl|DoOnce false) ; enters at Reset
)

(event EventBeginPlay
  (CallFunction|SetupWaves)
  (CallFunction|Interlude))

(fn ConstructionScript)

(fn OnEnemyEliminated
  (Math|Integer|DecrementInt (Variables|Default|GetEnemiesRemaning)
    (:%20%20
      (bind _result (Math|Integer|IncrementInt (Variables|Default|GetEnemiesKilled))
        (:%20%20
          (Default|CallOnEnemyKilled _result (Variables|Default|GetTotalEnemies))
          (if (< (Variables|Default|GetEnemiesRemaning) (Variables|Default|GetEnemyLimit))
            (if (<= (Variables|Default|GetEnemiesRemaning) 0)
              (CallFunction|Interlude))
            (else
              (CallFunction|AddEnemytoQueue))))))))

(fn AddEnemytoQueue
  (Default|AddEnemytoQueue (.OutItem (Utilities|Array|Random (Variables|Default|GetEnemySpawners))) (CallFunction|GetEnemyfromPool)))

(fn GetEnemySpawners
  (bind _outactors (Actor|GetAllActorsOfClass "/Game/WaveSystem/EnemySpawners/BP_EnemySpawner.BP_EnemySpawner_C"))
  (Variables|Default|SetEnemySpawners _outactors))

(fn GetEnemyfromPool
  ;[1 1 1] Gets a radom enemy from the pool, and then have functionality for adding or removing the enemy form that pool
  (bind _keys (Utilities|Map|Keys (Variables|Default|GetEnemyPool)))
  (bind _output_get (LocalVariables|SetLocal_EnemyClass (.OutItem (Utilities|Array|Random _keys))))
  (if (<= (- (.Value (Utilities|Map|Find (Variables|Default|GetEnemyPool) _output_get)) 1) 0)
    (Utilities|Map|Remove (Variables|Default|GetEnemyPool) (LocalVariables|GetLocal_EnemyClass))
    (else
      (Utilities|Map|Add (Variables|Default|GetEnemyPool) (LocalVariables|GetLocal_EnemyClass) (- (.Value (Utilities|Map|Find (Variables|Default|GetEnemyPool) _output_get)) 1))
      (return (LocalVariables|GetLocal_EnemyClass)))))

(fn StartWave
  (Development|PrintString "Wave Started")
  (CallFunction|WaveClock)
  (CallFunction|BuildWave)
  (Default|CallOnStartWave (Variables|Default|GetWaveNumber) (Variables|Default|GetEnemiesKilled) (Variables|Default|GetTotalEnemies) (Variables|Default|GetMaterialsCollected))
  (CallFunction|ResetTimer))

(fn EndWave
  (Variables|Default|SetEnemiesKilled 0)
  (Variables|Time|SetMinutes 0)
  (Variables|Time|SetSeconds 0)
  (for _array_element (Variables|Default|GetEnemySpawners)
    (Default|ClearAllEnemies _array_element))
  (Default|CallOnWaveEnd))

(fn GetPoolSize
  ;[1 1 1] Gets the Size of the pool
  (bind _values (Utilities|Map|Values (Variables|Default|GetEnemyPool)))
  (return (Utilities|Array|Length _values)))

(fn BuildEnemyPool
  (bind _enemypoolsize (CallFunction|GetPoolSize))
  ;[1 1 1] Gets the information out of the data table
  (bind _returnvalue (Utilities|GetDataTableRow (Variables|Default|GetEnemyDataTable) (Utilities|String|StringToName (Utilities|String|ToString(Integer) (Variables|Default|GetWaveNumber))))
    (:then
      (Variables|Default|SetEnemyPool (Utilities|Struct|BreakS_WaveInfo _returnvalue))
      (Variables|Default|SetEnemiesRemaning _enemypoolsize)
      (Variables|Default|SetTotalEnemies _enemypoolsize))))

(fn GameWon
  (bind _returnvalue (UserInterface|CreateWidget (Variables|Default|GetWinWidgetType) (Game|GetPlayerController 0)))
  (Viewport|RemoveAllWidgets)
  (UserInterface|Viewport|AddtoViewport _returnvalue 0))

(fn BuildWave
  (CallFunction|BuildEnemyPool)
  (for _index (range 0 (- (Math|Integer|Min(Integer) (CallFunction|GetPoolSize) (Variables|Default|GetEnemyLimit)) 1))
    (CallFunction|AddEnemytoQueue)))

(fn CountDownTimer
  (Utilities|Time|SetTimerbyEvent (EventDispatchers|CreateEvent :!event Custom|StartTimer) 1.0 true)
  (return (Variables|Time|GetMinutes) (Variables|Time|GetSeconds)))

(fn WaveClock
  (bind _output_get (Variables|Time|SetStoredSeconds (+ (Variables|Time|GetStoredSeconds) 20)))
  (if (>= _output_get 60)
    (Variables|Time|SetStoredSeconds 0)
    (bind _result (Math|Integer|IncrementInt (Variables|Time|GetStoredMinutes))
      (:%20%20
        (Variables|Time|SetMinutes _result)))
    (else
      (Variables|Time|SetStoredSeconds (Variables|Time|GetStoredSeconds))
      (Variables|Time|SetMinutes (Variables|Time|GetStoredMinutes)))))

(fn SetupWaves
  (CallFunction|GetEnemySpawners)
  ;[1 1 1] Get the number of rows in the data table - needs memory optimisation
  (bind _outrownames (DataTable|GetDataTableRowNames (Variables|Default|GetEnemyDataTable)))
  (Variables|Default|SetTotalWaves (Utilities|Array|Length _outrownames)))