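; BP_DebugComponent is a player-side Blueprint that toggles the game's pause menu from the IA_PauseGame input action or a T debug key.
; Opening creates a fresh WBP_PauseMenu, focuses it in Game and UI input mode with the cursor shown, pauses the game and plays a sound.
; Closing removes the stored widget, restores game-only input, hides the cursor and unpauses.
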(event Input|EnhancedActionEvents|EnhancedInputActionIA_PauseGame
  (params (ActionValue :type Boolean) (ElapsedSeconds :type Float%20%28double-precision%29) (TriggeredSeconds :type Float%20%28double-precision%29) (InputAction :type Input%20Action%20Object%20Reference :default "/Game/Tech/Input/Actions/IA_PauseGame.IA_PauseGame"))
  ;[0 0 0] Toggle pause menu
  (if (not (Variables|Default|GetbIsPauseMenuOpen))
    (CallFunction|OpensPauseMenu)
    (Audio|PlaySound2D "/Game/Audio/ui/Pause_tone/pause.pause" 1.0 1.0 0.0 0 0)
    (else
      (CallFunction|ClosesPauseMenu))))

(event Input|KeyboardEvents|DebugKeyT
  (params (Key :type Key%20Structure :default "None") (ActionValue :type Input%20Action%20Value%20Structure))
  ;[0 0 0] Toggle pause menu
  (:Pressed
    (if (not (Variables|Default|GetbIsPauseMenuOpen))
      (CallFunction|OpensPauseMenu)
      (Audio|PlaySound2D "/Game/Audio/ui/Pause_tone/pause.pause" 1.0 1.0 0.0 0 0)
      (else
        (CallFunction|ClosesPauseMenu)))))

(fn ClosesPauseMenu
  (bind _returnvalue (Game|GetPlayerController 0))
  ;[0 0 0] Closes pause menu and hides cursor
  (Variables|Default|SetbIsPauseMenuOpen false)
  (Widget|RemovefromParent (Variables|Default|GetPauseMenuREF))
  (Input|SetInputModeGameOnly _returnvalue false)
  (Variables|/Script/Engine.PlayerController|SetbShowMouseCursor _returnvalue false)
  (Game|SetGamePaused false))

(fn OpensPauseMenu
  (bind _returnvalue (Game|GetPlayerController 0))
  ;[0 0 0] Open pause menu and activate mouse cursor
  (Variables|Default|SetbIsPauseMenuOpen true)
  (bind _returnvalue_2 (UserInterface|CreateWidget "/Game/Tech/UI/Menus/WBP_PauseMenu.WBP_PauseMenu_C"))
  (bind _output_get (Variables|Default|SetPauseMenuREF _returnvalue_2))
  (UserInterface|Viewport|AddtoViewport _output_get 0)
  (Input|SetInputModeGameandUI _returnvalue _output_get "DoNotLock" true false)
  (Variables|/Script/Engine.PlayerController|SetbShowMouseCursor _returnvalue true)
  (Game|SetGamePaused true))