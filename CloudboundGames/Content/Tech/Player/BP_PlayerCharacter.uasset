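; Player character Blueprint built from components for combat, upgradeable health, dodge roll, lives and attack tokens.
; Pressing E opens an overlapping BP_Trader's shop, and ItemGet applies the chosen item: more max health, refreshed lives or a full heal.
; The attack token count is set at construction, with reserve and return calls forwarded to that component.
; SetupAudioEvents binds handlers to combat, health, roll and life events.
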(event Custom|ItemGet
  (params (ChosenShopItem :type E_ShopItems%20Enum :default "NewEnumerator0"))
  (bind _bpc_upgradeablehealth (Variables|Default|GetBPC_UpgradeableHealth))
  (bind _bpc_upgradeablehealth_2 (Variables|Default|GetBPC_UpgradeableHealth))
  ;[1 0.5918 0.07549] Gets the Item From the Shop
  (switch Utilities|FlowControl|Switch|SwitchonE_ShopItems ChosenShopItem
    (:NewEnumerator0
      ;[0.8549 0.09412 0.09412] Increase Max Health
      (bind _output_get (Variables|/Script/CloudboundGames.HealthComponent|SetMaxHealth _bpc_upgradeablehealth_2 (+ (Variables|/Script/CloudboundGames.HealthComponent|GetMaxHealth _bpc_upgradeablehealth_2) (Variables|Default|GetMaxHealthIncrease))))
      (Class|HealthComponent|SetMaxHealth _bpc_upgradeablehealth_2 _output_get))
    (:NewEnumerator1
      ;[0.8549 0.09412 0.09412] Refresh Lives
      (Class|LivesComponent|SetLives (Variables|Default|GetLives) (Variables|Default|GetDesiredAmountOfLives)))
    (:NewEnumerator2
      ;[0.8549 0.09412 0.09412] RefreshHealth
      (Default|HealHealth _bpc_upgradeablehealth (Variables|/Script/CloudboundGames.HealthComponent|GetMaxHealth _bpc_upgradeablehealth)))))

(event EventReturnAttackToken
  (params (Amount :type Integer))
  (Default|ReturnAttackTokens (Variables|Default|GetBPC_AttackToken) Amount))

(event Input|KeyboardEvents|E
  (params (Key :type Key%20Structure :default "None"))
  ;[1 0.7539 0.07181] Checks if the player is near the trader
  (:Pressed
    (for _array_element (Collision|GetOverlappingActors 0 :!class /Script/Engine.Actor)
      (bind _asbp_trader (Utilities|Casting|CastToBP_Trader _array_element))
      (Default|OpenShop _asbp_trader))))

(fn ConstructionScript
  (Variables|/Game/Tech/AI/BPC_AttackToken.BPC_AttackToken_C|SetAttackTokenCount (Variables|Default|GetBPC_AttackToken) (Variables|AttackToken|GetAttack%20Token%20Count)))

(fn SetupAudioEvents
  (bind _dodgerollcomponent (Variables|Default|GetDodgeRollComponent))
  (bind _bpc_upgradeablehealth (Variables|Default|GetBPC_UpgradeableHealth))
  (bind _lives (Variables|Default|GetLives))
  ;[1 1 1] Combat
  (EventDispatchers|BindEventtoOnAttack (Variables|Default|GetBPC_CharacterCombatV2) (EventDispatchers|CreateEvent (Variables|Default|GetBPC_PlayerSFX) :!event OnAttack))
  ;[1 1 1] Health
  (EventDispatchers|BindEventtoOnDamageTaken _bpc_upgradeablehealth (EventDispatchers|CreateEvent (Variables|Default|GetBPC_PlayerSFX) :!event OnDamaged))
  (EventDispatchers|BindEventtoOnDamageBlocked _bpc_upgradeablehealth (EventDispatchers|CreateEvent (Variables|Default|GetBPC_PlayerSFX) :!event OnDamageBlocked))
  (EventDispatchers|BindEventtoOnKilled _bpc_upgradeablehealth (EventDispatchers|CreateEvent (Variables|Default|GetBPC_PlayerSFX) :!event OnKilled))
  (EventDispatchers|BindEventtoOnHealthHealed _bpc_upgradeablehealth (EventDispatchers|CreateEvent (Variables|Default|GetBPC_PlayerSFX) :!event OnHealed))
  ;[1 1 1] Dodge/Roll
  (EventDispatchers|BindEventtoOnRollStarted _dodgerollcomponent (EventDispatchers|CreateEvent (Variables|Default|GetBPC_PlayerSFX) :!event OnRollTriggered))
  (EventDispatchers|BindEventtoOnRollRecovered _dodgerollcomponent (EventDispatchers|CreateEvent (Variables|Default|GetBPC_PlayerSFX) :!event OnRollRecovered))
  ;[1 1 1] Lives
  (EventDispatchers|BindEventtoOnLifeLost _lives (EventDispatchers|CreateEvent (Variables|Default|GetBPC_PlayerSFX) :!event OnLifeLost))
  (EventDispatchers|BindEventtoOnAllLivesLost _lives (EventDispatchers|CreateEvent (Variables|Default|GetBPC_PlayerSFX) :!event OnAllLivesLost)))

(fn ReserveAttackToken
  (params (Amount :type Integer))
  (bind _success (Default|ReserveAttackTokens (Variables|Default|GetBPC_AttackToken) Amount))
  (return _success))