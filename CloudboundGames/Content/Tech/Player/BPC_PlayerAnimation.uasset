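; Player animation component that plays one-shot montages on its owner's skeletal mesh in reaction to combat events.
; On BeginPlay it caches the mesh, HealthComponent and BPC_CharacterCombatV2, then binds to kill, damage and attack delegates.
; Death, hit reaction and attack each trigger their own montage, keeping animation event-driven and separate from health and combat logic.
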(event Custom|On%20Take%20Any%20Damage
  (params (DamagedActor :type Actor%20Object%20Reference) (Damage :type Float%20%28single-precision%29) (DamageType :type Damage%20Type%20Object%20Reference) (InstigatedBy :type Controller%20Object%20Reference) (DamageCauser :type Actor%20Object%20Reference))
  (Animation|Montage|PlayMontage (Variables|Default|GetSkeletalMeshComponent) (Variables|Default|GetDamagedMontage)))

(event Custom|On%20Killed
  (params (HealthComponent :type Health%20Component%20Object%20Reference))
  (Animation|Montage|PlayMontage (Variables|Default|GetSkeletalMeshComponent) (Variables|Default|GetDeathMontage)))

(event Custom|OnAttack
  (Animation|Montage|PlayMontage (Variables|Default|GetSkeletalMeshComponent) (Variables|Default|GetAttackMontage)))

(event EventBeginPlay
  (bind _returnvalue (Components|GetOwner))
  ;[1 1 1] Cache Player Components
  (Variables|Default|SetSkeletalMeshComponent (Actor|GetComponentbyClass _returnvalue "/Script/Engine.SkeletalMeshComponent"))
  (bind _output_get (Variables|Default|SetHealthComponent (Actor|GetComponentbyClass _returnvalue "/Script/CloudboundGames.HealthComponent")))
  (EventDispatchers|BindEventtoOnKilled _output_get (delegate Custom|On%20Killed))
  (EventDispatchers|BindEventtoOnTakeAnyDamage _returnvalue (delegate Custom|On%20Take%20Any%20Damage))
  (bind _output_get_2 (Variables|Default|SetWeaponComponent (Actor|GetComponentbyClass _returnvalue "/Game/Tech/Weapons/BPC_CharacterCombatV2.BPC_CharacterCombatV2_C")))
  (EventDispatchers|BindEventtoOnAttack _output_get_2 (EventDispatchers|CreateEvent :!event Custom|OnAttack)))