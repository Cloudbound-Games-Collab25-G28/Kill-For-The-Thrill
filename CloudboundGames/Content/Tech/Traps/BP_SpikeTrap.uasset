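; BP_SpikeTrap is a trap that repeatedly damages actors standing inside its Box trigger.
; An overlap while armed applies DamageToApply to every overlapping actor, disarms the trap and starts a timer at DamageTickTime.
; When the timer fires, it clears itself, re-arms the trap and repeats the damage pass if any actors remain inside.
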(event OnComponentBeginOverlap(Box)
  (params (OverlappedComponent :type Primitive%20Component%20Object%20Reference) (OtherActor :type Actor%20Object%20Reference) (OtherComp :type Primitive%20Component%20Object%20Reference) (OtherBodyIndex :type Integer) (bFromSweep :type Boolean) (SweepResult :type Hit%20Result%20Structure%20%28by%20ref%29))
  (if (Variables|Default|GetisArmed)
    (for _array_element (Collision|GetOverlappingActors OverlappedComponent "/Script/Engine.Actor" :!class /Script/Engine.PrimitiveComponent)
      (CallFunction|ApplyDamage _array_element)
      (Variables|Default|SetisArmed false)
      (bind _returnvalue (Utilities|Time|SetTimerbyEvent (delegate Custom|ApplyDamageEvent) (Variables|Default|GetDamageTickTime) true))
      (Variables|Default|SetApplyDamageTImerHandle _returnvalue))))

(event Custom|ApplyDamageEvent
  (Variables|Default|SetisArmed true)
  (Utilities|Time|ClearandInvalidateTimerbyHandle (stale OnComponentBeginOverlap(Box) _returnvalue))
  (CallFunction|CheckifAnymoreActorsAreinTrap))

(event Custom|Check%20if%20anymore%20actors%20are%20in%20trap
  (if (not (Utilities|Array|IsEmpty (Collision|GetOverlappingActors (stale OnComponentBeginOverlap(Box) OverlappedComponent) "/Script/Engine.Actor" :!class /Script/Engine.PrimitiveComponent)))
    (for _array_element (Collision|GetOverlappingActors (stale OnComponentBeginOverlap(Box) OverlappedComponent) "/Script/Engine.Actor" :!class /Script/Engine.PrimitiveComponent)
      (CallFunction|ApplyDamage _array_element)
      (Variables|Default|SetisArmed false)
      (bind _returnvalue (Utilities|Time|SetTimerbyEvent (delegate Custom|ApplyDamageEvent) (Variables|Default|GetDamageTickTime) true))
      (Variables|Default|SetApplyDamageTImerHandle _returnvalue))))

(fn ConstructionScript)

(fn ApplyDamage
  (params (DamagedActor :type Actor%20Object%20Reference))
  (Game|Damage|ApplyDamage DamagedActor (Variables|Default|GetDamageToApply) 0 0))