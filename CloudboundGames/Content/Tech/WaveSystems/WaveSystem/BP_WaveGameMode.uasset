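; Game mode that runs wave-based combat, alternating timed interludes, where a trader spawns if multiple waves exist, with enemy waves until the win screen.
; Each wave loads an enemy class-to-count pool from the data table row named by wave number, queuing random picks at random spawners up to EnemyLimit.
; Kills queue more enemies once the remaining count drops below that limit, or start the next interlude at zero.
; Dispatchers broadcast wave progress, with audio events bound.
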(event Custom|BeginNextWave
  (CallFunction|StartWave))

(event Custom|Interlude
  (bind _wavenumber (Variables|Default|GetWaveNumber))
  (CallFunction|EndWave)
  (Math|Integer|IncrementInt _wavenumber
    (:%20%20
      (if (<= _wavenumber (Variables|Default|GetTotalWaves))
        (Utilities|Time|SetTimerbyEvent (delegate Custom|BeginNextWave) (Variables|Default|GetInterludeDuration))
        (else
          (CallFunction|GameWon))))))

(event EventBeginPlay
  (CallFunction|SetupWaves)
  (CallFunction|SetupAudioEvents)
  (if (Utilities|Array|IsNotEmpty (Variables|Default|GetEnemySpawners))
    (CallFunction|Interlude)))

(event EventApplyWeapon
  (params (Class :type EWeaponType%20Enum :default "SWORD"))
  (|CallParentFunction Class)
  (Default|SelectWeapon (Actor|GetComponentbyClass (Variables|/Script/CloudboundGames.TP_TopDownPlayerController|GetPlayerPawn (Variables|Default|GetPlayerController)) "/Game/Tech/Weapons/BPC_CharacterCombatV2.BPC_CharacterCombatV2_C") Class))

(fn ConstructionScript)

(fn OnEnemyEliminated
  (Math|Integer|DecrementInt (Variables|Default|GetEnemiesRemaning)
    (:%20%20
      (bind _result (Math|Integer|IncrementInt (Variables|Default|GetEnemiesKilled))
        (:%20%20
          (Default|CallOnEnemyKilled _result (Variables|Default|GetTotalEnemies))
          (if (< (Variables|Default|GetEnemiesRemaning) (Variables|Default|GetEnemyLimit))
            (if (<= (Variables|Default|GetEnemiesRemaning) 0)
              (CallFunction|Interlude)
              (else
                (CallFunction|AddEnemytoQueue)))))))))

(fn AddEnemytoQueue
  (bind _output_get (LocalVariables|SetCachedEnemyClass (CallFunction|GetEnemyfromPool)))
  (if (Utilities|IsValidClass _output_get)
    (Default|AddEnemytoQueue (.OutItem (Utilities|Array|Random (Variables|Default|GetEnemySpawners))) _output_get)))

(fn GetEnemySpawners
  (bind _outactors (Actor|GetAllActorsOfClass "/Game/Tech/WaveSystems/WaveSystem/EnemySpawners/BP_EnemySpawner.BP_EnemySpawner_C"))
  (Variables|Default|SetEnemySpawners _outactors))

(fn GetEnemyfromPool
  ;[1 1 1] Gets a radom enemy from the pool, and then have functionality for adding or removing the enemy form that pool
  (bind _keys (Utilities|Map|Keys (Variables|Default|GetEnemyPool)))
  (if (>= (.OutIndex (Utilities|Array|Random _keys)) 0)
    (bind _output_get (LocalVariables|SetLocal_EnemyClass (.OutItem (Utilities|Array|Random _keys))))
    (if (<= (- (.Value (Utilities|Map|Find (Variables|Default|GetEnemyPool) _output_get)) 1) 0)
      (Utilities|Map|Remove (Variables|Default|GetEnemyPool) (LocalVariables|GetLocal_EnemyClass))
      (else
        (Utilities|Map|Add (Variables|Default|GetEnemyPool) (LocalVariables|GetLocal_EnemyClass) (- (.Value (Utilities|Map|Find (Variables|Default|GetEnemyPool) _output_get)) 1))))
    (return (LocalVariables|GetLocal_EnemyClass))
    (else
      (return 0))))

(fn StartWave
  (bind _wavenumber (Variables|Default|GetWaveNumber))
  (Actor|DestroyActor (Variables|Default|GetTrader%20Reference))
  (Development|PrintString "Wave Started")
  (CallFunction|BuildWave)
  (Default|CallOnWaveStart _wavenumber (Variables|Default|GetEnemiesKilled) (Variables|Default|GetTotalEnemies) (Variables|Default|GetMaterialsCollected))
  (if (>= _wavenumber (Variables|Default|GetTotalWaves))
    (Default|CallOnLastWave)))

(fn EndWave
  (Variables|Default|SetEnemiesKilled 0)
  (for _array_element (Variables|Default|GetEnemySpawners)
    (Default|ClearAllEnemies _array_element))
  (Default|CallOnWaveEnd)
  (if (> (Variables|Default|GetTotalWaves) 1)
    (bind _returnvalue (Game|SpawnActorfromClass "/Game/Tech/ShopSystem/Shop-Widgets/BP_Trader.BP_Trader_C" (Math|Transform|MakeTransform "0, 0, 0" "0, 0, 0" "1.000000,1.000000,1.000000") "Undefined" "MultiplyWithRoot" 0 0))
    (bind _output_get (Variables|Default|SetTrader%20Reference _returnvalue))
    (Utilities|IsValid _output_get
      (:Is%20Valid
        (Development|PrintString "Trader has spawned in")))))

(fn GetPoolSize
  ;[1 1 1] Gets the Size of the pool
  (bind _values (Utilities|Map|Values (Variables|Default|GetEnemyPool)))
  (for _array_element _values
    (LocalVariables|SetLocal_EnemyPool (+ _array_element (LocalVariables|GetLocal_EnemyPool))))
  (return (LocalVariables|GetLocal_EnemyPool)))

(fn BuildEnemyPool
  (bind _enemypoolsize (CallFunction|GetPoolSize))
  ;[1 1 1] Gets the information out of the data table
  (bind _returnvalue (Utilities|GetDataTableRow (Variables|Default|GetEnemyDataTable) (Utilities|String|StringToName (Utilities|String|ToString(Integer) (Variables|Default|GetWaveNumber))))
    (:then
      (Variables|Default|SetEnemyPool (Utilities|Struct|BreakS_WaveInfo _returnvalue))
      (Variables|Default|SetEnemiesRemaning _enemypoolsize)
      (Variables|Default|SetTotalEnemies _enemypoolsize))))

(fn GameWon
  (bind _returnvalue (UserInterface|CreateWidget (Variables|Default|GetWinWidgetType) (Game|GetPlayerController 0)))
  (Viewport|RemoveAllWidgets)
  (UserInterface|Viewport|AddtoViewport _returnvalue 0)
  (Default|CallOnGameWon))

(fn BuildWave
  (CallFunction|BuildEnemyPool)
  (bind _output_get (LocalVariables|SetLocalLimit (- (Math|Integer|Min(Integer) (CallFunction|GetPoolSize) (Variables|Default|GetEnemyLimit)) 1)))
  (for _index (range 0 _output_get)
    (CallFunction|AddEnemytoQueue)))

(fn SetupWaves
  (CallFunction|GetEnemySpawners)
  ;[1 1 1] Get the number of rows in the data table - needs memory optimisation
  (bind _outrownames (DataTable|GetDataTableRowNames (Variables|Default|GetEnemyDataTable)))
  (Variables|Default|SetTotalWaves (Utilities|Array|Length _outrownames)))

(fn SetupAudioEvents
  (EventDispatchers|BindEventtoOnLastWave (EventDispatchers|CreateEvent (Variables|Default|GetMusicPlayer) :!event OnLastWave))
  (EventDispatchers|BindEventtoOnWaveEnd (EventDispatchers|CreateEvent (Variables|Default|GetMusicPlayer) :!event OnInterludeStart))
  (EventDispatchers|BindEventtoOnWaveStart (EventDispatchers|CreateEvent (Variables|Default|GetMusicPlayer) :!event OnWaveStart))
  (EventDispatchers|BindEventtoOnGameWon (EventDispatchers|CreateEvent (Variables|Default|GetMusicPlayer) :!event OnWon))
  (EventDispatchers|BindEventtoOnGameOver (EventDispatchers|CreateEvent (Variables|Default|GetMusicPlayer) :!event OnLost)))

(fn RemoveCurrency
  (params (RemovedCurrency :type Integer))
  (Variables|Default|SetMaterialsCollected (- (Variables|Default|GetMaterialsCollected) RemovedCurrency)))