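; Enemy spawner actor for the wave system that spawns queued enemy classes at its own transform.
; Queuing an enemy spawns the queue head immediately if no enemy overlaps the sphere, while a looping timer also retries periodically without that check.
; Enemies with a health component are dequeued, tracked and bound to a kill event.
; Eliminations update the tracked list and notify the wave game mode; a separate event destroys all tracked enemies.
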(event Custom|OnEnemyEliminated
  (params (HealthComponent :type Health%20Component%20Object%20Reference))
  (bind _asbp_enemy_base (Utilities|Casting|CastToBP_Enemy_Base (Components|GetOwner HealthComponent))
    (:then
      (Utilities|Array|RemoveItem (Variables|Default|GetSpawnedEnemies) _asbp_enemy_base))
    (:CastFailed
      _))
  (Default|OnEnemyEliminated (CallFunction|GetWaveGameMode)))

(event Custom|TrySpawnEnemy
  (CallFunction|SpawnEnemy))

(event Custom|ClearAllEnemies
  ;[1 1 1] Clear enemy function for timer
  (for _array_element (Variables|Default|GetSpawnedEnemies)
    (Utilities|IsValid _array_element
      (:Is%20Valid
        (Actor|DestroyActor _array_element)))))

(event EventBeginPlay
  (Utilities|Time|SetTimerbyEvent (delegate Custom|TrySpawnEnemy) 5.0 true))

(fn ConstructionScript)

(fn SpawnEnemy
  (bind _enemyqueue (Variables|Default|GetEnemyQueue))
  (bind _output (Utilities|Array|Get(acopy) _enemyqueue))
  ;[1 1 1] This blueprint checks if the index for the enemys are valid and have functionality for getting all enemies within the array
  (if (Utilities|Array|IsValidIndex (Variables|Default|GetEnemyQueue))
    (LocalVariables|SetEnemyClass _output)
    (bind _returnvalue (Game|SpawnActorfromClass _output (Transformation|GetActorTransform) "AdjustIfPossibleButAlwaysSpawn" "MultiplyWithRoot" 0 0))
    (Utilities|IsValid _returnvalue
      (:Is%20Valid
        (Pawn|SpawnDefaultController _returnvalue)
        (Utilities|IsValid (Actor|GetComponentbyClass _returnvalue "/Script/CloudboundGames.HealthComponent")
          (:Is%20Valid
            (EventDispatchers|BindEventtoOnKilled (Actor|GetComponentbyClass _returnvalue "/Script/CloudboundGames.HealthComponent") (EventDispatchers|CreateEvent :!event Custom|OnEnemyEliminated))
            (Utilities|Array|RemoveIndex (Variables|Default|GetEnemyQueue))
            (Utilities|Array|Add (Variables|Default|GetSpawnedEnemies) _returnvalue)
            (Default|CallOnEnemySpawned (LocalVariables|GetEnemyClass))
            (return true))
          (:Is%20Not%20Valid
            _)))
      (:Is%20Not%20Valid
        _))
    (return false)
    (else
      (return false))))

(fn AddEnemytoQueue
  (params (EnemiesClass :type BP%20Enemy%20Base%20Class%20Reference%20%28by%20ref%29))
  ;[1 1 1] Checks if spawning is valid before spawning enemy
  (Utilities|Array|Add (Variables|Default|GetEnemyQueue) EnemiesClass)
  (if (not (Utilities|Array|IsValidIndex (Collision|GetOverlappingActors (Variables|Default|GetSphereCollision) "/Game/Tech/AI/BP_Enemy_Base.BP_Enemy_Base_C" :!class /Script/Engine.PrimitiveComponent)))
    (CallFunction|SpawnEnemy)))