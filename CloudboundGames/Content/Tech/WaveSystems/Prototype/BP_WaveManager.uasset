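; Prototype wave manager that runs timed enemy waves until a maximum count is cleared, then fires a game-won event.
; A timer paces waves, and each wave start broadcasts an event and has every spawner spawn the configured class, passing the manager along.
; Spawned actors with a BPC_Health component are counted and bound to its kill event.
; When the alive count reaches zero, the next timer starts or the game is won.
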(event Custom|TimerToNextWave
  (bind _returnvalue (Utilities|Time|SetTimerbyEvent (EventDispatchers|CreateEvent :!event Custom|StartWave) (Variables|Default|GetTimeToNextWave)))
  (Variables|Default|SetTimeToNextWaveHandle _returnvalue))

(event Custom|StartWave
  (bind _output_get (Variables|Default|SetWaveNumber (+ 1 (Variables|Default|GetWaveNumber))))
  (Development|PrintString (Utilities|String|ToString(Text) (Utilities|Text|FormatText "Wave {Number}" _output_get)) true true "(R=0.932556,G=0.000000,B=1.000000,A=1.000000)")
  (Default|CallEStartWave)
  (for _array_element (Variables|Default|GetSpawners)
    (Default|SpawnClass _array_element (Variables|Default|GetActor%20to%20Spawn) self)))

(event Custom|Event%20Wave%20End
  (if (> (Variables|Default|GetMaxWaves) (Variables|Default|GetWaveNumber))
    (CallFunction|TimertoNextWave)
    (else
      (Default|CallOnGameWon))))

(event Custom|Event%20Enemy%20Dead
  (params (HealthComponent :type Health%20Component%20Object%20Reference))
  (bind _aliveenemynumber (Variables|Default|GetAliveEnemyNumber))
  (Math|Integer|DecrementInt _aliveenemynumber
    (:%20%20
      (if (<= _aliveenemynumber 0)
        (CallFunction|EventWaveEnd)))))

(event EventBeginPlay
  (CallFunction|TimertoNextWave))

(event EventSpawnedActor
  (params (SpawnedActor :type Actor%20Object%20Reference))
  (bind _returnvalue (Actor|GetComponentbyClass SpawnedActor "/Game/Tech/BPC_Health.BPC_Health_C"))
  (bind _aliveenemynumber (Variables|Default|GetAliveEnemyNumber))
  (Utilities|Array|Add (Variables|Default|GetSpawned%20Actor) SpawnedActor)
  (if (Utilities|IsValid _returnvalue)
    (EventDispatchers|BindEventtoOnKilled _returnvalue (delegate Custom|Event%20Enemy%20Dead))
    (Math|Integer|IncrementInt _aliveenemynumber
      (:%20%20
        (Development|PrintString (Utilities|String|ToString(Text) (Utilities|Text|FormatText "Enemy {Number}" _aliveenemynumber)) true true "(R=0.932556,G=0.000000,B=1.000000,A=1.000000)")))))

(fn ConstructionScript)