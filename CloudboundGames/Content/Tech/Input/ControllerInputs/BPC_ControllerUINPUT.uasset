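; Controller component that routes gamepad UI navigation and switches between mouse and gamepad input modes.
; Face buttons, D-pad and left stick send confirm, back and directional messages to the UI reference supplied through SendCurrentUIReference.
; The weapon attack action shows the cursor and flags controller input disabled; any handled gamepad press hides it and clears the flag.
; Two DoOnce gates reset each other, so each switch fires once per device change.
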(event Custom|Send%20Current%20UI%20Reference
  (params (Current%20UI%20Reference :type Widget%20Object%20Reference))
  (Variables|Default|SetCurrent%20UI%20Reference Current%20UI%20Reference))

(event Custom|DISABLE%20MOUSE%20CONTROLLS%20FULLY
  (bind _returnvalue (Game|GetPlayerController 0))
  (Utilities|FlowControl|DoOnce false
    (:Completed
      (Utilities|FlowControl|Sequence
        (:then_0
          (Development|PrintString "Mouse Disabled")
          (Variables|Default|SetDisabled%20controller%20input? false)
          (Variables|/Script/Engine.PlayerController|SetbEnableClickEvents _returnvalue false)
          (Variables|/Script/Engine.PlayerController|SetbShowMouseCursor _returnvalue false)
          (Input|SetInputModeGameandUI _returnvalue 0 "LockAlways" true false)
          (Class|WidgetBlueprintLibrary|SetFocustoGameViewport)
          (Variables|/Script/Engine.PlayerController|SetbEnableTouchEvents _returnvalue false))
        (:then_1
          (Utilities|FlowControl|DoOnce false) ; enters at Reset
        )))))

(event Custom|DISABLE%20CONTROLLER%20CONTROLS%20FULLY
  (bind _returnvalue (Game|GetPlayerController 0))
  (Development|PrintString "Controller Disabled")
  (Variables|Default|SetDisabled%20controller%20input? true)
  (Variables|/Script/Engine.PlayerController|SetbEnableClickEvents _returnvalue true)
  (Variables|/Script/Engine.PlayerController|SetbShowMouseCursor _returnvalue true)
  (Input|SetInputModeGameandUI _returnvalue 0 "DoNotLock" false false)
  (Class|WidgetBlueprintLibrary|SetFocustoGameViewport)
  (Variables|/Script/Engine.PlayerController|SetbEnableTouchEvents _returnvalue true))

(event Input|EnhancedActionEvents|EnhancedInputActionIA_WeaponAttack_Held
  (params (ActionValue :type Boolean) (ElapsedSeconds :type Float%20%28double-precision%29) (TriggeredSeconds :type Float%20%28double-precision%29) (InputAction :type Input%20Action%20Object%20Reference :default "/Game/Tech/Input/Actions/IA_WeaponAttack_Held.IA_WeaponAttack_Held"))
  (bind _returnvalue (Game|GetPlayerController 0))
  (:Started
    (Utilities|FlowControl|DoOnce false
      (:Completed
        (Utilities|FlowControl|Sequence
          (:then_0
            (CallFunction|DISABLECONTROLLERCONTROLSFULLY))
          (:then_1
            (Utilities|FlowControl|DoOnce false) ; enters at Reset
          ))))))

(event EventBeginPlay
  (Class|WidgetBlueprintLibrary|SetFocustoGameViewport))

(event Input|GamepadEvents|GamepadDPadDown
  (params (Key :type Key%20Structure :default "None"))
  (bind _current_ui_reference (Variables|Default|GetCurrent%20UI%20Reference))
  (:Pressed
    (CallFunction|DISABLEMOUSECONTROLLSFULLY)
    (if (not (Variables|Default|GetDisabled%20controller%20input?))
      (Utilities|IsValid _current_ui_reference
        (:Is%20Valid
          (Class|BPIUIInputs|UIDown(Message) _current_ui_reference))))))

(event Input|GamepadEvents|GamepadDPadRight
  (params (Key :type Key%20Structure :default "None"))
  (bind _current_ui_reference (Variables|Default|GetCurrent%20UI%20Reference))
  (:Pressed
    (CallFunction|DISABLEMOUSECONTROLLSFULLY)
    (if (not (Variables|Default|GetDisabled%20controller%20input?))
      (Utilities|IsValid _current_ui_reference
        (:Is%20Valid
          (Class|BPIUIInputs|UIRight(Message) _current_ui_reference))))))

(event Input|GamepadEvents|GamepadDPadLeft
  (params (Key :type Key%20Structure :default "None"))
  (bind _current_ui_reference (Variables|Default|GetCurrent%20UI%20Reference))
  (:Pressed
    (CallFunction|DISABLEMOUSECONTROLLSFULLY)
    (if (not (Variables|Default|GetDisabled%20controller%20input?))
      (Utilities|IsValid _current_ui_reference
        (:Is%20Valid
          (Class|BPIUIInputs|UILeft(Message) _current_ui_reference))))))

(event Input|GamepadEvents|GamepadDPadUp
  (params (Key :type Key%20Structure :default "None"))
  (bind _current_ui_reference (Variables|Default|GetCurrent%20UI%20Reference))
  (:Pressed
    (CallFunction|DISABLEMOUSECONTROLLSFULLY)
    (if (not (Variables|Default|GetDisabled%20controller%20input?))
      (Utilities|IsValid _current_ui_reference
        (:Is%20Valid
          (Class|BPIUIInputs|UIUp(Message) _current_ui_reference))))))

(event Input|GamepadEvents|GamepadFaceButtonBottom
  (params (Key :type Key%20Structure :default "None"))
  (bind _current_ui_reference (Variables|Default|GetCurrent%20UI%20Reference))
  (:Pressed
    ;[1 1 1] Confirm Button
    (CallFunction|DISABLEMOUSECONTROLLSFULLY)
    (if (not (Variables|Default|GetDisabled%20controller%20input?))
      (Utilities|IsValid _current_ui_reference
        (:Is%20Valid
          (Class|BPIUIInputs|UIConfirm(Message) _current_ui_reference))))))

(event Input|GamepadEvents|GamepadLeftStickLeft
  (params (Key :type Key%20Structure :default "None"))
  (bind _current_ui_reference (Variables|Default|GetCurrent%20UI%20Reference))
  (:Pressed
    (CallFunction|DISABLEMOUSECONTROLLSFULLY)
    (if (not (Variables|Default|GetDisabled%20controller%20input?))
      (Utilities|IsValid _current_ui_reference
        (:Is%20Valid
          (Class|BPIUIInputs|UILeft(Message) _current_ui_reference))))))

(event Input|GamepadEvents|GamepadLeftStickDown
  (params (Key :type Key%20Structure :default "None"))
  (bind _current_ui_reference (Variables|Default|GetCurrent%20UI%20Reference))
  (:Pressed
    (CallFunction|DISABLEMOUSECONTROLLSFULLY)
    (if (not (Variables|Default|GetDisabled%20controller%20input?))
      (Utilities|IsValid _current_ui_reference
        (:Is%20Valid
          (Class|BPIUIInputs|UIDown(Message) _current_ui_reference))))))

(event Input|GamepadEvents|GamepadLeftStickRight
  (params (Key :type Key%20Structure :default "None"))
  (bind _current_ui_reference (Variables|Default|GetCurrent%20UI%20Reference))
  (:Pressed
    (CallFunction|DISABLEMOUSECONTROLLSFULLY)
    (if (not (Variables|Default|GetDisabled%20controller%20input?))
      (Utilities|IsValid _current_ui_reference
        (:Is%20Valid
          (Class|BPIUIInputs|UIRight(Message) _current_ui_reference))))))

(event Input|GamepadEvents|GamepadLeftStickUp
  (params (Key :type Key%20Structure :default "None"))
  (bind _current_ui_reference (Variables|Default|GetCurrent%20UI%20Reference))
  (:Pressed
    (CallFunction|DISABLEMOUSECONTROLLSFULLY)
    (if (not (Variables|Default|GetDisabled%20controller%20input?))
      (Utilities|IsValid _current_ui_reference
        (:Is%20Valid
          (Class|BPIUIInputs|UIUp(Message) _current_ui_reference))))))

(event Input|GamepadEvents|GamepadFaceButtonRight
  (params (Key :type Key%20Structure :default "None"))
  (bind _current_ui_reference (Variables|Default|GetCurrent%20UI%20Reference))
  ;[1 1 1] UnConfirm Button
  (:Pressed
    (CallFunction|DISABLEMOUSECONTROLLSFULLY)
    (if (not (Variables|Default|GetDisabled%20controller%20input?))
      (Utilities|IsValid _current_ui_reference
        (:Is%20Valid
          (Class|BPIUIInputs|UIBackOut(Message) _current_ui_reference))))))