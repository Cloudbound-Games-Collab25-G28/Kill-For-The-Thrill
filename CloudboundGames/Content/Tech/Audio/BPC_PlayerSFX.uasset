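; Player sound effects component that gives audio feedback for dodge rolls, life loss and death.
; Event handlers play roll, roll recovery and life lost sounds immediately as 2D audio.
; Death and all-lives-lost sounds instead go into a sound queue at a shared priority.
; Losing all lives also disables the SFX player after queuing its sound.
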(event Custom|On%20Roll%20Triggered
  (Audio|PlaySound2D (Variables|Default|GetDodgeSFX) 1.0 1.0 0.0 0 0))

(event Custom|On%20Roll%20Recovered
  (Audio|PlaySound2D (Variables|Default|GetDodgeRecoveredSFX) 1.0 1.0 0.0 0 0))

(event Custom|OnAllLivesLost
  (params (LivesComponent :type Lives%20Component%20Object%20Reference))
  (CallFunction|AddtoQueue (Variables|Default|GetAllLivesLostSFX) "NewEnumerator2")
  (CallFunction|DisableSFXPlayer))

(event Custom|OnLifeLost
  (params (LivesComponent :type Lives%20Component%20Object%20Reference))
  (Audio|PlaySound2D (Variables|Default|GetLifeLostSFX) 1.0 1.0 0.0 0 0))

(event EventOnKilled
  (params (HealthComponent :type Health%20Component%20Object%20Reference))
  (CallFunction|AddtoQueue (Variables|Default|GetDeathSFX) "NewEnumerator2"))