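; Character sound-effects component that plays audio for a character's appearance, attacks, footsteps, damage, blocks, healing and death.
; Each event handler plays its own sound variable through PlaySound2D, so playback is non-spatialized.
; Event payloads such as damage, heal amount and health component are unused, and the graph contains no event bindings.
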(event Custom|OnDamaged
  (params (Damage :type Float%20%28double-precision%29))
  (Audio|PlaySound2D (Variables|Default|GetDamagedSFX) 1.0 1.0 0.0 0 0))

(event Custom|OnHealed
  (params (Healed :type Float%20%28double-precision%29))
  (Audio|PlaySound2D (Variables|Default|GetHealedSFX) 1.0 1.0 0.0 0 0))

(event Custom|OnKilled
  (params (HealthComponent :type Health%20Component%20Object%20Reference))
  (Audio|PlaySound2D (Variables|Default|GetDeathSFX) 1.0 1.0 0.0 0 0))

(event Custom|OnAttack
  (Audio|PlaySound2D (Variables|Default|GetAttackSFX) 1.0 1.0 0.0 0 0))

(event Custom|OnDamageBlocked
  (Audio|PlaySound2D (Variables|Default|GetBlockedDamageSFX) 1.0 1.0 0.0 0 0))

(event Custom|OnFootsteps
  (Audio|PlaySound2D (Variables|Default|GetFootstepSFX) 1.0 1.0 0.0 0 0))

(event Custom|OnEnter
  (Audio|PlaySound2D (Variables|Default|GetAppearSFX) 1.0 1.0 0.0 0 0))