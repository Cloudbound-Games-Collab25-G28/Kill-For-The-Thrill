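; Announcer voice component that plays battle commentary for Honkules: one-time enemy-type intros, damage and winning remarks, and mid-battle quips.
; Event handlers append sounds to a queue, which an audio component added to the owner plays one at a time with a delay between lines.
; DoOnce gates with timer resets throttle damage and winning remarks.
; When the queue runs dry, a dead-zone timer queues a mid-battle quip if it is still empty.
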(event Custom|Handle_HonkulesWinning
  (params (EnemiesKilled :type Integer) (TotalEnemies :type Integer))
  (if (== (Math|Integer|%(Integer) (Variables|Winning|GetWin_EnemiesKilled_Threshold) EnemiesKilled) 0)
    (Utilities|FlowControl|DoOnce false
      (:Completed
        (CallFunction|AddtoQueue (Variables|Winning|GetHonkules%20Winning))
        (Utilities|Time|SetTimerbyEvent (delegate Custom|Reset_Winning_Cooldown) (Variables|Winning|GetWin_Comment_Delay))))))

(event Custom|On%20Clip%20Finished
  (Utilities|Array|RemoveIndex (Variables|Internal|GetVoiceClipCue))
  (Utilities|Time|SetTimerbyEvent (delegate Custom|Clip%20Delay%20Finished) (Variables|Internal|GetLine%20Delay)))

(event Custom|Clip%20Delay%20Finished
  (bind _voiceclipcue (Variables|Internal|GetVoiceClipCue))
  (if (Utilities|Array|IsEmpty _voiceclipcue)
    (Utilities|Time|SetTimerbyEvent (delegate Custom|Handle_MidQuipQuery) (Variables|Default|GetClipDeadzone))
    (else
      (CallFunction|PlayNextClip (Utilities|Array|Get(acopy) _voiceclipcue)))))

(event Custom|Handle_EnemySpawned
  (params (EnemyClass :type BP%20Enemy%20Base%20Class%20Reference))
  (switch string (Utilities|GetClassDisplayName EnemyClass)
    (:BP_Enemy_Melee_C
      (Utilities|FlowControl|DoOnce false
        (:Completed
          (CallFunction|AddtoQueue (Variables|Intros|GetIntro_Gladiator)))))
    (:BP_Miniboss_C
      (Utilities|FlowControl|DoOnce false
        (:Completed
          (CallFunction|AddtoQueue (Variables|Intros|GetIntro_Minotaur)))))
    (:BP_PlagueDoctor_C
      (Utilities|FlowControl|DoOnce false
        (:Completed
          (CallFunction|AddtoQueue (Variables|Intros|GetIntro_Plague)))))
    (:BP_Siren_C
      (Utilities|FlowControl|DoOnce false
        (:Completed
          (CallFunction|AddtoQueue (Variables|Intros|GetIntro_Siren)))))))

(event Custom|Handle_HonkulesDamaged
  (params (damage :type Float%20%28double-precision%29))
  (Utilities|FlowControl|DoOnce false
    (:Completed
      (CallFunction|AddtoQueue (Variables|Damage|GetHonkules_Damaged))
      (Utilities|Time|SetTimerbyEvent (delegate Custom|Reset_Damage_Cooldown) (Variables|Damage|GetHurt_Comment_Delay)))))

(event Custom|Reset_Damage_Cooldown
  (Utilities|FlowControl|DoOnce false) ; enters at Reset
)

(event Custom|Reset_Winning_Cooldown
  (Utilities|FlowControl|DoOnce false) ; enters at Reset
)

(event Custom|Handle_MidQuipQuery
  (if (Utilities|Array|IsEmpty (Variables|Internal|GetVoiceClipCue))
    (CallFunction|AddtoQueue (Variables|Default|GetMidBattle_Quip))
    (else
      (Utilities|Time|SetTimerbyEvent (delegate Custom|Handle_MidQuipQuery) (Variables|Default|GetClipDeadzone)))))

(event EventEndPlay
  (params (EndPlayReason :type EEndPlayReason%20Enum :default "Destroyed"))
  (Components|DestroyComponent (stale EventBeginPlay _returnvalue)))

(event EventBeginPlay
  (bind _returnvalue (Game|AddComponentbyClass (Components|GetOwner) "/Script/Engine.AudioComponent" false))
  (bind _output_get (Variables|Default|SetAnnouncerSoundComponent _returnvalue))
  (EventDispatchers|BindEventtoOnAudioFinished _output_get (delegate Custom|On%20Clip%20Finished)))

(fn AddtoQueue
  (params (New%20Sound :type Sound%20Base%20Object%20Reference))
  (bind _voiceclipcue (Variables|Internal|GetVoiceClipCue))
  (if (Utilities|Array|IsEmpty _voiceclipcue)
    (Utilities|Array|Add _voiceclipcue New%20Sound)
    (CallFunction|ClipDelayFinished)
    (else
      (Utilities|Array|Add _voiceclipcue New%20Sound))))

(fn PlayNextClip
  (params (Next%20Clip :type Sound%20Base%20Object%20Reference))
  (bind _announcersoundcomponent (Variables|Default|GetAnnouncerSoundComponent))
  (Audio|Components|Audio|Stop _announcersoundcomponent)
  (Audio|Components|Audio|SetSound _announcersoundcomponent Next%20Clip)
  (Audio|Components|Audio|Play _announcersoundcomponent 0.0))