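; Music player component that switches a wave-based game's soundtrack between default, interlude, boss, win and lose tracks.
; It spawns a persistent 2D sound on BeginPlay and destroys it on EndPlay.
; Game-phase events call SetNewMusic, which stops the current sound, swaps the track and plays from the start.
; A DoOnce reset by each interlude lets the next wave start restore the default music only once.
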(event Custom|OnLastWave
  (CallFunction|SetNewMusic (Variables|Default|GetBossMusic)))

(event Custom|OnInterludeStart
  (CallFunction|SetNewMusic (Variables|Default|GetInterludeMusic))
  (Utilities|FlowControl|DoOnce true) ; enters at Reset
)

(event Custom|OnWaveStart
  (params (WaveNumber :type Integer) (EnemiesKilled :type Integer) (TotalEnemies :type Integer) (MaterialsCollected :type Integer))
  (Utilities|FlowControl|DoOnce true
    (:Completed
      (CallFunction|SetNewMusic (Variables|Default|GetDefaultMusic)))))

(event Custom|OnWon
  (CallFunction|SetNewMusic (Variables|Default|GetWinMusic)))

(event Custom|OnLost
  (CallFunction|SetNewMusic (Variables|Default|GetLoseMusic)))

(event EventEndPlay
  (params (EndPlayReason :type EEndPlayReason%20Enum :default "Destroyed"))
  (Components|DestroyComponent (stale EventBeginPlay _returnvalue)))

(event EventBeginPlay
  (bind _returnvalue (Audio|SpawnSound2D (Variables|Default|GetDefaultMusic) 1.0 1.0 0.0 0 false false))
  (Variables|Default|SetSoundComponent _returnvalue))

(fn SetNewMusic
  (params (New%20Music :type Sound%20Base%20Object%20Reference))
  (bind _soundcomponent (Variables|Default|GetSoundComponent))
  (bind _output_get (Variables|Default|SetCurrentMusic New%20Music))
  (if (Audio|Components|Audio|IsPlaying _soundcomponent)
    (Audio|Components|Audio|Stop _soundcomponent))
  (Audio|Components|Audio|SetSound _soundcomponent _output_get)
  (Audio|Components|Audio|Play _soundcomponent 0.0))