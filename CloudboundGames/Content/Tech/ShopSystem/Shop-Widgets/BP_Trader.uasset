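; BP_Trader is the trader that opens the shop UI for the player.
; OpenShop creates a WB_Shop widget, initializes it with a reference to the trader, stores it and adds it to the viewport.
; An IsShopOpen flag guards against opening it twice; opening also shows the mouse cursor and clears CanFBePressed on the wave game mode.
; The file contains no closing logic.
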(event Custom|OpenShop
  ;[1 0.5961 0.03484] Trader Logic for opening the shop
  (if (not (Variables|Default|GetIsShopOpen))
    (bind _returnvalue (UserInterface|CreateWidget "/Game/Tech/ShopSystem/Shop-Widgets/WB_Shop.WB_Shop_C"))
    (bind _output_get (Variables|Default|SetShop%20ref _returnvalue))
    (Default|InitShopWidget _returnvalue self)
    (UserInterface|Viewport|AddtoViewport _output_get 0)
    (Variables|/Script/Engine.PlayerController|SetbShowMouseCursor (Game|GetPlayerController 0) true)
    (Variables|Default|SetIsShopOpen true)
    (Variables|/Game/Tech/WaveSystems/WaveSystem/BP_WaveGameMode.BP_WaveGameMode_C|SetCan%20F%20be%20Pressed? (CallFunction|GetWaveGameMode) false)))

(fn ConstructionScript)