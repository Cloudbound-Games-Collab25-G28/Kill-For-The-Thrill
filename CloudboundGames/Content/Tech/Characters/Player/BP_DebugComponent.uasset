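; Player debug component that toggles the pause menu and spawns UI screens from debug keys for testing.
; A debug key and the IA_PauseGame input share one toggle that creates or removes WBP_PauseMenu, switching input mode, cursor visibility and game pause state.
; Other debug keys each create and add a new credits, win, death or HUD widget to the viewport.
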(event Input|EnhancedActionEvents|EnhancedInputActionIA_PauseGame
  (params (ActionValue :type Boolean) (ElapsedSeconds :type Float%20%28double-precision%29) (TriggeredSeconds :type Float%20%28double-precision%29) (InputAction :type Input%20Action%20Object%20Reference :default "/Game/Tech/Input/Actions/IA_PauseGame.IA_PauseGame"))
  ;[0 0 0] Toggle pause menu
  (if (not (Variables|Default|GetbIsPauseMenuOpen))
    (CallFunction|OpensPauseMenu)
    (else
      (CallFunction|ClosesPauseMenu))))

(event Input|KeyboardEvents|DebugKeyT
  (params (Key :type Key%20Structure) (ActionValue :type Input%20Action%20Value%20Structure))
  ;[0 0 0] Toggle pause menu
  (:Pressed
    (if (not (Variables|Default|GetbIsPauseMenuOpen))
      (CallFunction|OpensPauseMenu)
      (else
        (CallFunction|ClosesPauseMenu)))))

(event Input|KeyboardEvents|DebugKeyK
  (params (Key :type Key%20Structure) (ActionValue :type Input%20Action%20Value%20Structure))
  ;[0 0 1] Debug to start credits
  (:Pressed
    (bind _returnvalue (UserInterface|CreateWidget "/Game/Tech/UI/WBP_Credits.WBP_Credits_C"))
    (UserInterface|Viewport|AddtoViewport _returnvalue 0)))

(event Input|KeyboardEvents|DebugKeyL
  (params (Key :type Key%20Structure) (ActionValue :type Input%20Action%20Value%20Structure))
  ;[0 -0 1] Debug to open death screen
  (:Pressed
    (bind _returnvalue (UserInterface|CreateWidget "/Game/Tech/UI/WBP_DeathScreen.WBP_DeathScreen_C"))
    (UserInterface|Viewport|AddtoViewport _returnvalue 0)))

(event Input|KeyboardEvents|DebugKeyJ
  (params (Key :type Key%20Structure) (ActionValue :type Input%20Action%20Value%20Structure))
  ;[0 -0 1] Debug to open win screen
  (:Pressed
    (bind _returnvalue (UserInterface|CreateWidget "/Game/Tech/UI/WBP_WinScreen.WBP_WinScreen_C"))
    (UserInterface|Viewport|AddtoViewport _returnvalue 0)))

(event Input|KeyboardEvents|DebugKeyI
  (params (Key :type Key%20Structure) (ActionValue :type Input%20Action%20Value%20Structure))
  ;[0 -0 1] Debug to Player HUD
  (:Pressed
    (bind _returnvalue (UserInterface|CreateWidget "/Game/Tech/UI/PlayerUI/WBP_HUD.WBP_HUD_C"))
    (UserInterface|Viewport|AddtoViewport _returnvalue 0)))

(fn ClosesPauseMenu
  (bind _returnvalue (Game|GetPlayerController 0))
  ;[0 0 0] Closes pause menu and hides cursor
  (Variables|Default|SetbIsPauseMenuOpen false)
  (Widget|RemovefromParent (Variables|Default|GetPauseMenuREF))
  (Input|SetInputModeGameOnly _returnvalue false)
  (Variables|/Script/Engine.PlayerController|SetbShowMouseCursor _returnvalue false)
  (Game|SetGamePaused false))

(fn OpensPauseMenu
  (bind _returnvalue (Game|GetPlayerController 0))
  ;[0 0 0] Open pause menu and activate mouse cursor
  (Variables|Default|SetbIsPauseMenuOpen true)
  (bind _returnvalue_2 (UserInterface|CreateWidget "/Game/Tech/UI/Menus/WBP_PauseMenu.WBP_PauseMenu_C"))
  (bind _output_get (Variables|Default|SetPauseMenuREF _returnvalue_2))
  (UserInterface|Viewport|AddtoViewport _output_get 0)
  (Input|SetInputModeGameandUI _returnvalue _output_get "DoNotLock" true false)
  (Variables|/Script/Engine.PlayerController|SetbShowMouseCursor _returnvalue true)
  (Game|SetGamePaused true))