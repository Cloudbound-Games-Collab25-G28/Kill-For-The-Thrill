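; Actor component that holds a character's stackable upgrade objects and turns them into combat stats, from damage, crits and agility to poison and rage.
; Getters poll every upgrade and fold the results into Add/AddProportion/Multiply modifiers or summed totals.
; Weapon hits roll crits, spawn delayed AOE damage, add poison upgrades to targets and bind kills to rage stacks.
; It also enforces stack caps and offers random prerequisite-gated upgrades.
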(event Custom|OnUpgradesChanged_Event
  (CallFunction|RecalculateMovementSpeed))

(event Custom|RecalculateMovementSpeed
  (params (Context :type F%20Movement%20Speed%20Context%20Structure))
  (bind _movementspeed (GetUpgradeEffect|GetMovementSpeed Context))
  (Default|CallOnMovementSpeedRecalculated _movementspeed))

(event Custom|BindToEnemyDeath
  (params (Enemy :type Actor%20Object%20Reference))
  (bind _returnvalue (Actor|GetComponentbyClass Enemy "/Game/Tech/UpgradeSystem/BPC_UpgradeableHealth.BPC_UpgradeableHealth_C"))
  (Utilities|IsValid _returnvalue
    (:Is%20Valid
      (EventDispatchers|BindEventtoOnKilled _returnvalue (delegate Custom|OnKill)))))

(event Custom|OnKill
  (params (HealthComponent :type Health%20Component%20Object%20Reference))
  (bind _returnvalue (Components|GetOwner))
  (bind _self self)
  (bind _stacks (GetUpgradeEffect|GetRageStacksReceivedonKill))
  (for _index (range 1 _stacks)
    (CallFunction|AddUpgradeOfClass "/Game/Tech/UpgradeSystem/BP_Rage.BP_Rage_C" (Utilities|Struct|MakeF_UpgradeChangeContext _returnvalue _self _returnvalue _self))))

(event EventBeginPlay
  (bind _returnvalue (Components|GetOwner))
  (bind _self self)
  (for _array_element (Variables|Default|GetInitialUpgrades)
    (CallFunction|AddUpgradeOfClass _array_element (Utilities|Struct|MakeF_UpgradeChangeContext _returnvalue _self _returnvalue _self))))

(fn CombineModifiers
  (params (A :type F%20Value%20Modifier%20Structure) (B :type F%20Value%20Modifier%20Structure))
  (return (Utilities|Struct|MakeF_ValueModifier (+ (.add A) (.add B)) (+ (.addproportion A) (.addproportion B)) (* (.multiply A) (.multiply B)))))

(fn ApplyModifier
  (params (Value :type Float%20%28double-precision%29) (Modifier :type F%20Value%20Modifier%20Structure))
  (return (* (+ Value (.add Modifier)) (+ (.addproportion Modifier) 1.0) (.multiply Modifier))))

(fn ModifyDamageApplied
  (params (BaseDamage :type Float%20%28double-precision%29) (Context :type F%20Damage%20Context%20Structure))
  (bind _target (Utilities|Struct|BreakF_DamageContext Context))
  (bind _returnvalue (Actor|GetComponentbyClass _target "BPC_Upgrades_C"))
  (bind _returnvalue_2 (Utilities|IsValid _returnvalue))
  (if _returnvalue_2
    (bind _agility (GetUpgradeEffect|GetAgility _returnvalue Context)))
  (bind _probability (GetUpgradeEffect|GetCritProbability Context))
  (bind _damagemodifier (GetUpgradeEffect|GetCritDamageModifier Context))
  (bind _damagemodifier_2 (GetUpgradeEffect|GetDamageModifier Context))
  (return (Modifiers|ApplyModifier BaseDamage (Modifiers|CombineModifiers _damagemodifier_2 (select (Math|Random|RandomBoolwithWeight (+ _probability (Math|Float|MapRangeClamped (select _returnvalue_2 _agility 0.0) 0.0 -1.0 0.0 1.0))) _damagemodifier "")))))

(fn AddUpgradeOfClass
  (params (UpgradeClass :type BP%20Upgrade%20Class%20Reference) (Context :type F%20Upgrade%20Change%20Context%20Structure))
  (bind _upgrades (Variables|Default|GetUpgrades))
  (bind _upgrades_2 (Variables|Default|GetUpgrades))
  (bind _output (CallFunction|GetArrayClasses _upgrades_2))
  (bind _returnvalue (Utilities|Array|FindItem _output UpgradeClass))
  (bind _output_2 (Utilities|Array|Get(acopy) _upgrades _returnvalue))
  (if (== _returnvalue -1)
    (bind _returnvalue_2 (Game|ConstructObjectfromClass UpgradeClass))
    (Utilities|Array|Add (Variables|Default|GetUpgrades) _returnvalue_2)
    (Default|Init _returnvalue_2 Context)
    (Default|CallOnUpgradesChanged)
    (return true _returnvalue_2)
    (else
      (bind _stackmap (GetUpgradeEffect|GetUpgradesMaxApplyableStacks Context))
      (if (< (StackMap|StackMapGetorDefault _stackmap UpgradeClass 1) (+ (Variables|/Game/Tech/UpgradeSystem/BP_Upgrade.BP_Upgrade_C|GetStacks _output_2) 1))
        (return false 0)
        (else
          (Variables|/Game/Tech/UpgradeSystem/BP_Upgrade.BP_Upgrade_C|SetStacks _output_2 (+ (Variables|/Game/Tech/UpgradeSystem/BP_Upgrade.BP_Upgrade_C|GetStacks _output_2) 1))
          (Default|StacksChanged _output_2 Context)
          (Default|CallOnUpgradesChanged))))))

(fn GetDamageModifier
  (params (Context :type F%20Damage%20Context%20Structure))
  (for _array_element (Variables|Default|GetUpgrades)
    (bind _damagemodifier (Default|GetDamageModifier _array_element Context))
    (LocalVariables|SetTotalDamageModifier (Modifiers|CombineModifiers _damagemodifier (LocalVariables|GetTotalDamageModifier))))
  (return (LocalVariables|GetTotalDamageModifier)))

(fn GetCritDamageModifier
  (params (Context :type F%20Damage%20Context%20Structure))
  (for _array_element (Variables|Default|GetUpgrades)
    (bind _damagemodifier (Default|GetCritDamageModifier _array_element Context))
    (LocalVariables|SetTotalDamageModifier (Modifiers|CombineModifiers _damagemodifier (LocalVariables|GetTotalDamageModifier))))
  (return (LocalVariables|GetTotalDamageModifier)))

(fn GetCritProbability
  (params (Context :type F%20Damage%20Context%20Structure))
  (for _array_element (Variables|Default|GetUpgrades)
    (bind _probability (Default|GetCritProbability _array_element Context))
    (LocalVariables|SetTotalProbability (+ _probability (LocalVariables|GetTotalProbability))))
  (return (Math|Float|Clamp(Float) (LocalVariables|GetTotalProbability))))

(fn RemoveAllUpgradeStacks
  (params (Upgrade :type BP%20Upgrade%20Object%20Reference) (Context :type F%20Upgrade%20Change%20Context%20Structure))
  (Utilities|Array|RemoveItem (Variables|Default|GetUpgrades) Upgrade)
  (Default|CallOnUpgradesChanged))

(fn GetMaxHealth
  (params (Context :type F%20Max%20Health%20Context%20Structure) (ActualHealth :type Float%20%28double-precision%29))
  (for _array_element (Variables|Default|GetUpgrades)
    (bind _maxhealth (Default|GetMaxHealthModifier _array_element Context))
    (LocalVariables|SetTotalMaxHealth (Modifiers|CombineModifiers _maxhealth (LocalVariables|GetTotalMaxHealth))))
  (return (Modifiers|ApplyModifier ActualHealth (LocalVariables|GetTotalMaxHealth))))

(fn GetMovementSpeed
  (params (Context :type F%20Movement%20Speed%20Context%20Structure))
  (bind _modifier (GetUpgradeEffect|GetMovementSpeedModifer Context))
  (return (Modifiers|ApplyModifier 0.0 _modifier)))

(fn GetAttackSpeed
  (params (Context :type F%20Attack%20Speed%20Context%20Structure))
  (for _array_element (Variables|Default|GetUpgrades)
    (bind _modifier (Default|GetAttackSpeedModifier _array_element Context))
    (LocalVariables|SetTotalAttackSpeedModifier (Modifiers|CombineModifiers _modifier (LocalVariables|GetTotalAttackSpeedModifier))))
  (return (Modifiers|ApplyModifier 1.0 (LocalVariables|GetTotalAttackSpeedModifier))))

(fn ModifyDamageReceived
  (params (IncomingDamage :type Float%20%28double-precision%29) (Context :type F%20Damage%20Context%20Structure))
  (bind _agility (GetUpgradeEffect|GetAgility Context))
  (return (select (Math|Random|RandomBoolwithWeight _agility) 0.0 IncomingDamage)))

(fn GetAgility
  (params (Context :type F%20Damage%20Context%20Structure))
  (for _array_element (Variables|Default|GetUpgrades)
    (bind _modifier (Default|GetAgilityModifier _array_element Context))
    (LocalVariables|SetTotalAgilityModifier (Modifiers|CombineModifiers _modifier (LocalVariables|GetTotalAgilityModifier))))
  (return (Modifiers|ApplyModifier 0.0 (LocalVariables|GetTotalAgilityModifier))))

(fn GetMovementSpeedModifer
  (params (Context :type F%20Movement%20Speed%20Context%20Structure))
  (for _array_element (Variables|Default|GetUpgrades)
    (bind _modifier (Default|GetMovementSpeedModifier _array_element Context))
    (LocalVariables|SetTotalMovementSpeedModifier (Modifiers|CombineModifiers _modifier (LocalVariables|GetTotalMovementSpeedModifier))))
  (return (LocalVariables|GetTotalMovementSpeedModifier)))

(fn GetAOEDamageProportionModifier
  (params (Context :type F%20Damage%20Context%20Structure))
  (for _array_element (Variables|Default|GetUpgrades)
    (bind _modiifer (Default|GetAOEDamageProportionModifier _array_element Context))
    (LocalVariables|SetTotalAOEDamageProportionModifier (Modifiers|CombineModifiers _modiifer (LocalVariables|GetTotalAOEDamageProportionModifier))))
  (return (LocalVariables|GetTotalAOEDamageProportionModifier)))

(fn GetAOEAreaModifier
  (params (Context :type F%20Damage%20Context%20Structure))
  (for _array_element (Variables|Default|GetUpgrades)
    (bind _modifier (Default|GetAOEAreaModifer _array_element Context))
    (LocalVariables|SetTotalAOEAreaModifier (Modifiers|CombineModifiers _modifier (LocalVariables|GetTotalAOEAreaModifier))))
  (return (LocalVariables|GetTotalAOEAreaModifier)))

(fn GetAOEDamageModifier
  (params (Context :type F%20Damage%20Context%20Structure))
  (for _array_element (Variables|Default|GetUpgrades)
    (bind _modiifer (Default|GetAOEDamageProportionModifier _array_element Context))
    (LocalVariables|SetTotalAOEDamageModifier (Modifiers|CombineModifiers _modiifer (LocalVariables|GetTotalAOEDamageModifier))))
  (return (LocalVariables|GetTotalAOEDamageModifier)))

(fn GetAOEDamageProportion
  (params (Context :type F%20Damage%20Context%20Structure))
  (bind _modifier (GetUpgradeEffect|GetAOEDamageProportionModifier Context))
  (return (Modifiers|ApplyModifier 0.0 _modifier)))

(fn ApplyWeaponDamage
  (params (BaseDamage :type Float%20%28double-precision%29) (Context :type F%20Damage%20Context%20Structure))
  (bind _returnvalue (Actor|GetComponentbyClass (.target Context) "BPC_Upgrades_C"))
  (CallFunction|BindtoEnemyDeath (.Target (Utilities|Struct|BreakF_DamageContext Context)))
  (bind _damageapplied (CallFunction|ModifyDamageApplied BaseDamage Context))
  (bind _proportion (GetUpgradeEffect|GetAOEDamageProportion Context))
  (Utilities|FlowControl|Sequence
    (:then_0
      (Game|Damage|ApplyDamage (.Target (Utilities|Struct|BreakF_DamageContext Context)) (* (- 1.0 _proportion) _damageapplied) 0 0))
    (:then_1
      (bind _modifier (GetUpgradeEffect|GetAOEAreaModifier Context))
      (bind _modifier_2 (GetUpgradeEffect|GetAOEDelayModifier Context))
      (Game|SpawnActorfromClass "/Game/Tech/UpgradeSystem/BP_AOEDamage.BP_AOEDamage_C" (Math|Transform|MakeTransform (.Position (Utilities|Struct|BreakF_DamageContext Context)) "0, 0, 0" "1.000000,1.000000,1.000000") "Undefined" "MultiplyWithRoot" 0 (Modifiers|ApplyModifier 0.0 _modifier_2) _damageapplied (Modifiers|ApplyModifier (Math|Float|MapRangeClamped _damageapplied 0.0 1e+02 5e+01 3e+02) _modifier) 0)))
  (Utilities|IsValid (.target Context)
    (:Is%20Valid
      (Utilities|IsValid _returnvalue
        (:Is%20Valid
          (bind _stacks (GetUpgradeEffect|GetPoisonStacksAppliedonHit Context))
          (for _index (range 1 _stacks)
            (CallFunction|AddUpgradeOfClass _returnvalue "/Game/Tech/UpgradeSystem/BP_Poison.BP_Poison_C" (Utilities|Struct|MakeF_UpgradeChangeContext (Components|GetOwner) self (.target Context) _returnvalue))))))))

(fn GetAOEDelayModifier
  (params (Context :type F%20Damage%20Context%20Structure))
  (for _array_element (Variables|Default|GetUpgrades)
    (bind _modiifer (Default|GetAOEDelayModifier _array_element Context))
    (LocalVariables|SetTotalAOEDelayModifier (Modifiers|CombineModifiers _modiifer (LocalVariables|GetTotalAOEDelayModifier))))
  (return (LocalVariables|GetTotalAOEDelayModifier)))

(fn CombineStackMap
  (params (A :type Map%20of%20BP%20Upgrade%20Class%20References%20to%20Integers) (B :type Map%20of%20BP%20Upgrade%20Class%20References%20to%20Integers))
  (bind _output_get (LocalVariables|SetStackMapTotal A))
  (bind _stackmap (StackMap|AddtoStackMap _output_get B))
  (return (StackMap|CleanStackMap _stackmap)))

(fn StackMapGetorDefault
  (params (StackMap :type Map%20of%20BP%20Upgrade%20Class%20References%20to%20Integers) (UpgradeClass :type BP%20Upgrade%20Class%20Reference) (Default :type Integer))
  (bind (_value _returnvalue) (Utilities|Map|Find StackMap UpgradeClass))
  (return (select _returnvalue _value Default)))

(fn CleanStackMap
  (params (Unclean :type Map%20of%20BP%20Upgrade%20Class%20References%20to%20Integers))
  (bind _output_get (LocalVariables|SetStackMapTotal Unclean))
  (bind _keys (Utilities|Map|Keys _output_get))
  (for _array_element _keys
    (if (<= (StackMap|StackMapGetorDefault (LocalVariables|GetStackMapTotal) _array_element) 0)
      (Utilities|Map|Remove (LocalVariables|GetStackMapTotal) _array_element)))
  (return (LocalVariables|GetStackMapTotal)))

(fn GetUpgradeStackMap
  (for _array_element (Variables|Default|GetUpgrades)
    (Utilities|Map|Add (LocalVariables|GetStackMapTotal) (Utilities|GetClass _array_element) (Variables|/Game/Tech/UpgradeSystem/BP_Upgrade.BP_Upgrade_C|GetStacks _array_element)))
  (return (LocalVariables|GetStackMapTotal)))

(fn StackMapSetorDefault
  (params (StackMap :type Map%20of%20BP%20Upgrade%20Class%20References%20to%20Integers) (Key :type BP%20Upgrade%20Class%20Reference) (Value :type Integer) (Default :type Integer))
  (if (== Value Default)
    (Utilities|Map|Remove StackMap Key)
    (else
      (Utilities|Map|Add StackMap Key Value))))

(fn GetUpgradesMaxApplyableStacks
  (params (Context :type F%20Upgrade%20Change%20Context%20Structure))
  (for _array_element (Variables|Default|GetUpgrades)
    (bind _stackmap (Default|GetUpgradesMaxApplyableStacks _array_element Context))
    (StackMap|AddtoStackMap (LocalVariables|GetTotalStackMap) _stackmap))
  (return (LocalVariables|GetTotalStackMap)))

(fn AddtoStackMap
  (params (A :type Map%20of%20BP%20Upgrade%20Class%20References%20to%20Integers) (B :type Map%20of%20BP%20Upgrade%20Class%20References%20to%20Integers))
  (bind _keys (Utilities|Map|Keys B))
  (for _array_element _keys
    (Utilities|Map|Add A _array_element (+ (StackMap|StackMapGetorDefault A _array_element) (StackMap|StackMapGetorDefault B _array_element))))
  (StackMap|CleanStackMapinPlace A)
  (return A))

(fn CleanStackMapinPlace
  (params (Unclean :type Map%20of%20BP%20Upgrade%20Class%20References%20to%20Integers))
  (bind _keys (Utilities|Map|Keys Unclean))
  (for _array_element _keys
    (if (<= (StackMap|StackMapGetorDefault Unclean _array_element) 0)
      (Utilities|Map|Remove Unclean _array_element)))
  (return Unclean))

(fn GetArrayClasses
  (params (Input :type Array%20of%20Object%20Object%20References))
  (for _array_element Input
    (Utilities|Array|Add (LocalVariables|GetClasses) (Utilities|GetClass _array_element)))
  (return (LocalVariables|GetClasses)))

(fn ModifyAOEDamage
  (params (BaseDamage :type Float%20%28double-precision%29) (Context :type F%20Damage%20Context%20Structure))
  (bind _proportion (GetUpgradeEffect|GetAOEDamageProportion Context))
  (bind _modifier (GetUpgradeEffect|GetAOEDamageModifier Context))
  (return (Modifiers|ApplyModifier (* _proportion BaseDamage) _modifier)))

(fn RemoveUpgrade
  (params (Upgrade :type BP%20Upgrade%20Object%20Reference) (Context :type F%20Upgrade%20Change%20Context%20Structure))
  (if (== (Variables|/Game/Tech/UpgradeSystem/BP_Upgrade.BP_Upgrade_C|GetStacks Upgrade) 1)
    (Utilities|Array|RemoveItem (Variables|Default|GetUpgrades) Upgrade)
    (Default|CallOnUpgradesChanged)
    (else
      (Variables|/Game/Tech/UpgradeSystem/BP_Upgrade.BP_Upgrade_C|SetStacks Upgrade (- (Variables|/Game/Tech/UpgradeSystem/BP_Upgrade.BP_Upgrade_C|GetStacks Upgrade) 1))
      (Default|StacksChanged Upgrade Context))))

(fn GetPoisonDurationModifier
  (params (Context :type F%20Status%20Effect%20Context%20Structure))
  (for _array_element (Variables|Default|GetUpgrades)
    (bind _modifier (Default|GetPoisonDurationModifier _array_element Context))
    (LocalVariables|SetTotalPoisonDurationModifier (Modifiers|CombineModifiers _modifier (LocalVariables|GetTotalPoisonDurationModifier))))
  (return (LocalVariables|GetTotalPoisonDurationModifier)))

(fn GetPoisonAgilityModifier
  (params (Context :type F%20Status%20Effect%20Context%20Structure))
  (for _array_element (Variables|Default|GetUpgrades)
    (bind _modifier (Default|GetPoisonAgilityModifier _array_element Context))
    (LocalVariables|SetTotalPoisonMovementSpeedModifier (Modifiers|CombineModifiers _modifier (LocalVariables|GetTotalPoisonMovementSpeedModifier))))
  (return (LocalVariables|GetTotalPoisonMovementSpeedModifier)))

(fn GetPoisonMovementSpeedModifier
  (params (Context :type F%20Status%20Effect%20Context%20Structure))
  (for _array_element (Variables|Default|GetUpgrades)
    (bind _modifier (Default|GetPoisonMovementSpeedModifier _array_element Context))
    (LocalVariables|SetTotalPoisonMovementSpeedModifier (Modifiers|CombineModifiers _modifier (LocalVariables|GetTotalPoisonMovementSpeedModifier))))
  (return (LocalVariables|GetTotalPoisonMovementSpeedModifier)))

(fn GetPoisonDamageModifier
  (params (Context :type F%20Status%20Effect%20Context%20Structure))
  (for _array_element (Variables|Default|GetUpgrades)
    (bind _modifier (Default|GetPoisonDamageModifier _array_element Context))
    (LocalVariables|SetTotalPoisonDamageModifier (Modifiers|CombineModifiers _modifier (LocalVariables|GetTotalPoisonDamageModifier))))
  (return (LocalVariables|GetTotalPoisonDamageModifier)))

(fn GetPoisonDamageCooldownTimeModifier
  (params (Context :type F%20Status%20Effect%20Context%20Structure))
  (for _array_element (Variables|Default|GetUpgrades)
    (bind _modifier (Default|GetPoisonDamageModifier _array_element Context))
    (LocalVariables|SetTotalPoisonDamageCooldownTimeModifier (Modifiers|CombineModifiers _modifier (LocalVariables|GetTotalPoisonDamageCooldownTimeModifier))))
  (return (LocalVariables|GetTotalPoisonDamageCooldownTimeModifier)))

(fn GetPoisonStacksAppliedonHit
  (params (Context :type F%20Damage%20Context%20Structure))
  (for _array_element (Variables|Default|GetUpgrades)
    (bind _modifier (Default|GetPoisonStacksAppliedonHit _array_element Context))
    (LocalVariables|SetTotalPoisonStacks (+ _modifier (LocalVariables|GetTotalPoisonStacks))))
  (return (LocalVariables|GetTotalPoisonStacks)))

(fn GetPoisonDuration
  (params (Context :type F%20Status%20Effect%20Context%20Structure))
  (bind _modifier (GetUpgradeEffect|GetPoisonDurationModifier Context))
  (return (Modifiers|ApplyModifier 0.0 _modifier)))

(fn GetPoisonDamage
  (params (Context :type F%20Status%20Effect%20Context%20Structure))
  (bind _modifier (GetUpgradeEffect|GetPoisonDamageModifier Context))
  (return (Modifiers|ApplyModifier 0.0 _modifier)))

(fn GetPoisonDamageCooldownTime
  (params (Context :type F%20Status%20Effect%20Context%20Structure))
  (bind _modifier (GetUpgradeEffect|GetPoisonDamageCooldownTimeModifier Context))
  (return (Modifiers|ApplyModifier 0.0 _modifier)))

(fn GetAvailableUpgrades
  (bind _currentupgrades (LocalVariables|GetCurrentUpgrades))
  (bind _stackmap (StackMap|GetUpgradeStackMap))
  (bind _keys (Utilities|Map|Keys _stackmap))
  (Utilities|Set|AddItems (LocalVariables|GetCurrentUpgrades) _keys)
  (for _array_element (Variables|Default|GetAllAvailableUpgrades)
    (bind _result (Utilities|Set|Difference (.Requires (Utilities|GetClassDefaults _array_element)) _currentupgrades))
    (if (and (== (Utilities|Set|Length _result) 0) (not (Utilities|Set|Contains _currentupgrades _array_element)))
      (Utilities|Array|Add (LocalVariables|GetTotalAvailableUpgrades) _array_element)))
  (return (LocalVariables|GetTotalAvailableUpgrades)))

(fn GetRandomAvailableUpgrades
  (params (Number :type Integer))
  (bind _availableupgrades (CallFunction|GetAvailableUpgrades))
  (LocalVariables|SetAvailable _availableupgrades)
  (for _index (range 1 Number)
    (bind _returnvalue (Utilities|Array|Add (LocalVariables|GetPicked) (.OutItem (Utilities|Array|Random (LocalVariables|GetAvailable)))))
    (Utilities|Array|RemoveItem (LocalVariables|GetAvailable) (Utilities|Array|Get(acopy) (LocalVariables|GetPicked) _returnvalue)))
  (return (LocalVariables|GetPicked)))

(fn GetRageStacksReceivedonKill
  (params (Context :type F%20Status%20Effect%20Context%20Structure))
  (for _array_element (Variables|Default|GetUpgrades)
    (bind _modifier (Default|GetRageStacksReceivedonKill _array_element Context))
    (LocalVariables|SetTotalRageStacks (+ _modifier (LocalVariables|GetTotalRageStacks))))
  (return (LocalVariables|GetTotalRageStacks)))

(fn GetRageDurationModifier
  (params (Context :type F%20Status%20Effect%20Context%20Structure))
  (for _array_element (Variables|Default|GetUpgrades)
    (bind _modifier (Default|GetRageDurationModifier _array_element Context))
    (LocalVariables|SetTotalRageDurationModifier (Modifiers|CombineModifiers _modifier (LocalVariables|GetTotalRageDurationModifier))))
  (return (LocalVariables|GetTotalRageDurationModifier)))

(fn GetRageDuration
  (params (Context :type F%20Status%20Effect%20Context%20Structure))
  (bind _modifier (GetUpgradeEffect|GetRageDurationModifier Context))
  (return (Modifiers|ApplyModifier 0.0 _modifier)))

(fn GetRageDamageModifier
  (params (Context :type F%20Status%20Effect%20Context%20Structure))
  (for _array_element (Variables|Default|GetUpgrades)
    (bind _modifier (Default|GetRageDamageModifier _array_element Context))
    (LocalVariables|SetTotalRageDamageModifier (Modifiers|CombineModifiers _modifier (LocalVariables|GetTotalRageDamageModifier))))
  (return (LocalVariables|GetTotalRageDamageModifier)))

(fn GetRageMovementSpeedModifier
  (params (Context :type F%20Movement%20Speed%20Context%20Structure))
  (for _array_element (Variables|Default|GetUpgrades)
    (bind _modifier (Default|GetRageMovementSpeedModifier _array_element Context))
    (LocalVariables|SetTotalRageMovementSpeedModifier (Modifiers|CombineModifiers _modifier (LocalVariables|GetTotalRageMovementSpeedModifier))))
  (return (LocalVariables|GetTotalRageMovementSpeedModifier)))