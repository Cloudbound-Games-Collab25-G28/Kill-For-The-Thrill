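; BP_AOEDamage is an actor that deals one delayed burst of area damage to characters around its location on behalf of an attacker.
; A timer set on BeginPlay runs a stationary sphere trace for pawns, provided the attacker has a BPC_Upgrades component.
; For each character hit, that component modifies the final weapon damage using attacker, target, position and direction context before it is applied.
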(event Custom|ApplyDamage
  (bind _returnvalue (Transformation|GetActorLocation))
  (bind _returnvalue_2 (Transformation|GetActorLocation))
  (bind _output_get (Variables|Default|SetUpgradeComponent (Actor|GetComponentbyClass (Variables|Default|GetAttacker) "/Game/Tech/UpgradeSystem/BPC_Upgrades.BPC_Upgrades_C")))
  (Utilities|IsValid _output_get
    (:Is%20Valid
      (bind _outhits (Collision|MultiSphereTraceForObjects _returnvalue _returnvalue 0.0 (Utilities|Array|MakeArray "ObjectTypeQuery3") false 0 "None"))
      (for _array_element _outhits
        (bind _ascharacter (Utilities|Casting|CastToCharacter (.HitActor (Collision|BreakHitResult _array_element))))
        (bind _finalaoedamage (Default|ModifyAOEDamage (Variables|Default|GetUpgradeComponent) (Variables|Default|GetFinalWeaponDamage) (Utilities|Struct|MakeF_DamageContext (Variables|Default|GetAttacker) _ascharacter _returnvalue_2 (Math|Vector|GetUnitDirection(Vector) _returnvalue_2 (Transformation|GetActorLocation (.HitActor (Collision|BreakHitResult _array_element)))))))
        (Game|Damage|ApplyDamage (.HitActor (Collision|BreakHitResult _array_element)) _finalaoedamage 0 0)))))

(event EventBeginPlay
  (Utilities|Time|SetTimerbyEvent (delegate Custom|ApplyDamage) (Variables|Default|GetDelay)))

(fn ConstructionScript)