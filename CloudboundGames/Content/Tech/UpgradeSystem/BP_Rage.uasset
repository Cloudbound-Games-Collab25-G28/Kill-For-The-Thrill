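; BP_Rage is a stacking, timed upgrade that modifies its owner's movement speed and damage.
; Base modifier values and duration come from the owner's upgrades component, with additive terms scaled linearly by stacks and multipliers raised to the stack count.
; Each stack change restarts a single shared timer, which removes all Rage stacks at once when it expires.
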(event Custom|SetDurationTimer
  (bind _duration (Default|GetRageDuration (Variables|Default|GetOwner%20Upgrades%20Component)))
  (Utilities|Time|SetTimerbyEvent (delegate Custom|ClearRage) _duration))

(event Custom|ClearRage
  (bind _owner (Variables|Default|GetOwner))
  (bind _owner_upgrades_component (Variables|Default|GetOwner%20Upgrades%20Component))
  (Default|RemoveAllUpgradeStacks (Variables|Default|GetOwner%20Upgrades%20Component) self (Utilities|Struct|MakeF_UpgradeChangeContext _owner _owner_upgrades_component _owner _owner_upgrades_component)))

(fn Init
  (params (Context :type F%20Upgrade%20Change%20Context%20Structure))
  (bind (_changer _changerupgradescomponent _owner _ownerupgradescomponent) (Utilities|Struct|BreakF_UpgradeChangeContext Context))
  (|CallParentFunction Context)
  (Variables|Default|SetOwner _owner)
  (Variables|Default|SetOwner%20Upgrades%20Component _ownerupgradescomponent))

(fn StacksChanged
  (params (Context :type F%20Upgrade%20Change%20Context%20Structure))
  (CallFunction|SetDurationTimer))

(fn GetMovementSpeedModifier
  (params (Context :type F%20Movement%20Speed%20Context%20Structure))
  (bind _stacks (Variables|Default|GetStacks))
  (bind _modifier (Default|GetRageMovementSpeedModifier (Variables|Default|GetOwner%20Upgrades%20Component) Context))
  (return (Utilities|Struct|MakeF_ValueModifier (* (.add _modifier) _stacks) (* (.addproportion _modifier) _stacks) (Math|Float|Power (.multiply _modifier) (Math|Conversions|ToFloat(Integer) _stacks)))))

(fn GetDamageModifier
  (params (Context :type F%20Damage%20Context%20Structure))
  (bind _stacks (Variables|Default|GetStacks))
  (bind _modifier (Default|GetRageDamageModifier (Variables|Default|GetOwner%20Upgrades%20Component)))
  (return (Utilities|Struct|MakeF_ValueModifier (* (.add _modifier) _stacks) (* (.addproportion _modifier) _stacks) (Math|Float|Power (.multiply _modifier) (Math|Conversions|ToFloat(Integer) _stacks)))))