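; BP_Upgrade is the base upgrade in the upgrade system, a template of hooks that apply no effect by default.
; Modifier getters cover damage, crits, health, speed, agility, AOE, poison and rage, each receiving a Context.
; Most stat getters return a neutral Add, AddProportion and Multiply triple, while several poison, rage and max-stack getters have blank returns.
; Init, Removed and StacksChanged are empty lifecycle hooks.
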(fn GetDamageModifier
  (params (Context :type F%20Damage%20Context%20Structure))
  (return (Utilities|Struct|MakeF_ValueModifier 0.0 0.0 1.0)))

(fn GetCritProbability
  (params (Context :type F%20Damage%20Context%20Structure))
  (return 0.0))

(fn GetCritDamageModifier
  (params (Context :type F%20Damage%20Context%20Structure))
  (return (Utilities|Struct|MakeF_ValueModifier 0.0 0.0 1.0)))

(fn Init
  (params (Context :type F%20Upgrade%20Change%20Context%20Structure)))

(fn Removed
  (params (Context :type F%20Upgrade%20Change%20Context%20Structure)))

(fn GetMaxHealthModifier
  (params (Context :type F%20Max%20Health%20Context%20Structure))
  (return (Utilities|Struct|MakeF_ValueModifier 0.0 0.0 1.0)))

(fn GetMovementSpeedModifier
  (params (Context :type F%20Movement%20Speed%20Context%20Structure))
  (return (Utilities|Struct|MakeF_ValueModifier 0.0 0.0 1.0)))

(fn GetAttackSpeedModifier
  (params (Context :type F%20Attack%20Speed%20Context%20Structure))
  (return (Utilities|Struct|MakeF_ValueModifier 0.0 0.0 1.0)))

(fn GetAgilityModifier
  (params (Context :type F%20Damage%20Context%20Structure))
  (return (Utilities|Struct|MakeF_ValueModifier 0.0 0.0 1.0)))

(fn GetAOEDamageProportionModifier
  (params (Context :type F%20Damage%20Context%20Structure))
  (return (Utilities|Struct|MakeF_ValueModifier 0.0 0.0 1.0)))

(fn GetAOEAreaModifer
  (params (Context :type F%20Damage%20Context%20Structure))
  (return (Utilities|Struct|MakeF_ValueModifier 0.0 0.0 1.0)))

(fn GetAOEDamageModifier
  (params (Context :type F%20Damage%20Context%20Structure))
  (return (Utilities|Struct|MakeF_ValueModifier 0.0 0.0 1.0)))

(fn GetAOEDelayModifier
  (params (Context :type F%20Damage%20Context%20Structure))
  (return (Utilities|Struct|MakeF_ValueModifier 0.0 0.0 1.0)))

(fn GetUpgradesMaxApplyableStacks
  (params (Context :type F%20Upgrade%20Change%20Context%20Structure))
  (return 0))

(fn StacksChanged
  (params (Context :type F%20Upgrade%20Change%20Context%20Structure)))

(fn GetPoisonDurationModifier
  (params (Context :type F%20Status%20Effect%20Context%20Structure))
  (return ""))

(fn GetPoisonDamageModifier
  (params (Context :type F%20Status%20Effect%20Context%20Structure))
  (return ""))

(fn GetPoisonMovementSpeedModifier
  (params (Context :type F%20Status%20Effect%20Context%20Structure))
  (return ""))

(fn GetPoisonAgilityModifier
  (params (Context :type F%20Status%20Effect%20Context%20Structure))
  (return ""))

(fn GetPoisonDamageCooldownTimeModifier
  (params (Context :type F%20Status%20Effect%20Context%20Structure))
  (return ""))

(fn GetPoisonStacksAppliedonHit
  (params (Context :type F%20Damage%20Context%20Structure))
  (return 0))

(fn GetRageStacksReceivedonKill
  (params (Context :type F%20Status%20Effect%20Context%20Structure))
  (return 0))

(fn GetRageDurationModifier
  (params (Context :type F%20Status%20Effect%20Context%20Structure))
  (return ""))

(fn GetRageDamageModifier
  (params (Context :type F%20Status%20Effect%20Context%20Structure))
  (return ""))

(fn GetRageMovementSpeedModifier
  (params (Context :type F%20Movement%20Speed%20Context%20Structure))
  (return (Utilities|Struct|MakeF_ValueModifier 0.0 0.0 1.0)))