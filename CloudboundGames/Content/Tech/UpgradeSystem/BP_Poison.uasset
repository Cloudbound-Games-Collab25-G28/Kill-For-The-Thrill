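; Poison upgrade in the upgrade system that periodically damages its owner and sheds stacks over time.
; Init caches the applier's upgrades component and the owner, then starts separate damage and duration timers.
; Damage amount, cooldown and duration come from the applier's component, which also handles the stack removal call.
; Both timers re-arm themselves after firing instead of looping, so changes to cooldown and duration take effect.
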(event Custom|SetDurationTimer
  (bind _duration (Default|GetPoisonDuration (Variables|Default|GetApplyerUpgradesComponent)))
  (Utilities|Time|SetTimerbyEvent (delegate Custom|RemoveStack) _duration))

(event Custom|RemoveStack
  (bind _applyerupgradescomponent (Variables|Default|GetApplyerUpgradesComponent))
  (bind _owner (Variables|Default|GetOwner))
  (Default|RemoveUpgrade _applyerupgradescomponent self (Utilities|Struct|MakeF_UpgradeChangeContext _owner _applyerupgradescomponent _owner _applyerupgradescomponent))
  (CallFunction|SetDurationTimer) ; Done like this rather than with a looping timer to allow the duration to update
)

(event Custom|SetDamageTimer
  (bind _duration (Default|GetPoisonDamageCooldownTime (Variables|Default|GetApplyerUpgradesComponent)))
  (Utilities|Time|SetTimerbyEvent (delegate Custom|Damage) _duration))

(event Custom|Damage
  (bind _damage (Default|GetPoisonDamage (Variables|Default|GetApplyerUpgradesComponent)))
  (Game|Damage|ApplyDamage (Variables|Default|GetOwner) _damage 0 0)
  (CallFunction|SetDamageTimer) ; Done like this rather than with a looping timer to allow the cooldown to update
)

(fn Init
  (params (Context :type F%20Upgrade%20Change%20Context%20Structure))
  (bind (_changer _changerupgradescomponent _owner) (Utilities|Struct|BreakF_UpgradeChangeContext Context))
  (Variables|Default|SetApplyerUpgradesComponent _changerupgradescomponent)
  (Variables|Default|SetOwner _owner)
  (CallFunction|SetDurationTimer)
  (CallFunction|SetDamageTimer))