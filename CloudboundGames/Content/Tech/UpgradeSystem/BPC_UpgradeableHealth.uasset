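; BPC_UpgradeableHealth is a health component whose MaxHealth follows the owning actor's upgrades.
; On BeginPlay it runs the parent logic, finds BPC_Upgrades on the owner and binds UpdateMaxHealth to its OnUpgradesChanged dispatcher, printing a red error if that component is missing.
; Each upgrade change copies GetMaxHealth from the upgrades component into MaxHealth, with no initial sync in this graph.
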(event Custom|UpdateMaxHealth
  (bind _maxhealth (Default|GetMaxHealth (Variables|Default|GetUpgrades)))
  (Variables|Default|SetMaxHealth _maxhealth))

(event EventBeginPlay
  (bind _returnvalue (Components|GetOwner))
  (bind _returnvalue_2 (Actor|GetComponentbyClass _returnvalue "/Game/Tech/UpgradeSystem/BPC_Upgrades.BPC_Upgrades_C"))
  (|CallParentFunction)
  (Utilities|IsValid _returnvalue_2
    (:Is%20Valid
      (bind _output_get (Variables|Default|SetUpgrades _returnvalue_2))
      (EventDispatchers|AssignOnUpgradesChanged _output_get (delegate Custom|UpdateMaxHealth)))
    (:Is%20Not%20Valid
      (Development|PrintString "BPC_UpgradeableHealth requires BPC_Upgrades" true true "(R=1.000000,G=0.000000,B=0.000000,A=1.000000)"))))