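; Gamepad UI input Blueprint that routes controller navigation to the current UI and opens the pause menu.
; SendCurrentUIReference stores the active UI and prints its name.
; Bottom and right face buttons send it confirm and back-out messages; D-pad and left-stick directions share paths for directional messages, all guarded by validity checks.
; The right special button creates WBP_PauseMenu once, gated by IsPauseMenuActive, which this graph never clears.
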(event Custom|Send%20Current%20UI%20Reference
  (params (Current%20UI%20Reference :type Widget%20Object%20Reference))
  (bind _output_get (Variables|Default|SetCurrent%20UI%20Reference Current%20UI%20Reference))
  (Development|PrintString (Utilities|GetDisplayName _output_get) true true "(R=1.000000,G=0.000000,B=0.651997,A=1.000000)" 4.0))

(event Input|GamepadEvents|GamepadDPadDown
  (params (Key :type Key%20Structure :default "None"))
  (bind _current_ui_reference (Variables|Default|GetCurrent%20UI%20Reference))
  (:Pressed
    (Utilities|IsValid _current_ui_reference
      (:Is%20Valid
        (Class|BPIUIInputs|UIDown(Message) _current_ui_reference)))))

(event Input|GamepadEvents|GamepadDPadRight
  (params (Key :type Key%20Structure :default "None"))
  (bind _current_ui_reference (Variables|Default|GetCurrent%20UI%20Reference))
  (:Pressed
    (Utilities|IsValid _current_ui_reference
      (:Is%20Valid
        (Class|BPIUIInputs|UIRight(Message) _current_ui_reference)))))

(event Input|GamepadEvents|GamepadSpecialRight
  (params (Key :type Key%20Structure :default "None"))
  ;[1 1 1] Right middle button on controller
  (:Pressed
    (if (not (Variables|Default|GetIs%20Pause%20Menu%20Active?))
      (bind _returnvalue (UserInterface|CreateWidget "/Game/Tech/UI/Menus/WBP_PauseMenu.WBP_PauseMenu_C"))
      (Variables|Default|SetIs%20Pause%20Menu%20Active? true)
      (UserInterface|Viewport|AddtoViewport _returnvalue 0))))

(event Input|GamepadEvents|GamepadSpecialLeft
  (params (Key :type Key%20Structure :default "None"))
  ;[1 1 1] Left middle button on controller
)

(event Input|GamepadEvents|GamepadDPadLeft
  (params (Key :type Key%20Structure :default "None"))
  (bind _current_ui_reference (Variables|Default|GetCurrent%20UI%20Reference))
  (:Pressed
    (Utilities|IsValid _current_ui_reference
      (:Is%20Valid
        (Class|BPIUIInputs|UILeft(Message) _current_ui_reference)))))

(event Input|GamepadEvents|GamepadDPadUp
  (params (Key :type Key%20Structure :default "None"))
  (bind _current_ui_reference (Variables|Default|GetCurrent%20UI%20Reference))
  (:Pressed
    (Utilities|IsValid _current_ui_reference
      (:Is%20Valid
        (Class|BPIUIInputs|UIUp(Message) _current_ui_reference)))))

(event Input|GamepadEvents|GamepadFaceButtonBottom
  (params (Key :type Key%20Structure :default "None"))
  (bind _current_ui_reference (Variables|Default|GetCurrent%20UI%20Reference))
  ;[1 1 1] Confirm Button
  (:Pressed
    (Utilities|IsValid _current_ui_reference
      (:Is%20Valid
        (Class|BPIUIInputs|UIConfirm(Message) _current_ui_reference)))))

(event Input|GamepadEvents|GamepadLeftStickLeft
  (params (Key :type Key%20Structure :default "None"))
  (bind _current_ui_reference (Variables|Default|GetCurrent%20UI%20Reference))
  (:Pressed
    (Utilities|IsValid _current_ui_reference
      (:Is%20Valid
        (Class|BPIUIInputs|UILeft(Message) _current_ui_reference)))))

(event Input|GamepadEvents|GamepadLeftStickDown
  (params (Key :type Key%20Structure :default "None"))
  (bind _current_ui_reference (Variables|Default|GetCurrent%20UI%20Reference))
  (:Pressed
    (Utilities|IsValid _current_ui_reference
      (:Is%20Valid
        (Class|BPIUIInputs|UIDown(Message) _current_ui_reference)))))

(event Input|GamepadEvents|GamepadLeftStickRight
  (params (Key :type Key%20Structure :default "None"))
  (bind _current_ui_reference (Variables|Default|GetCurrent%20UI%20Reference))
  (:Pressed
    (Utilities|IsValid _current_ui_reference
      (:Is%20Valid
        (Class|BPIUIInputs|UIRight(Message) _current_ui_reference)))))

(event Input|GamepadEvents|GamepadLeftStickUp
  (params (Key :type Key%20Structure :default "None"))
  (bind _current_ui_reference (Variables|Default|GetCurrent%20UI%20Reference))
  (:Pressed
    (Utilities|IsValid _current_ui_reference
      (:Is%20Valid
        (Class|BPIUIInputs|UIUp(Message) _current_ui_reference)))))

(event Input|GamepadEvents|GamepadFaceButtonRight
  (params (Key :type Key%20Structure :default "None"))
  (bind _current_ui_reference (Variables|Default|GetCurrent%20UI%20Reference))
  ;[1 1 1] UnConfirm Button
  (:Pressed
    (Utilities|IsValid _current_ui_reference
      (:Is%20Valid
        (Class|BPIUIInputs|UIBackOut(Message) _current_ui_reference)))))