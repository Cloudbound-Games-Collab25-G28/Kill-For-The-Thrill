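; Player weapon component that spawns the chosen melee or crossbow weapon and routes attack input to it.
; SelectWeapon attaches a sword, voulge or crossbow actor to the character's hand socket, then enables input, which BeginPlay disables until then.
; Releasing or canceling the held attack turns the owner toward the mouse via a ray-plane intersection, then fires a normal or charged attack based on hold time.
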(event Input|EnhancedActionEvents|EnhancedInputActionIA_WeaponAttack_Held
  (params (ActionValue :type Boolean) (ElapsedSeconds :type Float%20%28double-precision%29) (TriggeredSeconds :type Float%20%28double-precision%29) (InputAction :type Input%20Action%20Object%20Reference :default "/Game/Tech/Weapons/Wep_Inputs/IA_WeaponAttack_Held.IA_WeaponAttack_Held"))
  (:Canceled
    (CallFunction|LookattheMouse :!label _label)
    (if (>= ElapsedSeconds 0.25)
      (CallFunction|ChargedAttackFunction (Math|Float|Clamp(Float) (* ElapsedSeconds 1.0)))
      (else
        (Default|AttackwiththeWeapon (Variables|Default|GetCurrent%20Weapon%20Reference)))))
  (:Completed
    (goto _label)))

(event EventBeginPlay
  (Input|DisableInput (Components|GetOwner) (Game|GetPlayerController 0)))

(fn ChargedAttackFunction
  (params (Input%20Float :type Float%20%28double-precision%29))
  ;[1 1 1] Alternative action for using the BP parent function version
  (if (>= Input%20Float 0.25)
    (Default|ChargedAttackWeaponFunction (Variables|Default|GetCurrent%20Weapon%20Reference) (Math|Float|Clamp(Float) (* Input%20Float 1.0)))))

(fn SendReferenceForce
  (return 0))

(fn SelectWeapon
  (params (Weapon%20Enum :type E_WeaponType%20Enum :default "NewEnumerator0"))
  (bind _asbp_player_character (Utilities|Casting|CastToBP_PlayerCharacter (Components|GetOwner)))
  (switch Utilities|FlowControl|Switch|SwitchonE_WeaponType Weapon%20Enum
    (:NewEnumerator0
      (Variables|Default|SetWeapon%20Class%20To%20Use "/Game/Tech/Weapons/WeaponTypes/BP_SwordWepV2.BP_SwordWepV2_C"))
    (:NewEnumerator1
      (Variables|Default|SetWeapon%20Class%20To%20Use "/Game/Tech/Weapons/WeaponTypes/BP_SpearWepV2.BP_SpearWepV2_C"))
    (:NewEnumerator2
      (Variables|Default|SetWeapon%20Class%20To%20Use "/Game/Tech/Weapons/WeaponTypes/BP_CrossBowWepV2.BP_CrossBowWepV2_C")))
  (bind _returnvalue (Game|SpawnActorfromClass (Variables|Default|GetWeapon%20Class%20To%20Use) (Math|Transform|MakeTransform "1000.000000,1810.000000,100.000000" "0, 0, 0" "1.000000,1.000000,1.000000") "AlwaysSpawn" "MultiplyWithRoot" _asbp_player_character 0))
  (Transformation|AttachComponentToComponent _returnvalue (Actor|GetComponentbyClass (Components|GetOwner) "/Script/Engine.SkeletalMeshComponent") "hand_rSocketV2" "SnapToTarget" "KeepWorld" "SnapToTarget" true)
  (Variables|Default|SetCurrent%20Weapon%20Reference _returnvalue)
  (Variables|/Game/Tech/Weapons/WeaponTypes/BaseClass/BP_BaseWepClass.BP_BaseWepClass_C|SetPlayer%20Reference _returnvalue _asbp_player_character)
  (Input|EnableInput (Components|GetOwner) (Game|GetPlayerController 0)))

(fn LookattheMouse
  (bind _returnvalue (Game|GetPlayerController 0))
  (bind _returnvalue_2 (Components|GetOwner))
  (bind (_worldlocation _worlddirection) (Game|Player|ConvertMouseLocationToWorldSpace _returnvalue))
  (bind _returnvalue_3 (Transformation|GetActorLocation _returnvalue_2))
  (Transformation|SetActorRotation _returnvalue_2 (Math|Rotator|FindLookatRotation _returnvalue_3 (.Intersection (Class|KismetMathLibrary|LinePlaneIntersectionOriginNormal _worldlocation (+ (* _worlddirection 1e+05) _worldlocation) _returnvalue_3 "0.000000,0.000000,1.000000"))))
  (return))

(fn GetCurrentReference
  (return 0))