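; Actor component that gives its owner a spear and handles weapon attack input, filed under old weapon code.
; On BeginPlay it spawns BP_SpearWepV2 at the skeletal mesh's hand socket and attaches it, but sets CurrentWeaponReference to None.
; Releasing or canceling held attack input fires OnAttackOld, then calls a normal or charged attack on CurrentWeaponReference by hold time.
; SendReferenceForce and GetCurrentReference are empty stubs.
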(event Input|EnhancedActionEvents|EnhancedInputActionIA_WeaponAttack_Held
  (params (ActionValue :type Boolean) (ElapsedSeconds :type Float%20%28double-precision%29) (TriggeredSeconds :type Float%20%28double-precision%29) (InputAction :type Input%20Action%20Object%20Reference :default "/Game/Tech/Input/IA_WeaponAttack_Held.IA_WeaponAttack_Held"))
  (:Canceled
    (Default|CallOnAttackOld :!label _label)
    ;[1 1 1] Is the button held/charging?
    (if (>= ElapsedSeconds 0.25)
      (Default|ChargedAttackWeapon (Variables|Default|GetCurrent%20Weapon%20Reference) (Math|Float|Clamp(Float) (* ElapsedSeconds 1.0)))
      (else
        (Default|AttackwiththeWeapon (Variables|Default|GetCurrent%20Weapon%20Reference)))))
  (:Completed
    (goto _label)))

(event EventBeginPlay
  (CallFunction|SetupWeapon))

(fn ChargedAttackFunction
  (params (Input%20Float :type Float%20%28double-precision%29))
  ;[1 1 1] Alternative action for using the BP parent function version
  (if (>= Input%20Float 0.25)
    (Default|ChargedAttackWeapon (Variables|Default|GetCurrent%20Weapon%20Reference) (Math|Float|Clamp(Float) (* Input%20Float 1.0)))))

(fn SendReferenceForce
  (return 0))

(fn SetupWeapon
  (bind _returnvalue (Components|GetOwner))
  (bind _returnvalue_2 (Actor|GetComponentbyClass _returnvalue "/Script/Engine.SkeletalMeshComponent"))
  (Variables|Default|SetSkeletalMeshReference _returnvalue_2)
  (bind _returnvalue_3 (Game|SpawnActorfromClass "/Game/Tech/Weapons/WeaponTypes/BP_SpearWepV2.BP_SpearWepV2_C" (Transformation|GetSocketTransform _returnvalue_2 "hand_rSocket" "RTS_World") "AdjustIfPossibleButAlwaysSpawn" "MultiplyWithRoot" _returnvalue 0))
  (Transformation|AttachComponentToComponent _returnvalue_3 _returnvalue_2 "hand_rSocket" "SnapToTarget" "SnapToTarget" "SnapToTarget" true)
  (Variables|Default|SetCurrent%20Weapon%20Reference 0))

(fn GetCurrentReference
  (return 0))