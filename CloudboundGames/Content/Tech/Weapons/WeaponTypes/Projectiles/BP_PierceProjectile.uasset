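; Piercing weapon projectile that damages actors it overlaps without being destroyed on contact.
; A looping-free timer started on BeginPlay uses LifeTime to limit the projectile's lifespan, with ProjectileLifeTimesUp destroying it.
; Sphere overlaps take the hit actor from the sweep result, filter it through an equality check, apply rounded base damage with the configured damage type, and print a debug message.
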(event OnComponentBeginOverlap(Sphere)
  (params (OverlappedComponent :type Primitive%20Component%20Object%20Reference) (OtherActor :type Actor%20Object%20Reference) (OtherComp :type Primitive%20Component%20Object%20Reference) (OtherBodyIndex :type Integer) (bFromSweep :type Boolean) (SweepResult :type Hit%20Result%20Structure%20%28by%20ref%29))
  (bind _hitactor (Collision|BreakHitResult SweepResult))
  (if (not (== _hitactor 0))
    (Game|Damage|ApplyDamage _hitactor (Math|Conversions|ToFloat(Integer) (Math|Float|Round (Variables|Default|GetBase%20Damage%20Amount))) 0 0 "/Script/Engine.DamageType")
    (Development|PrintString (Utilities|String|Append "Damage dealt to" (Utilities|GetDisplayName _hitactor)))))

(event Custom|Projectile%20LifeTimes%20Up
  (Actor|DestroyActor)
  (Utilities|Time|ClearandInvalidateTimerbyHandle (stale EventBeginPlay _returnvalue)))

(event EventBeginPlay
  (bind _returnvalue (Utilities|Time|SetTimerbyEvent (EventDispatchers|CreateEvent :!event Custom|Projectile%20LifeTimes%20Up) (Variables|Default|GetLife%20Time) false true)))

(fn ConstructionScript)