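; Area-of-effect projectile that damages nearby objects when its sphere begins overlapping, then destroys itself.
; The overlap runs a multi-sphere trace at the actor's location, ignoring itself, its owner and instigator, and applies damage to the hits.
; DestroyActor is also called inside the hit loop; debug trace drawing and damage prints are enabled.
; A timer started on BeginPlay is set to the projectile's lifetime, with an expiry event that destroys it.
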(event OnComponentBeginOverlap(Sphere)
  (params (OverlappedComponent :type Primitive%20Component%20Object%20Reference) (OtherActor :type Actor%20Object%20Reference) (OtherComp :type Primitive%20Component%20Object%20Reference) (OtherBodyIndex :type Integer) (bFromSweep :type Boolean) (SweepResult :type Hit%20Result%20Structure%20%28by%20ref%29))
  (bind _self self)
  (bind _returnvalue (Transformation|GetActorLocation _self))
  (bind _outhits (Collision|MultiSphereTraceForObjects _returnvalue _returnvalue 2e+02 (Variables|Default|GetObject%20types) false (Utilities|Array|MakeArray (Variables|Actor|GetInstigator) self (Components|GetOwner)) "ForDuration" true "(R=0.060860,G=0.000000,B=1.000000,A=1.000000)" "(R=0.000000,G=1.000000,B=0.000000,A=1.000000)" 1.0))
  (for _array_element _outhits
    (Game|Damage|ApplyDamage (.HitActor (Collision|BreakHitResult _array_element)) (Math|Conversions|ToFloat(Integer) (Math|Float|Round (Variables|Default|GetBase%20Damage%20Amount))) 0 0 "/Script/Engine.DamageType")
    (Development|PrintString (Utilities|String|Append "Damage dealt to" (Utilities|GetDisplayName (.HitActor (Collision|BreakHitResult _array_element)))))
    (Actor|DestroyActor))
  (Actor|DestroyActor))

(event Custom|Projectiles%20LifeTime%20is%20Up
  (Actor|DestroyActor)
  (Utilities|Time|ClearandInvalidateTimerbyHandle (stale EventBeginPlay _returnvalue)))

(event EventBeginPlay
  (bind _returnvalue (Utilities|Time|SetTimerbyEvent (EventDispatchers|CreateEvent :!event Custom|Projectiles%20LifeTime%20is%20Up) (Variables|Default|GetLife%20Time) false true)))

(fn ConstructionScript)