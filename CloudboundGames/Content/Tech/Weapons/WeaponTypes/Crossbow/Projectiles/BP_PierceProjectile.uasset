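; BP_PierceProjectile is a crossbow projectile that damages actors it passes over without being destroyed on contact.
; Its Sphere overlap applies damage to each overlapped actor, crediting the instigator's controller, and prints a debug message naming the target.
; A timer started on BeginPlay destroys the projectile when its lifetime runs out.
; The overlap handler has no filtering of the actors it damages.
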(event OnComponentBeginOverlap(Sphere)
  (params (OverlappedComponent :type Primitive%20Component%20Object%20Reference) (OtherActor :type Actor%20Object%20Reference) (OtherComp :type Primitive%20Component%20Object%20Reference) (OtherBodyIndex :type Integer) (bFromSweep :type Boolean) (SweepResult :type Hit%20Result%20Structure%20%28by%20ref%29))
  (Game|Damage|ApplyDamage OtherActor (Variables|Default|GetBase%20Damage%20Amount) (Game|GetInstigatorController) self "/Script/Engine.DamageType")
  (Development|PrintString (Utilities|String|Append "Damage dealt to" (Utilities|GetDisplayName OtherActor))))

(event Custom|Projectile%20LifeTimes%20Up
  (Actor|DestroyActor)
  (Utilities|Time|ClearandInvalidateTimerbyHandle (stale EventBeginPlay _returnvalue)))

(event EventBeginPlay
  (bind _returnvalue (Utilities|Time|SetTimerbyEvent (delegate Custom|Projectile%20LifeTimes%20Up) (Variables|Default|GetLife%20Time) false true)))

(fn ConstructionScript)