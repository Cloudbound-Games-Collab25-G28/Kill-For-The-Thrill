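; Sword-and-shield weapon variant whose three-hit combo and charged shield bash also fire a short-lived projectile.
; Every attack calls a shared function that spawns the projectile at half damage, plays the attack montage and box-traces that attack's hitbox to apply damage through the player's upgrades component.
; Charging makes the player invincible as a block until release or end.
; Releasing within a narrow charge window gives a stronger perfect bash with its own hitbox.
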(event Custom|Start%20Blocking
  (Class|HealthComponent|SetInvincibility (Variables|/Game/Tech/Player/BP_PlayerCharacter.BP_PlayerCharacter_C|GetBPC_UpgradeableHealth (Variables|Default|GetPlayer%20Reference)) true))

(event Custom|Allow%20player%20to%20take%20damage%20again
  (Class|HealthComponent|SetInvincibility (Variables|/Game/Tech/Player/BP_PlayerCharacter.BP_PlayerCharacter_C|GetBPC_UpgradeableHealth (Variables|Default|GetPlayer%20Reference)) false))

(fn ConstructionScript
  (|CallParentFunction))

(fn RegularComboSwapper
  (|CallParentFunction))

(fn RegularCombo1
  (CallFunction|DamageObjectinRangeBoxesV2 (+ (Variables|Default|GetBase%20Damage%20Amount) (Variables|Default|GetCombo%201%20Damage)) (Variables|Default|GetAttack%201%20Combo)))

(fn RegularCombo2
  (CallFunction|DamageObjectinRangeBoxesV2 (+ (Variables|Default|GetBase%20Damage%20Amount) (Variables|Default|GetCombo%202%20Damage)) (Variables|Default|GetAttack%202%20Combo)))

(fn RegularCombo3
  (CallFunction|DamageObjectinRangeBoxesV2 (+ (Variables|Default|GetBase%20Damage%20Amount) (Variables|Default|GetCombo%203%20Damage)) (Variables|Default|GetAttack%203%20Combo)))

(fn ChargedAttackScaling
  (params (Charged%20Amount :type Float%20%28double-precision%29))
  ;[1 1 1] Scaling Numeral amount from 0.1 to 1.0, used for charged attacks currently.
  (if (and (> Charged%20Amount 1.0) (< Charged%20Amount 1.25))
    (CallFunction|DamageObjectinRangeBoxesV2 1.5e+02 (Variables|Default|GetPerfect%20Shield%20Bash%20Radius))
    (else
      (CallFunction|DamageObjectinRangeBoxesV2 5e+01 (Variables|Default|GetShield%20Bash%20Radius))))
  (CallFunction|AllowPlayertoTakeDamageAgain)
  (CallFunction|ChargeCompleted))

(fn DamageObjectinRangeBoxesV2
  (params (BaseDamage :type Float%20%28single-precision%29) (Attack%20Combo :type Box%20Component%20Object%20Reference))
  (bind _returnvalue (Transformation|GetRelativeTransform Attack%20Combo))
  (bind _player_reference (Variables|Default|GetPlayer%20Reference))
  (bind _player_reference_2 (Variables|Default|GetPlayer%20Reference))
  (bind _weapon_arrow_placeholder (Variables|/Game/Tech/Player/BP_PlayerCharacter.BP_PlayerCharacter_C|GetWeapon%20Arrow%20PlaceHolder _player_reference))
  (bind _returnvalue_2 (Transformation|GetWorldTransform _weapon_arrow_placeholder))
  (bind _returnvalue_3 (Math|Transform|TransformLocation _returnvalue_2 (.location _returnvalue)))
  ;[1 1 1] Used for the hurtboxes of the sword when attacking (Attack Combo 1-3)
  (Game|SpawnActorfromClass "/Game/Tech/Weapons/WeaponTypes/Projectiles/BP_SwordProjectile.BP_SwordProjectile_C" (Transformation|GetWorldTransform (Variables|/Game/Tech/Player/BP_PlayerCharacter.BP_PlayerCharacter_C|GetWeapon%20Arrow%20PlaceHolder (Variables|Default|GetPlayer%20Reference))) "AlwaysSpawn" "MultiplyWithRoot" 0 (/ BaseDamage 2.0) 0.3 (Variables|Default|GetPlayer%20Reference))
  (Animation|PlayAnimMontage (Variables|Default|GetPlayer%20Reference) (Variables|Default|GetAttackAnimation) 1.0 "None")
  (bind _outhits (Class|KismetSystemLibrary|BoxTraceMultiforObjects _returnvalue_3 _returnvalue_3 (Variables|/Script/Engine.BoxComponent|GetBoxExtent Attack%20Combo) (Math|Rotator|MakeRotator 0.0 0.0 (+ (Variables|Default|GetZ%20Rotation) (.yaw (.rotation _returnvalue)))) (Variables|Default|Getobject%20types) false (Utilities|Array|MakeArray (Variables|Default|GetPlayer%20Reference)) "ForDuration" true "(R=1.000000,G=0.000000,B=0.121054,A=1.000000)" "(R=0.000000,G=1.000000,B=0.000000,A=1.000000)" 0.2))
  (for _array_element _outhits
    (Default|ApplyWeaponDamage (Variables|/Game/Tech/Player/BP_PlayerCharacter.BP_PlayerCharacter_C|GetBPC_Upgrades _player_reference_2) BaseDamage (Utilities|Struct|MakeF_DamageContext _player_reference_2 (.HitActor (Collision|BreakHitResult _array_element)) _returnvalue_3 "0.000000,0.000000,0.000000"))
    (Development|PrintString (Utilities|String|Append "Damage dealt to" (Utilities|GetDisplayName (.HitActor (Collision|BreakHitResult _array_element)))))
    (CallFunction|AfterAttack))
  (CallFunction|AfterAttack))

(fn ChargeAttackOngoing
  (params (Charged%20Amount :type Float%20%28double-precision%29))
  (CallFunction|ChargeStarted)
  (CallFunction|StartBlocking))

(fn ChargeAttackEnded
  (CallFunction|AllowPlayertoTakeDamageAgain))