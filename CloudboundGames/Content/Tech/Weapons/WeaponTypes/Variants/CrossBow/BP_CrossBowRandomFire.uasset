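; Crossbow weapon variant that fires a random projectile type (short, AoE or pierce) on each normal or charged attack.
; All three combo steps share one fire function, which randomizes damage and lifetime, then slows the player.
; Charging past a threshold traces below the player to place an arrow decal that follows player rotation.
; The charged shot also randomizes scale and charge-based damage multipliers, then removes the decal.
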(fn ConstructionScript
  (|CallParentFunction))

(fn RegularComboSwapper
  ;[1 1 1] This is the parent function (can be changed if using only one combo)
  (switch int (Variables|Default|GetLocal%20Index%20Attack%20Combo)
    (:0
      (Variables|Default|SetLocal%20Index%20Attack%20Combo 1)
      (CallFunction|RegularCombo1))
    (:1
      (Variables|Default|SetLocal%20Index%20Attack%20Combo 2)
      (CallFunction|RegularCombo2))
    (:2
      (Variables|Default|SetLocal%20Index%20Attack%20Combo 0)
      (CallFunction|RegularCombo3))))

(fn RegularCombo1
  (CallFunction|FireProjectileBasic))

(fn RegularCombo2
  (CallFunction|FireProjectileBasic))

(fn RegularCombo3
  (CallFunction|FireProjectileBasic))

(fn FireProjectileBasic
  (bind _int (CallFunction|RandomizeNormalAttack))
  (Animation|PlayAnimMontage (Variables|Default|GetPlayer%20Reference) "/Game/Art/PlayableCharacter/Duck-Final/Animations/Weapons/Crossbow_Animations/AM_Crossbow_Hit_1_Montage.AM_Crossbow_Hit_1_Montage" 1.0 "None")
  (switch int _int
    (:1
      (Game|SpawnActorfromClass "/Game/Tech/Weapons/WeaponTypes/Projectiles/BP_ShortProjectile.BP_ShortProjectile_C" (Transformation|GetWorldTransform (Variables|/Game/Tech/Player/BP_PlayerCharacter.BP_PlayerCharacter_C|GetWeapon%20Arrow%20PlaceHolder (Variables|Default|GetPlayer%20Reference))) "AlwaysSpawn" "MultiplyWithRoot" 0 (+ (Variables|Default|GetBase%20Damage%20Amount) (Variables|Default|GetCombo%20Projectile%20Damge%20Amount)) (Variables|Default|GetProjectile%20Lifetime) (Variables|Default|GetPlayer%20Reference)))
    (:2
      (Game|SpawnActorfromClass "/Game/Tech/Weapons/WeaponTypes/Projectiles/BP_AoeProjectile.BP_AoeProjectile_C" (Transformation|GetWorldTransform (Variables|/Game/Tech/Player/BP_PlayerCharacter.BP_PlayerCharacter_C|GetWeapon%20Arrow%20PlaceHolder (Variables|Default|GetPlayer%20Reference))) "AlwaysSpawn" "MultiplyWithRoot" 0 (+ (Variables|Default|GetBase%20Damage%20Amount) (Variables|Default|GetCombo%20Projectile%20Damge%20Amount)) (Variables|Default|GetProjectile%20Lifetime) (Variables|Default|GetPlayer%20Reference)))
    (:3
      (Game|SpawnActorfromClass "/Game/Tech/Weapons/WeaponTypes/Projectiles/BP_PierceProjectile.BP_PierceProjectile_C" (Transformation|GetWorldTransform (Variables|/Game/Tech/Player/BP_PlayerCharacter.BP_PlayerCharacter_C|GetWeapon%20Arrow%20PlaceHolder (Variables|Default|GetPlayer%20Reference))) "AlwaysSpawn" "MultiplyWithRoot" 0 (+ (Variables|Default|GetBase%20Damage%20Amount) (Variables|Default|GetCombo%20Projectile%20Damge%20Amount)) (Variables|Default|GetProjectile%20Lifetime) (Variables|Default|GetPlayer%20Reference))))
  (CallFunction|SlowPlayeronAttack))

(fn ChargedAttackScaling
  (params (Charged%20Amount :type Float%20%28double-precision%29))
  (bind _int (CallFunction|RandomizeChargedAttack))
  (Animation|PlayAnimMontage (Variables|Default|GetPlayer%20Reference) "/Game/Art/PlayableCharacter/Duck-Final/Animations/Weapons/Crossbow_Animations/AM_Crossbow_Hit_1_Montage.AM_Crossbow_Hit_1_Montage" 1.0 "None")
  (switch int _int
    (:1
      (bind _returnvalue (Game|SpawnActorfromClass "/Game/Tech/Weapons/WeaponTypes/Projectiles/BP_PierceProjectile.BP_PierceProjectile_C" (Transformation|GetWorldTransform (Variables|/Game/Tech/Player/BP_PlayerCharacter.BP_PlayerCharacter_C|GetWeapon%20Arrow%20PlaceHolder (Variables|Default|GetPlayer%20Reference))) "AlwaysSpawn" "OverrideRootScale" 0 (+ (+ (Variables|Default|GetBase%20Damage%20Amount) (Variables|Default|GetAdditional%20Damage)) (* (* Charged%20Amount (Variables|Default|GetMultiplier%201)) (Variables|Default|GetMultiplier%202))) (Variables|Default|GetProjectile%20Lifetime) (Variables|Default|GetPlayer%20Reference)))
      (Transformation|SetActorScale3D _returnvalue (Variables|Default|GetSizeScale))
      (Variables|Default|SetClose%20Boolean true)
      (Components|DestroyComponent (Variables|Default|GetCurrent%20Decal)))
    (:2
      (bind _returnvalue_2 (Game|SpawnActorfromClass "/Game/Tech/Weapons/WeaponTypes/Projectiles/BP_AoeProjectile.BP_AoeProjectile_C" (Transformation|GetWorldTransform (Variables|/Game/Tech/Player/BP_PlayerCharacter.BP_PlayerCharacter_C|GetWeapon%20Arrow%20PlaceHolder (Variables|Default|GetPlayer%20Reference))) "AlwaysSpawn" "OverrideRootScale" 0 (+ (+ (Variables|Default|GetBase%20Damage%20Amount) (Variables|Default|GetAdditional%20Damage)) (* (* Charged%20Amount (Variables|Default|GetMultiplier%201)) (Variables|Default|GetMultiplier%202))) (Variables|Default|GetProjectile%20Lifetime) (Variables|Default|GetPlayer%20Reference)))
      (Transformation|SetActorScale3D _returnvalue_2 (Variables|Default|GetSizeScale))
      (Variables|Default|SetClose%20Boolean true)
      (Components|DestroyComponent (Variables|Default|GetCurrent%20Decal)))
    (:3
      (bind _returnvalue_3 (Game|SpawnActorfromClass "/Game/Tech/Weapons/WeaponTypes/Projectiles/BP_ShortProjectile.BP_ShortProjectile_C" (Transformation|GetWorldTransform (Variables|/Game/Tech/Player/BP_PlayerCharacter.BP_PlayerCharacter_C|GetWeapon%20Arrow%20PlaceHolder (Variables|Default|GetPlayer%20Reference))) "AlwaysSpawn" "OverrideRootScale" 0 (+ (+ (Variables|Default|GetBase%20Damage%20Amount) (Variables|Default|GetAdditional%20Damage)) (* (* Charged%20Amount (Variables|Default|GetMultiplier%201)) (Variables|Default|GetMultiplier%202))) (Variables|Default|GetProjectile%20Lifetime) (Variables|Default|GetPlayer%20Reference)))
      (Transformation|SetActorScale3D _returnvalue_3 (Variables|Default|GetSizeScale))
      (Variables|Default|SetClose%20Boolean true)
      (Components|DestroyComponent (Variables|Default|GetCurrent%20Decal))))
  (CallFunction|ChargeCompleted))

(fn ChargeAttackOngoing
  (params (Charged%20Amount :type Float%20%28double-precision%29))
  (bind _player_reference (Variables|Default|GetPlayer%20Reference))
  (bind _capsulecomponent (Variables|/Script/Engine.Character|GetCapsuleComponent _player_reference))
  (bind _returnvalue (Transformation|GetWorldTransform _capsulecomponent))
  (Utilities|FlowControl|Sequence
    (:then_0
      (if (> Charged%20Amount 0.5)
        (if (Variables|Default|GetClose%20Boolean)
          (Variables|Default|SetClose%20Boolean false)
          (CallFunction|ChargeStarted)
          (bind _outhit (Collision|LineTraceByChannel (.location _returnvalue) (+ (.location _returnvalue) (* (* (Math|Vector|GetUpVector (.rotation _returnvalue)) -1.0) 1e+05)) "TraceTypeQuery1" false 0 "ForDuration"))
          (bind _returnvalue_2 (Rendering|Decal|SpawnDecalatLocation "/Game/Tech/Weapons/M_DecalArrow.M_DecalArrow" "100.000000,100.000000,100.000000" (.Location (Collision|BreakHitResult _outhit)) (Math|Conversions|RotationFromXVector (.Normal (Collision|BreakHitResult _outhit))) 0.0))
          (Variables|Default|SetCurrent%20Decal _returnvalue_2))))
    (:then_1
      (Utilities|IsValid (Variables|Default|GetCurrent%20Decal)
        (:Is%20Valid
          (Transformation|SetWorldRotation (Variables|Default|GetCurrent%20Decal) (.rotation _returnvalue) false false))))))

(fn RandomizeNormalAttack
  (Variables|Default|SetCombo%20Projectile%20Damge%20Amount (Math|Random|RandomFloatinRange 5.0 4e+01))
  (Variables|Default|SetProjectile%20Lifetime (Math|Random|RandomFloatinRange 0.1 0.4))
  (return (Math|Random|RandomIntegerinRange 1 3)))

(fn RandomizeChargedAttack
  (Variables|Default|SetAdditional%20Damage (Math|Random|RandomIntegerinRange 20 160))
  (Variables|Default|SetMultiplier%201 (Math|Random|RandomIntegerinRange 1 5))
  (Variables|Default|SetMultiplier%202 (Math|Random|RandomIntegerinRange 1 2))
  (Variables|Default|SetProjectile%20Lifetime (Math|Random|RandomFloatinRange 0.2 0.5))
  (Variables|Default|SetSizeScale (Math|Conversions|ToVector(Float) (Math|Random|RandomIntegerinRange 1 3)))
  (return (Math|Random|RandomIntegerinRange 1 3)))