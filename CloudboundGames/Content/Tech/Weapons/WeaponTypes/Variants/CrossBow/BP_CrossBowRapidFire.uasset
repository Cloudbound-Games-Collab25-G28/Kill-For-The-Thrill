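; Rapid-fire crossbow weapon variant that shoots short-lived piercing projectiles from the player's arrow placeholder.
; The three-step regular combo fires one identical shot per step.
; Charging past halfway starts a looping timer for repeated shots and traces down to place an arrow decal on the ground, which follows the player capsule's rotation.
; The charged-attack scaling override stops the timer, resets the one-shot gate and destroys the decal.
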(event Custom|Start%20Rapid%20Fire
  (bind _returnvalue (Utilities|Time|SetTimerbyEvent (EventDispatchers|CreateEvent self :!event Custom|Rapid%20Fire) (Variables|Default|GetAttack%20Spam%20Delay) true true)))

(event Custom|Rapid%20Fire
  (Game|SpawnActorfromClass "/Game/Tech/Weapons/WeaponTypes/Projectiles/BP_PierceProjectile.BP_PierceProjectile_C" (Transformation|GetWorldTransform (Variables|/Game/Tech/Player/BP_PlayerCharacter.BP_PlayerCharacter_C|GetWeapon%20Arrow%20PlaceHolder (Variables|Default|GetPlayer%20Reference))) "AlwaysSpawn" "MultiplyWithRoot" 0 (+ (Variables|Default|GetBase%20Damage%20Amount) (Variables|Default|GetCombo%20Projectile%20Damge%20Amount)) 0.2 (Variables|Default|GetPlayer%20Reference)))

(event Custom|Rapid%20Fire%20Ended
  (Utilities|Time|ClearandInvalidateTimerbyHandle (stale Custom|Start%20Rapid%20Fire _returnvalue)))

(fn ConstructionScript
  (|CallParentFunction))

(fn RegularComboSwapper
  ;[1 1 1] This is the parent function (can be changed if using only one combo)
  (switch int (Variables|Default|GetLocal%20Index%20Attack%20Combo)
    (:0
      (Variables|Default|SetLocal%20Index%20Attack%20Combo 1)
      (CallFunction|RegularCombo1))
    (:1
      (Variables|Default|SetLocal%20Index%20Attack%20Combo 2)
      (CallFunction|RegularCombo2))
    (:2
      (Variables|Default|SetLocal%20Index%20Attack%20Combo 0)
      (CallFunction|RegularCombo3))))

(fn RegularCombo1
  (CallFunction|FireProjectileBasic))

(fn RegularCombo2
  (CallFunction|FireProjectileBasic))

(fn RegularCombo3
  (CallFunction|FireProjectileBasic))

(fn FireProjectileBasic
  (Game|SpawnActorfromClass "/Game/Tech/Weapons/WeaponTypes/Projectiles/BP_PierceProjectile.BP_PierceProjectile_C" (Transformation|GetWorldTransform (Variables|/Game/Tech/Player/BP_PlayerCharacter.BP_PlayerCharacter_C|GetWeapon%20Arrow%20PlaceHolder (Variables|Default|GetPlayer%20Reference))) "AlwaysSpawn" "MultiplyWithRoot" 0 (+ (Variables|Default|GetBase%20Damage%20Amount) (Variables|Default|GetCombo%20Projectile%20Damge%20Amount)) 0.2 (Variables|Default|GetPlayer%20Reference)))

(fn ChargedAttackScaling
  (params (Charged%20Amount :type Float%20%28double-precision%29))
  (CallFunction|RapidFireEnded)
  (Variables|Default|SetClose%20Boolean true)
  (Components|DestroyComponent (Variables|Default|GetCurrent%20Decal)))

(fn ChargeAttackOngoing
  (params (Charged%20Amount :type Float%20%28double-precision%29))
  (bind _player_reference (Variables|Default|GetPlayer%20Reference))
  (bind _capsulecomponent (Variables|/Script/Engine.Character|GetCapsuleComponent _player_reference))
  (bind _returnvalue (Transformation|GetWorldTransform _capsulecomponent))
  (Utilities|FlowControl|Sequence
    (:then_0
      (if (> Charged%20Amount 0.5)
        (if (Variables|Default|GetClose%20Boolean)
          (Variables|Default|SetClose%20Boolean false)
          (CallFunction|ChargeStarted)
          (CallFunction|StartRapidFire)
          (bind _outhit (Collision|LineTraceByChannel (.location _returnvalue) (+ (.location _returnvalue) (* (* (Math|Vector|GetUpVector (.rotation _returnvalue)) -1.0) 1e+05)) "TraceTypeQuery1" false 0 "ForDuration"))
          (bind _returnvalue_2 (Rendering|Decal|SpawnDecalatLocation "/Game/Tech/Weapons/M_DecalArrow.M_DecalArrow" "100.000000,100.000000,100.000000" (.Location (Collision|BreakHitResult _outhit)) (Math|Conversions|RotationFromXVector (.Normal (Collision|BreakHitResult _outhit))) 0.0))
          (Variables|Default|SetCurrent%20Decal _returnvalue_2))))
    (:then_1
      (Utilities|IsValid (Variables|Default|GetCurrent%20Decal)
        (:Is%20Valid
          (Transformation|SetWorldRotation (Variables|Default|GetCurrent%20Decal) (.rotation _returnvalue) false false))))))