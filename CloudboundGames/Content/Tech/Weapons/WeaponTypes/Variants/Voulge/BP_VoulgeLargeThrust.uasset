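; Large-thrust Voulge weapon variant that implements a three-hit regular combo and a charged attack.
; Each attack passes its damage and hitbox component to a shared box trace placed relative to the player's weapon arrow.
; Hit actors take damage through the player's upgrades component, with debug drawing and printing left on.
; Charged attacks fire only above half charge, scaling damage with charge amount.
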(fn ConstructionScript
  (|CallParentFunction))

(fn RegularComboSwapper
  (|CallParentFunction))

(fn RegularCombo1
  (CallFunction|DamageObjectinRangeV2 (+ (Variables|Default|GetBase%20Damage%20Amount) (Variables|Default|GetCombo%201%20Damage)) (Variables|Default|GetAttack%201%20Combo)))

(fn RegularCombo2
  (CallFunction|DamageObjectinRangeV2 (+ (Variables|Default|GetBase%20Damage%20Amount) (Variables|Default|GetCombo%202%20Damage)) (Variables|Default|GetAttack%202%20Combo)))

(fn RegularCombo3
  (CallFunction|DamageObjectinRangeV2 (+ (Variables|Default|GetBase%20Damage%20Amount) (Variables|Default|GetCombo%203%20Damage)) (Variables|Default|GetAttack%203%20Combo)))

(fn ChargedAttackScaling
  (params (Charged%20Amount :type Float%20%28double-precision%29))
  ;[1 1 1] Charged attack scaling amount from 0.1 - 1.0 for spear
  (if (> Charged%20Amount 0.5)
    (CallFunction|DamageObjectinRangeV2 (* (+ (Variables|Default|GetBase%20Damage%20Amount) (Variables|Default|GetCharged%20Attack%20Damage)) (* Charged%20Amount 2.0)) (Variables|Default|GetAttack%20"4"%20Combo/Charge))
    (CallFunction|ChargeCompleted)))

(fn DamageObjectinRangeV2
  (params (BaseDamage :type Float%20%28single-precision%29) (Attack%20Combo :type Box%20Component%20Object%20Reference))
  (bind _returnvalue (Transformation|GetRelativeTransform Attack%20Combo))
  (bind _player_reference (Variables|Default|GetPlayer%20Reference))
  (bind _player_reference_2 (Variables|Default|GetPlayer%20Reference))
  (bind _weapon_arrow_placeholder (Variables|/Game/Tech/Player/BP_PlayerCharacter.BP_PlayerCharacter_C|GetWeapon%20Arrow%20PlaceHolder _player_reference_2))
  (bind _returnvalue_2 (Transformation|GetWorldTransform _weapon_arrow_placeholder))
  (bind _returnvalue_3 (Math|Transform|TransformLocation _returnvalue_2 (.location _returnvalue)))
  ;[1 1 1] Used for the hurtboxes of the Spear when attacking (Attack Combo 1-3)
  (bind _outhits (Class|KismetSystemLibrary|BoxTraceMultiforObjects _returnvalue_3 _returnvalue_3 (Variables|/Script/Engine.BoxComponent|GetBoxExtent Attack%20Combo) (Math|Rotator|MakeRotator 0.0 0.0 (+ (Variables|Default|GetZ%20Rotation) (.yaw (.rotation _returnvalue)))) (Variables|Default|Getobject%20types) false (Utilities|Array|MakeArray (Variables|Default|GetPlayer%20Reference)) "ForDuration" true "(R=1.000000,G=0.000000,B=0.121054,A=1.000000)" "(R=0.000000,G=1.000000,B=0.000000,A=1.000000)" 0.2))
  (for _array_element _outhits
    (Default|ApplyWeaponDamage (Variables|/Game/Tech/Player/BP_PlayerCharacter.BP_PlayerCharacter_C|GetBPC_Upgrades _player_reference) BaseDamage (Utilities|Struct|MakeF_DamageContext _player_reference (.HitActor (Collision|BreakHitResult _array_element)) _returnvalue_3 "0.000000,0.000000,0.000000"))
    (Development|PrintString (Utilities|String|Append "Damage dealt to" (Utilities|GetDisplayName (.HitActor (Collision|BreakHitResult _array_element)))))
    (CallFunction|AfterAttack))
  (CallFunction|AfterAttack))

(fn ChargeAttackOngoing
  (params (Charged%20Amount :type Float%20%28double-precision%29))
  (CallFunction|ChargeStarted))