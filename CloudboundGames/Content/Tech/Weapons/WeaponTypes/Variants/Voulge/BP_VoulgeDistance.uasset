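; Voulge weapon variant with spear-style attacks: a three-hit combo and a charged area attack.
; Each combo step uses its attack box component, placed relative to the player's weapon arrow, to spawn Niagara effects, box trace and deal damage through the upgrades component.
; Charges above half fire a sphere trace around the arrow, scaling radius and upgrade-modified damage with charge.
; Both traces draw debug shapes and print hit actors.
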(fn ConstructionScript
  (|CallParentFunction))

(fn RegularComboSwapper
  (|CallParentFunction))

(fn RegularCombo1
  (CallFunction|DamageObjectinRangeV2 (+ (Variables|Default|GetBase%20Damage%20Amount) (Variables|Default|GetCombo%201%20Damage)) (Variables|Default|GetAttack%201%20Combo)))

(fn RegularCombo2
  (CallFunction|DamageObjectinRangeV2 (+ (Variables|Default|GetBase%20Damage%20Amount) (Variables|Default|GetCombo%202%20Damage)) (Variables|Default|GetAttack%202%20Combo)))

(fn RegularCombo3
  (CallFunction|DamageObjectinRangeV2 (+ (Variables|Default|GetBase%20Damage%20Amount) (Variables|Default|GetCombo%203%20Damage)) (Variables|Default|GetAttack%203%20Combo)))

(fn DamageObjectinRangeSphere
  (params (Start :type Vector) (End :type Vector) (Radius :type Float%20%28single-precision%29) (BaseDamage :type Float%20%28single-precision%29))
  ;[1 1 1] Charged attack sphere radius around spear.
  (bind _outhits (Collision|MultiSphereTraceForObjects Start End Radius (Variables|Default|Getobject%20types) false (Utilities|Array|MakeArray (Variables|Default|GetPlayer%20Reference)) "ForDuration" true "(R=1.000000,G=0.000000,B=0.034709,A=1.000000)" "(R=0.000000,G=1.000000,B=0.000000,A=1.000000)" 0.2))
  (for _array_element _outhits
    (bind _damageapplied (Default|ModifyDamageApplied (Variables|/Game/Tech/Player/BP_PlayerCharacter.BP_PlayerCharacter_C|GetBPC_Upgrades (Variables|Default|GetPlayer%20Reference)) BaseDamage))
    (Game|Damage|ApplyDamage (.HitActor (Collision|BreakHitResult _array_element)) _damageapplied 0 0 "/Script/Engine.DamageType")
    (Development|PrintString (Utilities|String|Append "Damage dealt to" (Utilities|GetDisplayName (.HitActor (Collision|BreakHitResult _array_element)))))))

(fn ChargedAttackScaling
  (params (Charged%20Amount :type Float%20%28double-precision%29))
  (bind _player_reference (Variables|Default|GetPlayer%20Reference))
  (bind _weapon_arrow_placeholder (Variables|/Game/Tech/Player/BP_PlayerCharacter.BP_PlayerCharacter_C|GetWeapon%20Arrow%20PlaceHolder _player_reference))
  (bind _returnvalue (Transformation|GetWorldLocation _weapon_arrow_placeholder))
  ;[1 1 1] Charged attack scaling amount from 0.1 - 1.0 for spear
  (if (> Charged%20Amount 0.5)
    (CallFunction|DamageObjectinRangeSphere _returnvalue _returnvalue (* (+ (Variables|Default|GetSphere%20trace%20radius) 1.5e+02) Charged%20Amount) (* (+ (Variables|Default|GetBase%20Damage%20Amount) (Variables|Default|GetCharged%20Attack%20Damage)) (* Charged%20Amount 2.0)))
    (CallFunction|ChargeCompleted)))

(fn DamageObjectinRangeV2
  (params (BaseDamage :type Float%20%28single-precision%29) (Attack%20Combo :type Box%20Component%20Object%20Reference))
  (bind _returnvalue (Transformation|GetRelativeTransform Attack%20Combo))
  (bind _player_reference (Variables|Default|GetPlayer%20Reference))
  (bind _player_reference_2 (Variables|Default|GetPlayer%20Reference))
  (bind _z_rotation (Variables|Default|GetZ%20Rotation))
  (bind _returnvalue_2 (+ _z_rotation (.yaw (.rotation _returnvalue))))
  (bind _weapon_arrow_placeholder (Variables|/Game/Tech/Player/BP_PlayerCharacter.BP_PlayerCharacter_C|GetWeapon%20Arrow%20PlaceHolder _player_reference_2))
  (bind _returnvalue_3 (Transformation|GetWorldTransform _weapon_arrow_placeholder))
  (bind _returnvalue_4 (Math|Transform|TransformLocation _returnvalue_3 (.location _returnvalue)))
  ;[1 1 1] Used for the hurtboxes of the Spear when attacking (Attack Combo 1-3)
  (Niagara|SpawnSystematLocation "/Game/Tech/Weapons/Weapon_VFX/HitDust/NS_DustArea.NS_DustArea" _returnvalue_4 (Math|Rotator|MakeRotator 0.0 0.0 _returnvalue_2) "1.000000,0.500000,1.000000")
  (Niagara|SpawnSystematLocation "/Game/Tech/Weapons/Weapon_VFX/SpearEffects/NS_SpearV3FX.NS_SpearV3FX" (- _returnvalue_4 (* (Math|Vector|GetForwardVector _weapon_arrow_placeholder) 2.5e+02)) (Math|Rotator|MakeRotator 0.0 9e+01 _returnvalue_2) "0.500000,0.500000,0.100000")
  (bind _outhits (Class|KismetSystemLibrary|BoxTraceMultiforObjects _returnvalue_4 _returnvalue_4 (Variables|/Script/Engine.BoxComponent|GetBoxExtent Attack%20Combo) (Math|Rotator|MakeRotator 0.0 0.0 _returnvalue_2) (Variables|Default|Getobject%20types) false (Utilities|Array|MakeArray (Variables|Default|GetPlayer%20Reference)) "ForDuration" true "(R=1.000000,G=0.000000,B=0.121054,A=1.000000)" "(R=0.000000,G=1.000000,B=0.000000,A=1.000000)" 0.2))
  (for _array_element _outhits
    (Default|ApplyWeaponDamage (Variables|/Game/Tech/Player/BP_PlayerCharacter.BP_PlayerCharacter_C|GetBPC_Upgrades _player_reference) BaseDamage (Utilities|Struct|MakeF_DamageContext _player_reference (.HitActor (Collision|BreakHitResult _array_element)) _returnvalue_4 "0.000000,0.000000,0.000000"))
    (Development|PrintString (Utilities|String|Append "Damage dealt to" (Utilities|GetDisplayName (.HitActor (Collision|BreakHitResult _array_element)))))
    (CallFunction|AfterAttack))
  (CallFunction|AfterAttack))

(fn ChargeAttackOngoing
  (params (Charged%20Amount :type Float%20%28double-precision%29))
  (CallFunction|ChargeStarted))