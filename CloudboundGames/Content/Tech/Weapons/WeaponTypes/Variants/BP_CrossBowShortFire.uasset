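; Short-range crossbow weapon variant that fires shotgun-like spreads of short-lived projectiles from the player's arrow placeholder.
; All three regular combo steps share FireProjectileBasic, a three-shot fan, through an overridden combo swapper.
; The charged attack fires a tighter five-shot fan, with damage and lifetime scaling by charge.
; While charging, a downward trace places a ground arrow decal once, which follows player rotation until release destroys it.
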(fn ConstructionScript
  (|CallParentFunction))

(fn RegularComboSwapper
  ;[1 1 1] This is the parent function (can be changed if using only one combo)
  (switch int (Variables|Default|GetLocal%20Index%20Attack%20Combo)
    (:0
      (Variables|Default|SetLocal%20Index%20Attack%20Combo 1)
      (CallFunction|RegularCombo1))
    (:1
      (Variables|Default|SetLocal%20Index%20Attack%20Combo 2)
      (CallFunction|RegularCombo2))
    (:2
      (Variables|Default|SetLocal%20Index%20Attack%20Combo 0)
      (CallFunction|RegularCombo3))))

(fn RegularCombo1
  (CallFunction|FireProjectileBasic))

(fn RegularCombo2
  (CallFunction|FireProjectileBasic))

(fn RegularCombo3
  (CallFunction|FireProjectileBasic))

(fn FireProjectileBasic
  (bind _base_damage_amount (Variables|Default|GetBase%20Damage%20Amount))
  (bind _player_reference (Variables|Default|GetPlayer%20Reference))
  (bind _player_reference_2 (Variables|Default|GetPlayer%20Reference))
  (bind _player_reference_3 (Variables|Default|GetPlayer%20Reference))
  (bind _combo_projectile_damge_amount (Variables|Default|GetCombo%20Projectile%20Damge%20Amount))
  (bind _returnvalue (+ _base_damage_amount _combo_projectile_damge_amount))
  (bind _weapon_arrow_placeholder (Variables|/Game/Tech/Player/BP_PlayerCharacter.BP_PlayerCharacter_C|GetWeapon%20Arrow%20PlaceHolder _player_reference))
  (bind _weapon_arrow_placeholder_2 (Variables|/Game/Tech/Player/BP_PlayerCharacter.BP_PlayerCharacter_C|GetWeapon%20Arrow%20PlaceHolder _player_reference_2))
  (bind _returnvalue_2 (Transformation|GetWorldTransform _weapon_arrow_placeholder_2))
  (bind _returnvalue_3 (Transformation|GetWorldTransform _weapon_arrow_placeholder))
  (Game|SpawnActorfromClass "/Game/Tech/Weapons/WeaponTypes/Projectiles/BP_ShortProjectile.BP_ShortProjectile_C" (Transformation|GetWorldTransform (Variables|/Game/Tech/Player/BP_PlayerCharacter.BP_PlayerCharacter_C|GetWeapon%20Arrow%20PlaceHolder (Variables|Default|GetPlayer%20Reference))) "AlwaysSpawn" "MultiplyWithRoot" 0 _returnvalue 0.1 _player_reference_3)
  (Game|SpawnActorfromClass "/Game/Tech/Weapons/WeaponTypes/Projectiles/BP_ShortProjectile.BP_ShortProjectile_C" (Math|Transform|MakeTransform (.location _returnvalue_3) (Math|Rotator|MakeRotator (.roll (.rotation _returnvalue_3)) (.pitch (.rotation _returnvalue_3)) (- (.yaw (.rotation _returnvalue_3)) 35.0)) (.scale _returnvalue_3)) "AlwaysSpawn" "MultiplyWithRoot" _player_reference_3 _returnvalue 0.1 0)
  (Game|SpawnActorfromClass "/Game/Tech/Weapons/WeaponTypes/Projectiles/BP_ShortProjectile.BP_ShortProjectile_C" (Math|Transform|MakeTransform (.location _returnvalue_2) (Math|Rotator|MakeRotator (.roll (.rotation _returnvalue_2)) (.pitch (.rotation _returnvalue_2)) (+ (.yaw (.rotation _returnvalue_2)) 35.0)) (.scale _returnvalue_2)) "AlwaysSpawn" "MultiplyWithRoot" 0 _returnvalue 0.1 0))

(fn ChargedAttackScaling
  (params (Charged%20Amount :type Float%20%28double-precision%29))
  (bind _returnvalue (/ Charged%20Amount 1e+01))
  (bind _returnvalue_2 (* Charged%20Amount 4.0))
  (bind _spread_projectile_damage_amounts (Variables|Default|GetSpread%20Projectile%20damage%20amounts))
  (bind _player_reference (Variables|Default|GetPlayer%20Reference))
  (bind _player_reference_2 (Variables|Default|GetPlayer%20Reference))
  (bind _player_reference_3 (Variables|Default|GetPlayer%20Reference))
  (bind _player_reference_4 (Variables|Default|GetPlayer%20Reference))
  (bind _base_damage_amount (Variables|Default|GetBase%20Damage%20Amount))
  (bind _returnvalue_3 (+ _returnvalue 0.1))
  (bind _returnvalue_4 (+ _base_damage_amount _spread_projectile_damage_amounts))
  (bind _weapon_arrow_placeholder (Variables|/Game/Tech/Player/BP_PlayerCharacter.BP_PlayerCharacter_C|GetWeapon%20Arrow%20PlaceHolder _player_reference_2))
  (bind _weapon_arrow_placeholder_2 (Variables|/Game/Tech/Player/BP_PlayerCharacter.BP_PlayerCharacter_C|GetWeapon%20Arrow%20PlaceHolder _player_reference_3))
  (bind _weapon_arrow_placeholder_3 (Variables|/Game/Tech/Player/BP_PlayerCharacter.BP_PlayerCharacter_C|GetWeapon%20Arrow%20PlaceHolder _player_reference_4))
  (bind _weapon_arrow_placeholder_4 (Variables|/Game/Tech/Player/BP_PlayerCharacter.BP_PlayerCharacter_C|GetWeapon%20Arrow%20PlaceHolder _player_reference))
  (bind _returnvalue_5 (Transformation|GetWorldTransform _weapon_arrow_placeholder_4))
  (bind _returnvalue_6 (Transformation|GetWorldTransform _weapon_arrow_placeholder))
  (bind _returnvalue_7 (Transformation|GetWorldTransform _weapon_arrow_placeholder_2))
  (bind _returnvalue_8 (Transformation|GetWorldTransform _weapon_arrow_placeholder_3))
  (bind _returnvalue_9 (/ _returnvalue_3 2.0))
  (bind _returnvalue_10 (+ _returnvalue_4 _returnvalue_2))
  (Game|SpawnActorfromClass "/Game/Tech/Weapons/WeaponTypes/Projectiles/BP_ShortProjectile.BP_ShortProjectile_C" (Transformation|GetWorldTransform (Variables|/Game/Tech/Player/BP_PlayerCharacter.BP_PlayerCharacter_C|GetWeapon%20Arrow%20PlaceHolder (Variables|Default|GetPlayer%20Reference))) "AlwaysSpawn" "MultiplyWithRoot" 0 _returnvalue_10 _returnvalue_9 (Variables|Default|GetPlayer%20Reference))
  (Game|SpawnActorfromClass "/Game/Tech/Weapons/WeaponTypes/Projectiles/BP_ShortProjectile.BP_ShortProjectile_C" (Math|Transform|MakeTransform (.location _returnvalue_8) (Math|Rotator|MakeRotator (.roll (.rotation _returnvalue_8)) (.pitch (.rotation _returnvalue_8)) (- (.yaw (.rotation _returnvalue_8)) 15.0)) (.scale _returnvalue_8)) "AlwaysSpawn" "MultiplyWithRoot" (Variables|Default|GetPlayer%20Reference) _returnvalue_10 _returnvalue_9 0)
  (Game|SpawnActorfromClass "/Game/Tech/Weapons/WeaponTypes/Projectiles/BP_ShortProjectile.BP_ShortProjectile_C" (Math|Transform|MakeTransform (.location _returnvalue_5) (Math|Rotator|MakeRotator (.roll (.rotation _returnvalue_5)) (.pitch (.rotation _returnvalue_5)) (- (.yaw (.rotation _returnvalue_5)) 25.0)) (.scale _returnvalue_5)) "AlwaysSpawn" "MultiplyWithRoot" (Variables|Default|GetPlayer%20Reference) _returnvalue_10 _returnvalue_9 0)
  (Game|SpawnActorfromClass "/Game/Tech/Weapons/WeaponTypes/Projectiles/BP_ShortProjectile.BP_ShortProjectile_C" (Math|Transform|MakeTransform (.location _returnvalue_6) (Math|Rotator|MakeRotator (.roll (.rotation _returnvalue_6)) (.pitch (.rotation _returnvalue_6)) (+ (.yaw (.rotation _returnvalue_6)) 15.0)) (.scale _returnvalue_6)) "AlwaysSpawn" "MultiplyWithRoot" (Variables|Default|GetPlayer%20Reference) _returnvalue_10 _returnvalue_9 0)
  (Game|SpawnActorfromClass "/Game/Tech/Weapons/WeaponTypes/Projectiles/BP_ShortProjectile.BP_ShortProjectile_C" (Math|Transform|MakeTransform (.location _returnvalue_7) (Math|Rotator|MakeRotator (.roll (.rotation _returnvalue_7)) (.pitch (.rotation _returnvalue_7)) (+ (.yaw (.rotation _returnvalue_7)) 25.0)) (.scale _returnvalue_7)) "AlwaysSpawn" "MultiplyWithRoot" (Variables|Default|GetPlayer%20Reference) _returnvalue_10 _returnvalue_9 0)
  (Variables|Default|SetClose%20Boolean true)
  (Components|DestroyComponent (Variables|Default|GetCurrent%20Decal)))

(fn ChargeAttackOngoing
  (params (Charged%20Amount :type Float%20%28double-precision%29))
  (bind _player_reference (Variables|Default|GetPlayer%20Reference))
  (bind _capsulecomponent (Variables|/Script/Engine.Character|GetCapsuleComponent _player_reference))
  (bind _returnvalue (Transformation|GetWorldTransform _capsulecomponent))
  (Utilities|FlowControl|Sequence
    (:then_0
      (if (> Charged%20Amount 0.5)
        (if (Variables|Default|GetClose%20Boolean)
          (Variables|Default|SetClose%20Boolean false)
          (CallFunction|ChargeStarted)
          (bind _outhit (Collision|LineTraceByChannel (.location _returnvalue) (+ (.location _returnvalue) (* (* (Math|Vector|GetUpVector (.rotation _returnvalue)) -1.0) 1e+05)) "TraceTypeQuery1" false 0 "ForDuration"))
          (bind _returnvalue_2 (Rendering|Decal|SpawnDecalatLocation "/Game/Tech/Weapons/M_DecalArrow.M_DecalArrow" "100.000000,100.000000,100.000000" (.Location (Collision|BreakHitResult _outhit)) (Math|Conversions|RotationFromXVector (.Normal (Collision|BreakHitResult _outhit))) 0.0))
          (Variables|Default|SetCurrent%20Decal _returnvalue_2))))
    (:then_1
      (Utilities|IsValid (Variables|Default|GetCurrent%20Decal)
        (:Is%20Valid
          (Transformation|SetWorldRotation (Variables|Default|GetCurrent%20Decal) (.rotation _returnvalue) false false))))))