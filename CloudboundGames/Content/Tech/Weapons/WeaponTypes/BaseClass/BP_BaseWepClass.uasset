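; Base weapon Blueprint for player melee or other attacks, providing a three-step combo and charged-attack framework with empty combo hooks for child weapons to override.
; Attacks pass a timed spam lock, turn the player to controller facing or mouse cursor (ray-plane intersection), then cycle the combo and briefly slow movement.
; Charging manages slowdown and montage; charge tiers only print debug text.
; Attack, special and charge-start dispatchers are bound for audio.
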(event Custom|Attack%20with%20the%20weapon
  ;[1 1 1] Should be replaced in child bp's by their anim timer
  (if (not (Game|IsGamePaused))
    (if (Variables|Default|GetIs%20Closed?)
      (CallFunction|ClearThatTimer)
      (else
        (Utilities|FlowControl|DoOnce false
          (:Completed
            (Variables|Default|SetIs%20Closed? true)
            (Default|CallOnAttack)
            (Utilities|Time|SetTimerbyEvent (delegate Custom|Spam%20limit%20reset) (Variables|Default|GetAttack%20Spam%20Delay) false true)
            (CallFunction|AlignCorrectlyEnum)))))))

(event Custom|Reset%20Combo%20Action%20to%200
  ;[1 1 1] Should be replaced in child bp's by their anim timer
  (Variables|Default|SetLocal%20Index%20Attack%20Combo 0)
  (Variables|Default|SetIs%20Closed? false)
  (Utilities|FlowControl|DoOnce false) ; enters at Reset
)

(event Custom|Charge%20Started
  ;[1 1 1] Keeping rotation along with disabling movement when attacking
  (Utilities|FlowControl|DoOnce false
    (:Completed
      (Default|CallOnChargeStart)
      (Default|SlowMovement (Variables|/Game/Tech/Player/BP_PlayerCharacter.BP_PlayerCharacter_C|GetBPC_MovementModifiers (Variables|Default|GetPlayer%20Reference)) 1.5e+02)
      (Animation|PlayAnimMontage (Variables|Default|GetPlayer%20Reference) (Variables|Default|GetChargeAnimation) 1.0 "None"))))

(event Custom|Slow%20player%20on%20attack
  ;[1 1 1] Keeping rotation along with disabling movement when attacking
  (Default|SlowMovement (Variables|/Game/Tech/Player/BP_PlayerCharacter.BP_PlayerCharacter_C|GetBPC_MovementModifiers (Variables|Default|GetPlayer%20Reference)) 3e+02)
  (Utilities|Time|SetTimerbyEvent (EventDispatchers|CreateEvent :!event Custom|Clear%20that%20timer) 0.3 false true))

(event Custom|After%20Attack
  ;[1 1 1] Should be replaced in child bp's by their anim timer
  (Utilities|Time|SetTimerbyEvent (EventDispatchers|CreateEvent :!event Custom|Reset%20Combo%20Action%20to%200) (Variables|Default|GetCombo%20Timer%20Amount%20%28Refreshes%29) false true))

(event Custom|Charge%20Completed
  (bind _player_reference (Variables|Default|GetPlayer%20Reference))
  (bind _chargeanimation (Variables|Default|GetChargeAnimation))
  (bind _player_reference_2 (Variables|Default|GetPlayer%20Reference))
  (bind _bpc_movementmodifiers (Variables|/Game/Tech/Player/BP_PlayerCharacter.BP_PlayerCharacter_C|GetBPC_MovementModifiers _player_reference))
  ;[1 1 1] Keeping rotation along with disabling movement when attacking
  (Default|ResetPlayerMovement _bpc_movementmodifiers)
  (Animation|StopAnimMontage _player_reference_2 _chargeanimation)
  (Utilities|FlowControl|DoOnce false) ; enters at Reset
)

(event Custom|Clear%20that%20timer
  (bind _player_reference (Variables|Default|GetPlayer%20Reference))
  (bind _chargeanimation (Variables|Default|GetChargeAnimation))
  (bind _player_reference_2 (Variables|Default|GetPlayer%20Reference))
  (bind _bpc_movementmodifiers (Variables|/Game/Tech/Player/BP_PlayerCharacter.BP_PlayerCharacter_C|GetBPC_MovementModifiers _player_reference))
  ;[1 1 1] Keeping rotation along with disabling movement when attacking
  (Default|ResetPlayerMovement _bpc_movementmodifiers)
  (Animation|StopAnimMontage _player_reference_2 _chargeanimation)
  (Utilities|FlowControl|DoOnce false) ; enters at Reset
)

(event Custom|Spam%20limit%20reset
  ;[1 1 1] Should be replaced in child bp's by their anim timer
  (Variables|Default|SetIs%20Closed? false)
  (Utilities|FlowControl|DoOnce false) ; enters at Reset
)

(event EventBeginPlay
  ;[1 1 1] Should be replaced in child bp's by their anim timer
  (CallFunction|SetupAudioEvents))

(fn ConstructionScript)

(fn ChargedAttackWeaponFunctionEnum
  (params (Charged%20Amount :type Float%20%28double-precision%29))
  (Default|CallOnSpecialAttack)
  (switch Utilities|FlowControl|Switch|SwitchonE_ControllerOrMouse (Variables|Default|GetEnumControllerOrMouse)
    (:NewEnumerator0
      (CallFunction|RotatePlayeratCameraCONTROLLER))
    (:NewEnumerator1
      (CallFunction|RotatePlayeratCameraMOUSE)))
  (CallFunction|ChargedAttackScaling Charged%20Amount))

(fn RegularComboSwapper
  ;[1 1 1] This is just due to not having notifiers from anims currently
  (Default|CallOnAttack)
  (switch int (Variables|Default|GetLocal%20Index%20Attack%20Combo)
    (:0
      (Variables|Default|SetLocal%20Index%20Attack%20Combo 1)
      (CallFunction|RegularCombo1)
      (CallFunction|SlowPlayeronAttack))
    (:1
      (Variables|Default|SetLocal%20Index%20Attack%20Combo 2)
      (CallFunction|RegularCombo2)
      (CallFunction|SlowPlayeronAttack))
    (:2
      (Variables|Default|SetLocal%20Index%20Attack%20Combo 0)
      (CallFunction|RegularCombo3)
      (CallFunction|SlowPlayeronAttack))))

(fn RegularCombo1
  ;[1 1 1] Change in child bp
)

(fn RegularCombo2
  ;[1 1 1] Change in child bp
)

(fn RegularCombo3
  ;[1 1 1] Change in child bp
)

(fn ChargedAttackScaling
  (params (Charged%20Amount :type Float%20%28double-precision%29))
  (if (>= Charged%20Amount 1.5)
    (Development|PrintString "Full Charge")
    (elif (>= Charged%20Amount 1.0)
      (Development|PrintString "Medium Charge")
      (elif (>= Charged%20Amount 0.5)
        (Development|PrintString "Short Charge")))))

(fn AlignCorrectlyEnum
  (Utilities|FlowControl|Sequence
    (:then_0
      (switch Utilities|FlowControl|Switch|SwitchonE_ControllerOrMouse (Variables|Default|GetEnumControllerOrMouse)
        (:NewEnumerator0
          (CallFunction|RotatePlayeratCameraCONTROLLER))
        (:NewEnumerator1
          (CallFunction|RotatePlayeratCameraMOUSE))))
    (:then_1
      (CallFunction|RegularComboSwapper))))

(fn CreateWidgetUponDealingDamage
  (params (Damaged%20Actor :type Actor%20Object%20Reference))
  (bind _returnvalue (UserInterface|CreateWidget "/Game/Tech/UI/GameplayUI/WBP_DamageNumbers.WBP_DamageNumbers_C"))
  (UserInterface|Viewport|AddtoViewport _returnvalue 0))

(fn ChargeAttackOngoing
  (params (Charged%20Amount :type Float%20%28double-precision%29)))

(fn SetupAudioEvents
  (EventDispatchers|BindEventtoOnAttack (EventDispatchers|CreateEvent (Variables|Default|GetBPC_WeaponSFX) :!event OnAttack))
  (EventDispatchers|BindEventtoOnSpecialAttack (EventDispatchers|CreateEvent (Variables|Default|GetBPC_WeaponSFX) :!event OnSpecialAttack))
  (EventDispatchers|BindEventtoOnChargeStart (EventDispatchers|CreateEvent (Variables|Default|GetBPC_WeaponSFX) :!event OnChargeStart)))

(fn RotatePlayerVisuallyMOUSE
  (bind _returnvalue (Game|GetPlayerController 0))
  (bind _player_reference (Variables|Default|GetPlayer%20Reference))
  (bind (_worldlocation _worlddirection) (Game|Player|ConvertMouseLocationToWorldSpace _returnvalue))
  (bind _returnvalue_2 (Transformation|GetActorLocation _player_reference))
  (Transformation|SetActorRotation _player_reference (Math|Rotator|MakeRotator 0.0 0.0 (.yaw (Math|Rotator|FindLookatRotation _returnvalue_2 (.Intersection (Class|KismetMathLibrary|LinePlaneIntersectionOriginNormal _worldlocation (+ (* _worlddirection 1e+05) _worldlocation) _returnvalue_2 "0.000000,0.000000,1.000000")))))))

(fn RotatePlayeratCameraMOUSE
  (bind _returnvalue (Game|GetPlayerController 0))
  (bind _player_reference (Variables|Default|GetPlayer%20Reference))
  (bind (_worldlocation _worlddirection) (Game|Player|ConvertMouseLocationToWorldSpace _returnvalue))
  (bind _returnvalue_2 (Transformation|GetActorLocation _player_reference))
  (bind _returnvalue_3 (* _worlddirection 1e+05))
  (bind _returnvalue_4 (+ _returnvalue_3 _worldlocation))
  (bind _intersection (Class|KismetMathLibrary|LinePlaneIntersectionOriginNormal _worldlocation _returnvalue_4 _returnvalue_2 "0.000000,0.000000,1.000000"))
  (bind _returnvalue_5 (Math|Rotator|FindLookatRotation _returnvalue_2 _intersection))
  (Transformation|SetActorRotation _player_reference (Math|Rotator|MakeRotator 0.0 0.0 (.yaw _returnvalue_5)))
  (Variables|Default|SetZ%20Rotation (.yaw _returnvalue_5))
  (return))

(fn RotatePlayeratCameraCONTROLLER
  (bind _player_reference (Variables|Default|GetPlayer%20Reference))
  (bind _returnvalue (Transformation|GetActorRotation _player_reference))
  (Transformation|SetActorRotation (Math|Rotator|MakeRotator 0.0 0.0 (.yaw _returnvalue)))
  (Variables|Default|SetZ%20Rotation (.yaw _returnvalue))
  (return))

(fn GetCurrentReference
  (return 0))

(fn VariantUpgrade
  (params (Weapon%20Variant%20Bp :type BP%20Base%20Wep%20Class%20Class%20Reference))
  (return))