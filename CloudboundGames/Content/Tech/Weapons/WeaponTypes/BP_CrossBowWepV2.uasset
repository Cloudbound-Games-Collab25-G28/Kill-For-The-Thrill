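; Crossbow weapon, a child weapon Blueprint that fires projectiles for basic combo and charged attacks.
; The three-step combo cycles through identical shots, each playing a montage, spawning a short-lived piercing projectile and slowing the player.
; Holding a charge spawns an arrow decal via a downward trace, then keeps it aligned to the player and stretches it with charge.
; Release fires a projectile whose damage and lifetime scale with charge, then removes the decal.
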(fn ConstructionScript
  (|CallParentFunction))

(fn RegularComboSwapper
  ;[1 1 1] This is the parent function (can be changed if using only one combo)
  (switch int (Variables|Default|GetLocal%20Index%20Attack%20Combo)
    (:0
      (Variables|Default|SetLocal%20Index%20Attack%20Combo 1)
      (CallFunction|RegularCombo1))
    (:1
      (Variables|Default|SetLocal%20Index%20Attack%20Combo 2)
      (CallFunction|RegularCombo2))
    (:2
      (Variables|Default|SetLocal%20Index%20Attack%20Combo 0)
      (CallFunction|RegularCombo3))))

(fn RegularCombo1
  (CallFunction|FireProjectileBasic))

(fn RegularCombo2
  (CallFunction|FireProjectileBasic))

(fn RegularCombo3
  (CallFunction|FireProjectileBasic))

(fn FireProjectileBasic
  (bind _player_reference (Variables|Default|GetPlayer%20Reference))
  (Animation|PlayAnimMontage _player_reference "/Game/Art/PlayableCharacter/Duck-Final/Animations/Weapons/Crossbow_Animations/AM_Crossbow_Hit_1_Montage.AM_Crossbow_Hit_1_Montage" 1.0 "None")
  (Game|SpawnActorfromClass "/Game/Tech/Weapons/WeaponTypes/Projectiles/BP_PierceProjectile.BP_PierceProjectile_C" (Transformation|GetWorldTransform (Variables|/Game/Tech/Player/BP_PlayerCharacter.BP_PlayerCharacter_C|GetWeapon%20Arrow%20PlaceHolder _player_reference)) "AlwaysSpawn" "MultiplyWithRoot" 0 (+ (Variables|Default|GetBase%20Damage%20Amount) (Variables|Default|GetCombo%20Projectile%20Damge%20Amount)) 0.3 (Variables|Default|GetPlayer%20Reference))
  (CallFunction|SlowPlayeronAttack))

(fn ChargedAttackScaling
  (params (Charged%20Amount :type Float%20%28double-precision%29))
  (bind _player_reference (Variables|Default|GetPlayer%20Reference))
  (Animation|PlayAnimMontage _player_reference "/Game/Art/PlayableCharacter/Duck-Final/Animations/Weapons/Crossbow_Animations/AM_Crossbow_Hit_1_Montage.AM_Crossbow_Hit_1_Montage" 1.0 "None")
  (Game|SpawnActorfromClass "/Game/Tech/Weapons/WeaponTypes/Projectiles/BP_AoeProjectile.BP_AoeProjectile_C" (Transformation|GetWorldTransform (Variables|/Game/Tech/Player/BP_PlayerCharacter.BP_PlayerCharacter_C|GetWeapon%20Arrow%20PlaceHolder _player_reference)) "AlwaysSpawn" "MultiplyWithRoot" 0 (+ (+ (Variables|Default|GetBase%20Damage%20Amount) (Variables|Default|GetExploding%20Projectile%20Damage%20Amount)) (* (* Charged%20Amount 1e+01) 2.0)) (+ (/ Charged%20Amount 1e+01) 0.3) (Variables|Default|GetPlayer%20Reference))
  (Variables|Default|SetClose%20Boolean true)
  (Components|DestroyComponent (Variables|Default|GetCurrent%20Decal))
  (CallFunction|ChargeCompleted))

(fn ChargeAttackOngoing
  (params (Charged%20Amount :type Float%20%28double-precision%29))
  (bind _player_reference (Variables|Default|GetPlayer%20Reference))
  (bind _player_reference_2 (Variables|Default|GetPlayer%20Reference))
  (bind _capsulecomponent (Variables|/Script/Engine.Character|GetCapsuleComponent _player_reference))
  (bind _returnvalue (Transformation|GetWorldTransform _capsulecomponent))
  (Utilities|FlowControl|Sequence
    (:then_0
      (if (> Charged%20Amount 0.5)
        (if (Variables|Default|GetClose%20Boolean)
          (Variables|Default|SetClose%20Boolean false)
          (CallFunction|ChargeStarted)
          (bind _outhit (Collision|LineTraceByChannel (.location _returnvalue) (+ (.location _returnvalue) (* (* (Math|Vector|GetUpVector (.rotation _returnvalue)) -1.0) 1e+03)) "TraceTypeQuery1" false 0 "ForDuration"))
          (bind _returnvalue_2 (Rendering|Decal|SpawnDecalatLocation "/Game/Tech/Weapons/M_DecalArrow.M_DecalArrow" "128.000000,128.000000,256.000000" (.Location (Collision|BreakHitResult _outhit)) "-90.000000,0.000000,0.000000" 0.0))
          (Variables|Default|SetCurrent%20Decal _returnvalue_2))))
    (:then_1
      (Utilities|IsValid (Variables|Default|GetCurrent%20Decal)
        (:Is%20Valid
          (Transformation|SetRelativeScale3D (Variables|Default|GetCurrent%20Decal) (Math|Vector|MakeVector 1.0 1.0 (/ (Math|Float|Lerp 0.5 2.0 Charged%20Amount) 2.0)))
          (Transformation|SetWorldRotation (Variables|Default|GetCurrent%20Decal) (Math|Rotator|MakeRotator 0.0 -9e+01 (.yaw (.rotation (Transformation|GetWorldTransform _capsulecomponent)))) false false)
          (Transformation|SetWorldLocation (Variables|Default|GetCurrent%20Decal) (Math|Transform|TransformLocation (Transformation|GetWorldTransform (Variables|/Game/Tech/Player/BP_PlayerCharacter.BP_PlayerCharacter_C|GetDecal%20Arrow%20Placeholder _player_reference_2)) (.location (Transformation|GetRelativeTransform (Variables|/Game/Tech/Player/BP_PlayerCharacter.BP_PlayerCharacter_C|GetWeapon%20Arrow%20PlaceHolder _player_reference_2)))) false false))))))