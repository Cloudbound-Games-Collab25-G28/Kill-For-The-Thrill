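; Player combat component that equips a sword, voulge or crossbow chosen through UI and routes attack input to it.
; Owner input stays disabled until SelectWeapon spawns the weapon, attaches it to the hand socket and stores its reference.
; Holding attack rotates the player and feeds clamped charge time to the weapon; ending it triggers a normal or charged attack by hold duration.
; The weapon upgrade replacement is unwired.
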(event Input|EnhancedActionEvents|EnhancedInputActionIA_WeaponAttack_Held
  (params (ActionValue :type Boolean) (ElapsedSeconds :type Float%20%28double-precision%29) (TriggeredSeconds :type Float%20%28double-precision%29) (InputAction :type Input%20Action%20Object%20Reference :default "/Game/Tech/Input/Actions/IA_WeaponAttack_Held.IA_WeaponAttack_Held"))
  (bind _returnvalue (Math|Float|Clamp(Float) ElapsedSeconds 0.1 1.5))
  (:Started
    (if (>= _returnvalue 0.5) :!label _label
      (CallFunction|ChargedAttackFunction (Math|Float|Clamp(Float) _returnvalue 0.5 1.5))
      (else
        (Default|AttackwiththeWeapon (Variables|Default|GetCurrent%20Weapon%20Reference)))))
  (:Ongoing
    (Default|RotatePlayerVisually (Variables|Default|GetCurrent%20Weapon%20Reference))
    (if (or (> _returnvalue 0.5) (not (== _returnvalue 1.5)))
      (Utilities|FlowControl|Sequence
        (:then_0
          (goto _label_2 Open))
        (:then_1
          (Utilities|FlowControl|Gate true :!label _label_2
            (:Exit
              (Default|ChargeAttackOngoing (Variables|Default|GetCurrent%20Weapon%20Reference) _returnvalue)
              (Development|PrintString (Utilities|String|ToString(Float) _returnvalue))))))
      (else
        (goto _label_2 Close))))
  (:Canceled
    (goto _label))
  (:Completed
    (goto _label)))

(event EventBeginPlay
  (Input|DisableInput (Components|GetOwner) (Game|GetPlayerController 0)))

(fn ChargedAttackFunction
  (params (Input%20Float :type Float%20%28double-precision%29))
  ;[1 1 1] Alternative action for using the BP parent function version
  (if (>= Input%20Float 0.25)
    (Default|ChargedAttackWeaponFunction (Variables|Default|GetCurrent%20Weapon%20Reference) (Math|Float|Clamp(Float) Input%20Float 0.5 2.0))))

(fn SendReferenceForce
  (return 0))

(fn SelectWeapon
  (params (Weapon%20Enum :type EWeaponType%20Enum :default "SWORD"))
  ;[1 1 1] Setting Weapon Through UI
  (bind _asbp_player_character (Utilities|Casting|CastToBP_PlayerCharacter (Components|GetOwner)))
  (switch Utilities|FlowControl|Switch|SwitchonEWeaponType Weapon%20Enum
    (:SWORD
      (Variables|Default|SetWeapon%20Class%20To%20Use "/Game/Tech/Weapons/WeaponTypes/BP_SwordWepV2.BP_SwordWepV2_C"))
    (:VOULGE
      (Variables|Default|SetWeapon%20Class%20To%20Use "/Game/Tech/Weapons/WeaponTypes/BP_SpearWepV2.BP_SpearWepV2_C"))
    (:CROSSBOW
      (Variables|Default|SetWeapon%20Class%20To%20Use "/Game/Tech/Weapons/WeaponTypes/BP_CrossBowWepV2.BP_CrossBowWepV2_C")))
  (bind _returnvalue (Game|SpawnActorfromClass (Variables|Default|GetWeapon%20Class%20To%20Use) (Math|Transform|MakeTransform "1000.000000,1810.000000,100.000000" "0, 0, 0" "1.000000,1.000000,1.000000") "AlwaysSpawn" "MultiplyWithRoot" _asbp_player_character 0))
  (Transformation|AttachComponentToComponent _returnvalue (Actor|GetComponentbyClass (Components|GetOwner) "/Script/Engine.SkeletalMeshComponent") "hand_rSocketV2" "SnapToTarget" "KeepWorld" "SnapToTarget" false)
  (Variables|Default|SetCurrent%20Weapon%20Reference _returnvalue)
  (Variables|/Game/Tech/Weapons/WeaponTypes/BaseClass/BP_BaseWepClass.BP_BaseWepClass_C|SetPlayer%20Reference _returnvalue _asbp_player_character)
  (Input|EnableInput (Components|GetOwner) (Game|GetPlayerController 0)))

(fn ReplaceWeaponwithUpgrade
  (params (Weapon%20Class%20Upgrade :type BP%20Base%20Wep%20Class%20Class%20Reference)))

(fn GetCurrentReference
  (return 0))