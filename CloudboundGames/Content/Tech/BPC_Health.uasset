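; BPC_Health is a component that tracks health for its owning actor and reduces it when that actor takes damage.
; It starts at MaxHealth, binds to the owner's TakeAnyDamage event and clamps health through setters that broadcast change events.
; Damage that leaves health at zero fires OnKilled, with no guard against repeats, and optionally destroys the owner.
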(event Custom|OnTakeAnyDamage_Event
  (params (DamagedActor :type Actor%20Object%20Reference) (Damage :type Float%20%28single-precision%29) (DamageType :type Damage%20Type%20Object%20Reference) (InstigatedBy :type Controller%20Object%20Reference) (DamageCauser :type Actor%20Object%20Reference))
  (bind _health (Variables|Default|GetHealth))
  (CallFunction|SetHealth (- _health Damage))
  (if (<= _health 0.0)
    (Default|CallOnKilled self)
    (if (Variables|Default|GetDestroyOnDeath)
      (Actor|DestroyActor (Components|GetOwner)))))

(event EventBeginPlay
  (Variables|Default|SetHealth (Variables|Default|GetMaxHealth))
  (EventDispatchers|AssignOnTakeAnyDamage (Components|GetOwner) (delegate Custom|OnTakeAnyDamage_Event)))

(fn SetHealth
  (params (NewHealth :type Float%20%28double-precision%29))
  (Variables|Default|SetHealth (Math|Float|Clamp(Float) NewHealth 0.0 (Variables|Default|GetMaxHealth)))
  (Default|CallOnHealthChanged self))

(fn SetMaxHealth
  (params (NewMaxHealth :type Float%20%28double-precision%29))
  (bind _output_get (Variables|Default|SetMaxHealth NewMaxHealth))
  (Variables|Default|SetHealth (Math|Float|Clamp(Float) (Variables|Default|GetHealth) 0.0 _output_get))
  (Default|CallOnMaxHealthChanged (Variables|Default|GetMaxHealth)))