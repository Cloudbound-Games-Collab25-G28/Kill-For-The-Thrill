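; Temporary ranged enemy Blueprint that fires a crossbow-style hitscan attack at its AI controller's attack target.
; Attack plays a sound and montage; a notify triggers a debug-drawn Camera-channel trace toward the target, damaging whatever it hits.
; Montage completion or interruption signals attack finish, and "hit target" prints only when the trace reports no hit.
; Overrides supply ideal attack/defend ranges, speed-state walk speeds and an empty patrol route.
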(event EventBeginPlay)

(event Collision|EventActorBeginOverlap
  (params (OtherActor :type Actor%20Object%20Reference)))

(event EventTick
  (params (DeltaSeconds :type Float%20%28single-precision%29)))

(event EventAttack
  (Audio|PlaySoundatLocation "/Game/Audio/combat/crossbow/crossbow_fire_1.crossbow_fire_1" (Transformation|GetActorLocation) "0, 0, 0" 1.0 1.0 0.0 0 0 0 0)
  (bind _notifyname (Animation|Montage|PlayMontage (Variables|Character|GetMesh) (Variables|Default|GetAttackAnimation))
    (:OnCompleted
      (Default|CallOnAttackFinish :!label _label))
    (:OnInterrupted
      (goto _label))
    (:OnNotifyBegin
      (switch name _notifyname
        (:Fire
          (bind _asaic_enemy_base (Utilities|Casting|CastToAIC_Enemy_Base (AI|GetAIController self)))
          (bind _attack_target (Variables|/Game/Tech/AI/AIC_Enemy_Base.AIC_Enemy_Base_C|GetAttack%20Target _asaic_enemy_base)
            (:then
              (bind (_outhit _returnvalue) (Collision|LineTraceByChannel (Transformation|GetWorldLocation (Variables|Default|GetAttackPosition)) (Transformation|GetActorLocation _attack_target) "TraceTypeQuery2" false 0 "ForDuration"))
              (Game|Damage|ApplyDamage (.HitActor (Collision|BreakHitResult _outhit)) (Variables|Default|GetDamage) 0 0)
              (if (not _returnvalue)
                (Development|PrintString "hit target")))
            (:else)))))))

(fn ConstructionScript
  (|CallParentFunction))

(fn GetPatrolRoute
  (return 0))

(fn GetIdealRange
  (return 4e+02 4e+02))

(fn SetMovementSpeed
  (params (Speed :type E_MovementSpeed%20Enum :default "NewEnumerator0"))
  (bind _output_get (Variables|/Script/Engine.CharacterMovementComponent|SetMaxWalkSpeed (Variables|Character|GetCharacterMovement) (Utilities|Select :Index Speed :NewEnumerator0 0.0 :NewEnumerator1 2e+02 :NewEnumerator2 3e+02 :NewEnumerator3 5e+02)))
  (return _output_get))