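; BP_Siren is an AI enemy character with a ranged projectile attack.
; Attack plays a montage, spawns a projectile from AttackPosition on a montage notify, and calls AttackEnd on completion or interruption.
; Shots lead player 0 using distance, bullet speed and velocity, regardless of the AttackTarget passed to the projectile.
; Overrides supply equal attack and defend ranges, map movement states to walk speeds, and leave the patrol route empty.
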(event EventBeginPlay)

(event Collision|EventActorBeginOverlap
  (params (OtherActor :type Actor%20Object%20Reference)))

(event EventAttack
  (params (AttackTarget :type Actor%20Object%20Reference))
  (bind _returnvalue (Game|GetPlayerCharacter 0))
  (bind _attackposition (Variables|Default|GetAttackPosition))
  (bind _returnvalue_2 (Transformation|GetWorldLocation _attackposition))
  ;[1 1 1] AOE Attack
  (|CallParentFunction AttackTarget)
  (bind _notifyname (Animation|Montage|PlayMontage (Variables|Character|GetMesh) (Variables|Default|GetAttackAnimation))
    (:OnCompleted
      (CallFunction|AttackEnd AttackTarget :!label _label))
    (:OnInterrupted
      (goto _label))
    (:OnNotifyBegin
      (switch name _notifyname
        (:Fire
          (Game|SpawnActorfromClass "/Game/Tech/AI/RangedAttacks/ProjectileAttacks/BP_ProjectileBase_Child.BP_ProjectileBase_Child_C" (Math|Transform|MakeTransform _returnvalue_2 (Math|Rotator|FindLookatRotation _returnvalue_2 (+ (+ (Transformation|GetWorldLocation (Variables|/Script/Engine.Character|GetCapsuleComponent _returnvalue)) "0.000000,0.000000,80.000000") (* (/ (Transformation|GetDistanceTo _returnvalue) (Variables|Default|GetBulletSpeed)) (Transformation|GetVelocity _returnvalue)))) "1.000000,1.000000,1.000000") "Undefined" "MultiplyWithRoot" (Components|GetOwner) AttackTarget (Variables|Default|GetBulletSpeed) (Variables|Default|GetDamage) 0))))))

(fn ConstructionScript
  (|CallParentFunction))

(fn GetPatrolRoute
  (return 0))

(fn GetIdealRange
  (return 4e+02 4e+02))

(fn SetMovementSpeed
  (params (Speed :type E_MovementSpeed%20Enum :default "NewEnumerator0"))
  (bind _output_get (Variables|/Script/Engine.CharacterMovementComponent|SetMaxWalkSpeed (Variables|Character|GetCharacterMovement) (Utilities|Select :Index Speed :NewEnumerator0 0.0 :NewEnumerator1 2e+02 :NewEnumerator2 3e+02 :NewEnumerator3 5e+02)))
  (return _output_get))