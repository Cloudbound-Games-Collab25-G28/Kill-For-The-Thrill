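; BPC_AttackToken is an AI component that holds a pool of attack tokens, named for limiting attacks.
; ReserveAttackToken calls ReserveTokens, which deducts the requested amount and reports success only when enough tokens remain.
; The ReturnAttackToken event calls ReturnTokens to add the amount back to the count, with no upper cap.
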(event EventBeginPlay)

(event EventTick
  (params (DeltaSeconds :type Float%20%28single-precision%29)))

(event EventReturnAttackToken
  (params (Amount :type Integer))
  (CallFunction|ReturnTokens Amount))

(fn ReserveTokens
  (params (Amount :type Integer))
  (if (>= (Variables|Default|GetAttackTokenCount) Amount)
    (Variables|Default|SetAttackTokenCount (- (Variables|Default|GetAttackTokenCount) Amount))
    (return true)
    (else
      (return false))))

(fn ReturnTokens
  (params (Amount :type Integer))
  (Variables|Default|SetAttackTokenCount (+ Amount (Variables|Default|GetAttackTokenCount))))

(fn ReserveAttackToken
  (params (Amount :type Integer))
  (bind _success (CallFunction|ReserveTokens Amount))
  (return _success))