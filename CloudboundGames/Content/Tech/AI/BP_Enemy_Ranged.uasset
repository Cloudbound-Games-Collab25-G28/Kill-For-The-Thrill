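; Ranged enemy character Blueprint that extends a parent enemy with a hitscan attack and its own movement speeds and combat ranges.
; Attack plays a montage, uses a notify to line trace from AttackPosition to the target and damage the hit actor, then calls AttackEnd on completion or interruption.
; The debug "hit target" message prints only when the trace finds nothing.
; Overrides supply equal attack and defend radii and map speed states to walk speed, while GetPatrolRoute returns nothing.
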(event EventBeginPlay)

(event Collision|EventActorBeginOverlap
  (params (OtherActor :type Actor%20Object%20Reference)))

(event EventTick
  (params (DeltaSeconds :type Float%20%28single-precision%29)))

(event EventAttack
  (params (AttackTarget :type Actor%20Object%20Reference))
  (|CallParentFunction AttackTarget)
  (bind _notifyname (Animation|Montage|PlayMontage (Variables|Character|GetMesh) (Variables|Default|GetAttackAnimation))
    (:OnCompleted
      (CallFunction|AttackEnd AttackTarget :!label _label))
    (:OnInterrupted
      (goto _label))
    (:OnNotifyBegin
      (switch name _notifyname
        (:Fire
          (bind (_outhit _returnvalue) (Collision|LineTraceByChannel (Transformation|GetWorldLocation (Variables|Default|GetAttackPosition)) (Transformation|GetActorLocation AttackTarget) "TraceTypeQuery2" false 0 "ForDuration"))
          (Game|Damage|ApplyDamage (.HitActor (Collision|BreakHitResult _outhit)) (Variables|Default|GetDamage) 0 0)
          (if (not _returnvalue)
            (Development|PrintString "hit target")))))))

(fn ConstructionScript
  (|CallParentFunction))

(fn GetPatrolRoute
  (return 0))

(fn GetIdealRange
  (return 4e+02 4e+02))

(fn SetMovementSpeed
  (params (Speed :type E_MovementSpeed%20Enum :default "NewEnumerator0"))
  (bind _output_get (Variables|/Script/Engine.CharacterMovementComponent|SetMaxWalkSpeed (Variables|Character|GetCharacterMovement) (Utilities|Select :Index Speed :NewEnumerator0 0.0 :NewEnumerator1 2e+02 :NewEnumerator2 3e+02 :NewEnumerator3 5e+02)))
  (return _output_get))