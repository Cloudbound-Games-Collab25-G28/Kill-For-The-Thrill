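; Miniboss enemy character with an intro montage, a basic melee attack and a targeted area attack.
; Basic attack plays its montage while a timed delay triggers a debug-drawn sphere overlap that damages nearby pawns.
; AOE attack spawns AOE_BossStrike at the target's location on montage notifies, and both attacks call AttackEnd when their montage ends.
; Helper functions supply combat ranges, patrol route and walk speed per movement state.
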(event Custom|AOEAttack
  (params (AttackTarget :type Actor%20Object%20Reference))
  (bind _notifyname (Animation|Montage|PlayMontage (Variables|Character|GetMesh) (Variables|Default|GetAOEAttackAnimation))
    (:OnCompleted
      (CallFunction|AttackEnd AttackTarget :!label _label))
    (:OnInterrupted
      (goto _label))
    (:OnNotifyBegin
      (switch name _notifyname
        (:Strike
          (Game|SpawnActorfromClass "/Game/Tech/AI/AOE_Attack/AOE_BossStrike.AOE_BossStrike_C" (Math|Transform|MakeTransform (Transformation|GetActorLocation AttackTarget) "0, 0, 0" "1.000000,1.000000,1.000000") "Undefined" "MultiplyWithRoot" 0 2.0 "/Game/Tech/AI/AOE_Attack/M_Attack.M_Attack" (Game|GetPlayerCharacter 0) true true true 0))))))

(event Custom|DealDamage
  (bind _attacksphere (Variables|Default|GetAttackSphere))
  (bind _returnvalue (Transformation|GetWorldLocation _attacksphere))
  ;[1 1 1] Deal damage
  (Utilities|FlowControl|Delay 1.5)
  (bind _outactors (Collision|SphereOverlapActors _returnvalue (Variables|Default|GetAttackRange) (Utilities|Array|MakeArray "ObjectTypeQuery3") "/Script/Engine.Actor" (Utilities|Array|MakeArray self)))
  (Rendering|Debug|DrawDebugSphere _returnvalue (Variables|Default|GetAttackRange) 12 "(R=1.000000,G=0.073826,B=0.000000,A=1.000000)" 2.0)
  (for _array_element _outactors
    (Game|Damage|ApplyDamage _array_element (Variables|AI|GetAttackDamage) (Pawn|GetController) self "/Script/Engine.DamageType")))

(event Custom|StartSequence
  (Animation|Montage|PlayMontage (Variables|Character|GetMesh) (Variables|Default|GetStartAniamtion)
    (:OnCompleted
      _)
    (:OnInterrupted
      _))
  (Default|CallOnAttackFinish))

(event Custom|OnAOEOverlapActor_Event
  (params (Actor :type Actor%20Object%20Reference)))

(event EventBeginPlay
  (bind _output_get (Variables|Default|SetStartLocation (Transformation|GetWorldLocation (Variables|Character|GetMesh))))
  (Development|PrintString (Utilities|String|ToString(Vector) _output_get)))

(event Collision|EventActorBeginOverlap
  (params (OtherActor :type Actor%20Object%20Reference)))

(event EventTick
  (params (DeltaSeconds :type Float%20%28single-precision%29)))

(event EventAttack
  (params (AttackTarget :type Actor%20Object%20Reference))
  ;[1 1 1] Play attack anim
  (CallFunction|DealDamage)
  (Animation|Montage|PlayMontage (Variables|Character|GetMesh) (Variables|AI|GetBasicAttackAnimation)
    (:OnCompleted
      _)
    (:OnInterrupted
      _))
  (CallFunction|AttackEnd AttackTarget))

(fn ConstructionScript
  (|CallParentFunction))

(fn GetIdealRange
  (return 1.5e+02 3.5e+02))

(fn SetMovementSpeed
  (params (Speed :type E_MovementSpeed%20Enum :default "NewEnumerator0"))
  (bind _output_get (Variables|/Script/Engine.CharacterMovementComponent|SetMaxWalkSpeed (Variables|Character|GetCharacterMovement) (Utilities|Select :Index Speed :NewEnumerator0 0.0 :NewEnumerator1 1e+02 :NewEnumerator2 3e+02 :NewEnumerator3 5e+02)))
  (return _output_get))

(fn GetPatrolRoute
  (return (Variables|Default|GetPatrolRoute)))