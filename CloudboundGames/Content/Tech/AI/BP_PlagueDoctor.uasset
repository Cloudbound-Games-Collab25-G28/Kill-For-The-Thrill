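; Plague Doctor AI character that attacks with delayed area-of-effect blasts.
; Attack runs an EQS query for all matching locations, then plays the attack montage, whose notify spawns a decal-marked blast at each location, targeting player 0.
; Montage completion or interruption ends the attack.
; Also supplies attack and defend ranges and maps movement states to walk speeds, while its patrol route getter returns nothing.
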(event Custom|QueryFinished
  (params (QueryInstance :type Env%20Query%20Instance%20Blueprint%20Wrapper%20Object%20Reference) (QueryStatus :type EEnvQueryStatus%20Enum :default "Processing"))
  ;[1 1 1] Attack
  (bind _resultlocations (AI|EQS|GetQueryResultsasLocations QueryInstance))
  (bind _notifyname (Animation|Montage|PlayMontage (Variables|Character|GetMesh) (Variables|Default|GetAttackAnimation))
    (:OnCompleted
      (CallFunction|AttackEnd (stale EventAttack AttackTarget) :!label _label))
    (:OnInterrupted
      (goto _label))
    (:OnNotifyBegin
      (switch name _notifyname
        (:Fire
          (for _array_element _resultlocations
            (Game|SpawnActorfromClass "/Game/Tech/AI/RangedAttacks/AOE_Attack/BP_AOE_Blast_PlagueDoctor.BP_AOE_Blast_PlagueDoctor_C" (Math|Transform|MakeTransform _array_element "0, 0, 0" "1.000000,1.000000,1.000000") "Undefined" "MultiplyWithRoot" 0 "/Game/Tech/AI/RangedAttacks/AOE_Attack/M_Attack1.M_Attack1" 2.0 (Game|GetPlayerCharacter 0) true true true 5.0 0)))))))

(event EventAttack
  (params (AttackTarget :type Actor%20Object%20Reference))
  ;[1 1 1] Attack
  (|CallParentFunction AttackTarget)
  (bind _returnvalue (AI|EQS|RunEQSQuery "/Game/Tech/AI/EQS/EQS_PlagueDoctorAttack.EQS_PlagueDoctorAttack" self "AllMatching"))
  (EventDispatchers|BindEventtoOnQueryFinishedEvent _returnvalue (delegate Custom|QueryFinished)))

(fn ConstructionScript
  (|CallParentFunction))

(fn GetPatrolRoute
  (return 0))

(fn GetIdealRange
  (return 4e+02 4e+02))

(fn SetMovementSpeed
  (params (Speed :type E_MovementSpeed%20Enum :default "NewEnumerator0"))
  (bind _output_get (Variables|/Script/Engine.CharacterMovementComponent|SetMaxWalkSpeed (Variables|Character|GetCharacterMovement) (Utilities|Select :Index Speed :NewEnumerator0 0.0 :NewEnumerator1 2e+02 :NewEnumerator2 3e+02 :NewEnumerator3 5e+02)))
  (return _output_get))