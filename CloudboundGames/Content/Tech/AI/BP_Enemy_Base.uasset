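; BP_Enemy_Base is a base enemy character that supplies movement and range data, likely for AI logic.
; It returns fixed attack and defend radii and exposes its assigned patrol route.
; SetMovementSpeed maps an idle-to-sprint speed state to CharacterMovement's max walk speed and returns the result.
; The construction script is empty, and LaunchDirectionAndVelocity holds only an unused roll velocity calculation.
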(fn ConstructionScript)

(fn GetIdealRange
  (return 1.5e+02 3.5e+02))

(fn GetPatrolRoute
  (return (Variables|AI|GetPatrolRoute)))

(fn SetMovementSpeed
  (params (Speed :type E_MovementSpeed%20Enum :default "NewEnumerator0"))
  (bind _output_get (Variables|/Script/Engine.CharacterMovementComponent|SetMaxWalkSpeed (Variables|Character|GetCharacterMovement) (Utilities|Select :Index Speed :NewEnumerator0 0.0 :NewEnumerator1 1e+02 :NewEnumerator2 3e+02 :NewEnumerator3 5e+02)))
  (return _output_get))