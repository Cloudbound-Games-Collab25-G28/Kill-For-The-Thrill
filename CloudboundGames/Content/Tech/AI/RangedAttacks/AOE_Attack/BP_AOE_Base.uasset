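; BP_AOE_Base is a base area-of-effect attack that damages pawns within a radius around itself.
; Trigger runs a sphere overlap, optionally ignoring the instigator and drawing a debug sphere, and can also fire automatically after a short delay on BeginPlay.
; For each actor hit, it calls OnAOEOverlapActor, prints the actor's name and applies damage of a configurable amount and type.
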(event Custom|SpawnAOESphere
  (if (Variables|Default|GetDrawDebugSphere)
    (Rendering|Debug|DrawDebugSphere (Transformation|GetActorLocation) (Variables|Default|GetRadius) 12 "(R=0.500000,G=0.000000,B=1.000000,A=1.000000)" 2.0 1.0))
  (bind _outactors (Collision|SphereOverlapActors (Transformation|GetActorLocation) (Variables|Default|GetRadius) (Utilities|Array|MakeArray "ObjectTypeQuery3") 0 (select (Variables|Default|GetIgnoreInstiagtor) (Utilities|Array|MakeArray (Game|GetInstigator)) 0)))
  (for _array_element _outactors
    (Default|CallOnAOEOverlapActor _array_element)
    (Development|PrintString (Utilities|GetDisplayName _array_element))
    (Game|Damage|ApplyDamage _array_element (Variables|Default|GetDamage) 0 self "/Script/Engine.DamageType")))

(event Custom|Trigger
  (CallFunction|SpawnAOESphere))

(event EventBeginPlay
  (if (Variables|Default|GetTriggerOnBeginPlay)
    (Utilities|FlowControl|Delay 2.0)
    (CallFunction|Trigger)))

(fn ConstructionScript)