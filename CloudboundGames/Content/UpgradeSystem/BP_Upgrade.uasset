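; BP_Upgrade is the base upgrade in the upgrade system, defining the stat hooks an upgrade can provide.
; Hooks cover damage, crit chance and crit damage, max health, movement speed and attack speed, plus an empty Init, each receiving a Context.
; Modifiers return separate add, proportional-add and multiply terms.
; All defaults are neutral, so a child upgrade needs to override only the stats it changes.
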(fn GetDamageModifier
  (params (Context :type F%20Damage%20Context%20Structure))
  (return (Utilities|Struct|MakeF_ValueModifier 0.0 0.0 1.0)))

(fn GetCritProbability
  (params (Context :type F%20Damage%20Context%20Structure))
  (return 0.0))

(fn GetCritDamageModifier
  (params (Context :type F%20Damage%20Context%20Structure))
  (return (Utilities|Struct|MakeF_ValueModifier 0.0 0.0 1.0)))

(fn Init
  (params (Context :type F%20Init%20Context%20Structure)))

(fn GetMaxHealth
  (params (Context :type F%20Max%20Health%20Context%20Structure))
  (return (Utilities|Struct|MakeF_ValueModifier 0.0 0.0 1.0)))

(fn GetMovementSpeedModifier
  (params (Context :type F%20Movement%20Speed%20Context%20Structure))
  (return (Utilities|Struct|MakeF_ValueModifier 0.0 0.0 1.0)))

(fn GetAttackSpeedModifier
  (params (Context :type F%20Attack%20Speed%20Context%20Structure))
  (return (Utilities|Struct|MakeF_ValueModifier 0.0 0.0 1.0)))