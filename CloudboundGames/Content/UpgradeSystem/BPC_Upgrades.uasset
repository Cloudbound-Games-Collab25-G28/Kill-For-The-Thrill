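; Upgrade component that holds an actor's upgrade objects and uses them to compute modified damage.
; It builds initial upgrades from classes on BeginPlay and fires OnUpgradesChanged whenever one is added or removed.
; ModifyDamage combines every upgrade's context-based damage modifier, adding crit modifiers on a weighted roll of summed, clamped crit probability.
; Modifiers stack by summing flat and proportional bonuses and multiplying multipliers, then apply in that order.
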(event EventBeginPlay
  (for _array_element (Variables|Default|GetInitialUpgrades)
    (CallFunction|AddUpgradeOfClass _array_element)))

(fn CombineModifiers
  (params (A :type F%20Value%20Modifier%20Structure) (B :type F%20Value%20Modifier%20Structure))
  (return (Utilities|Struct|MakeF_ValueModifier (+ (.add A) (.add B)) (+ (.addproportion A) (.addproportion B)) (* (.multiply A) (.multiply B)))))

(fn ApplyModifier
  (params (Value :type Float%20%28double-precision%29) (Modifier :type F%20Value%20Modifier%20Structure))
  (return (* (+ Value (.add Modifier)) (+ (.addproportion Modifier) 1.0) (.multiply Modifier))))

(fn ModifyDamage
  (params (BaseDamage :type Float%20%28double-precision%29) (Context :type F%20Damage%20Context%20Structure))
  (bind _probability (CallFunction|GetCritProbability Context))
  (bind _damagemodifier (CallFunction|GetCritDamageModifier Context))
  (bind _damagemodifier_2 (CallFunction|GetDamageModifier Context))
  (return (CallFunction|ApplyModifier BaseDamage (CallFunction|CombineModifiers _damagemodifier_2 (select (Math|Random|RandomBoolwithWeight _probability) _damagemodifier "")))))

(fn AddUpgradeOfClass
  (params (Upgrade :type BP%20Upgrade%20Class%20Reference))
  (bind _returnvalue (Game|ConstructObjectfromClass Upgrade))
  (CallFunction|AddUpgrade _returnvalue))

(fn GetDamageModifier
  (params (Context :type F%20Damage%20Context%20Structure))
  (for _array_element (Variables|Default|GetUpgrades)
    (bind _damagemodifier (Default|GetDamageModifier _array_element Context))
    (LocalVariables|SetTotalDamageModifier (CallFunction|CombineModifiers _damagemodifier (LocalVariables|GetTotalDamageModifier))))
  (return (LocalVariables|GetTotalDamageModifier)))

(fn GetCritDamageModifier
  (params (Context :type F%20Damage%20Context%20Structure))
  (for _array_element (Variables|Default|GetUpgrades)
    (bind _damagemodifier (Default|GetCritDamageModifier _array_element Context))
    (LocalVariables|SetTotalDamageModifier (CallFunction|CombineModifiers _damagemodifier (LocalVariables|GetTotalDamageModifier))))
  (return (LocalVariables|GetTotalDamageModifier)))

(fn GetCritProbability
  (params (Context :type F%20Damage%20Context%20Structure))
  (for _array_element (Variables|Default|GetUpgrades)
    (bind _probability (Default|GetCritProbability _array_element Context))
    (LocalVariables|SetTotalProbability (+ _probability (LocalVariables|GetTotalProbability))))
  (return (Math|Float|Clamp(Float) (LocalVariables|GetTotalProbability))))

(fn AddUpgrade
  (params (Upgrade :type BP%20Upgrade%20Object%20Reference))
  (Utilities|Array|Add (Variables|Default|GetUpgrades) Upgrade)
  (Default|CallOnUpgradesChanged))

(fn RemoveUpgrade
  (params (Upgrade :type BP%20Upgrade%20Object%20Reference))
  (Utilities|Array|RemoveItem (Variables|Default|GetUpgrades) Upgrade)
  (Default|CallOnUpgradesChanged))